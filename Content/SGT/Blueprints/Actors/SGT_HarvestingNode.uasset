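; SGT_HarvestingNode is a harvestable resource actor that exposes its reward, tool requirement, damage requirement and remaining uses through getter functions.
; The construction script applies the configured mesh, and BeginPlay fills the use count, which callers change through SetUses.
; When expended, it either destroys itself or optionally shrinks, waits a recharge delay, then restores unit scale and full uses.
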(event Custom|ExpendNode
  (bind _drainedscale (Variables|HarvestingNode|GetDrainedScale))
  (if (Variables|HarvestingNode|GetDestroyWhenDrained) ; Is this node set to be destroyed when drained?
    (Actor|DestroyActor) ; Destroy this harvesting node.
    (else
      (if (Variables|HarvestingNode|GetShrinkWhenDrained) ; Is the node set to shrink when drained?
        (Transformation|SetWorldScale3D (Variables|Default|GetActorMesh) (Math|Vector|MakeVector _drainedscale _drainedscale _drainedscale)) ; Update mesh scale to DrainedScale.
      )
      (Utilities|FlowControl|Delay (Variables|HarvestingNode|GetRechargeDelay)) ; Wait for the recharge delay.
      (CallFunction|ResetNode) ; Reset node to normal scale.
    )))

(event Custom|ResetNode
  (if (Variables|HarvestingNode|GetShrinkWhenDrained) ; Is this node set to shrink when drained?
    (Transformation|SetWorldScale3D (Variables|Default|GetActorMesh) "1.000000,1.000000,1.000000") ; Reset mesh scale to normal.
  )
  (Variables|HarvestingNode|SetUsesRemaining (Variables|HarvestingNode|GetUses)) ; Reset the remaining uses.
)

(event EventBeginPlay
  (Variables|HarvestingNode|SetUsesRemaining (Variables|HarvestingNode|GetUses)) ; Set uses remainign to max.
)

(event EventExpendEvent
  (CallFunction|ExpendNode) ; Call node expend event.
)

(event EventSetUses
  (params (UsesRemaining :type Integer))
  (Variables|HarvestingNode|SetUsesRemaining UsesRemaining) ; Update the current remaining uses.
)

(fn ConstructionScript
  (|CallParentFunction)
  (Components|StaticMesh|SetStaticMesh (Variables|Default|GetActorMesh) (Variables|HarvestingNode|GetMesh)))

(fn GetDamageInfo
  (return (Variables|HarvestingNode|GetMustBeDamaged) (Variables|HarvestingNode|GetDamageAmount)))

(fn GetReward
  (return (Variables|HarvestingNode|GetReward)))

(fn GetToolInfo
  (return (Variables|HarvestingNode|GetToolRequired) (Variables|HarvestingNode|GetRequiredTool)))

(fn GetUses
  (return (Variables|HarvestingNode|GetUsesRemaining)))