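; SGT_Pickup is a world item pickup actor configured from its row in the DT_SGT_Items data table.
; InitiateData, run at construction and BeginPlay, sets the mesh, clamps quantity to max stack size and builds a name with a count suffix.
; It ignores Pawn collision when spawned overlapping a pawn, then restores blocking when a pawn's overlap with CollisionDetection ends.
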(event OnComponentEndOverlap(CollisionDetection)
  (params (OverlappedComponent :type Primitive%20Component%20Object%20Reference) (OtherActor :type Actor%20Object%20Reference) (OtherComp :type Primitive%20Component%20Object%20Reference) (OtherBodyIndex :type Integer))
  (if (Utilities|ClassIsChildOf (Utilities|GetClass OtherActor) "/Script/Engine.Pawn") ; Is the overlapping item a pawn?
    (Utilities|IsValid (Variables|Default|GetActorMesh) ; Is there a valid actor mesh?
      (:Is%20Valid
        (Collision|SetCollisionResponsetoChannel (Variables|Default|GetActorMesh) "ECC_Pawn" "ECR_Block") ; Set actor mesh to block pawn collision.
      ))))

(event Custom|CreatePickup
  (CallFunction|InitiateData (Variables|Default|GetItem)) ; Run data intiation logic.
)

(event EventBeginPlay
  (CallFunction|CreatePickup) ; Upon begin play, create pickup with pickup data.
)

(fn ConstructionScript
  (|CallParentFunction)
  (bind _returnvalue (Utilities|GetDataTableRow "/Game/SGT/Blueprints/Data/DT_SGT_Items.DT_SGT_Items" (Utilities|Struct|BreakDataTableRowHandle (Variables|Default|GetItem))) ; Retrieve item data from inventory items data table.
    (:then
      (if (> (Variables|Default|GetQuantity) (Utilities|Struct|BreakStr_SGT_InventoryItem _returnvalue)) ; Is the quantity higher than the max stack size?
        (Variables|Default|SetQuantity (Utilities|Struct|BreakStr_SGT_InventoryItem _returnvalue)) ; Force quantity to max.
      )
      (CallFunction|InitiateData (Variables|Default|GetItem)) ; Initiate item data.
    )))

(fn InitiateData
  (params (ItemReference :type Data%20Table%20Row%20Handle%20Structure))
  (bind _returnvalue (Utilities|GetDataTableRow "/Game/SGT/Blueprints/Data/DT_SGT_Items.DT_SGT_Items" (Utilities|Struct|BreakDataTableRowHandle ItemReference)) ; Retrieve item data from inventory items data table.
    (:then
      (LocalVariables|SetItemData _returnvalue) ; Store data for cleaner use.
      (Variables|Default|SetQuantity (Math|Integer|Clamp(Integer) (Variables|Default|GetQuantity) 0 (.MaxStackSize (Utilities|Struct|BreakStr_SGT_InventoryItem _returnvalue)))) ; Set quantity, ensuring it is between 0 and the max stack size\nto prevent overstacking.
      (Components|StaticMesh|SetStaticMesh (Variables|Default|GetActorMesh) (.PickupMesh (Utilities|Struct|BreakStr_SGT_InventoryItem _returnvalue))) ; Update static mesh.
      (if (== (Variables|Default|GetQuantity) 1) ; Is this a singular item?
        (Variables|Default|SetName (Utilities|Text|ToText(String) (Utilities|Struct|BreakStr_SGT_InventoryItem (LocalVariables|GetItemData)))) ; Set single quantity version of name.
        (else
          (Variables|Default|SetName (Utilities|Text|ToText(String) (Utilities|String|Append (Utilities|Struct|BreakStr_SGT_InventoryItem (LocalVariables|GetItemData)) " (x" (Utilities|String|ToString(Integer) (Variables|Default|GetQuantity)) ")"))) ; Set multiple quantity version of name.
        ))
      (if (>= (Utilities|Array|Length (Collision|GetOverlappingActors (Variables|Components|GetCollisionDetection) "/Script/Engine.Pawn" :!class /Script/Engine.PrimitiveComponent)) 1) ; Is the actor overlapping at least one pawn?
        (Collision|SetCollisionResponsetoChannel (Variables|Default|GetActorMesh) "ECC_Pawn" "ECR_Ignore") ; Disable collision with pawns.
        (return) ; Done.
        (else
          (return) ; Done.
        )))
    (:RowNotFound
      (return) ; Done.
    )))