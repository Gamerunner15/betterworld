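; Workstation actor that registers itself with the inventory manager of players within its range.
; The construction script applies the configured mesh and sizes the trigger sphere from Range.
; Sphere begin and end overlaps add or remove the actor in NearbyWorkstations, reached through the pawn's controller.
; These array edits run on authority, with remote instances forwarding the call through server events.
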(event OnComponentBeginOverlap(Sphere)
  (params (OverlappedComponent :type Primitive%20Component%20Object%20Reference) (OtherActor :type Actor%20Object%20Reference) (OtherComp :type Primitive%20Component%20Object%20Reference) (OtherBodyIndex :type Integer) (bFromSweep :type Boolean) (SweepResult :type Hit%20Result%20Structure%20%28by%20ref%29))
  ;[1 1 1] Add this workstation to the player's nearby workstations.
  (CallFunction|AddNearbyWorkstation OtherActor))

(event OnComponentEndOverlap(Sphere)
  (params (OverlappedComponent :type Primitive%20Component%20Object%20Reference) (OtherActor :type Actor%20Object%20Reference) (OtherComp :type Primitive%20Component%20Object%20Reference) (OtherBodyIndex :type Integer))
  ;[1 1 1] Remove this workstation from the player's nearby workstations.
  (CallFunction|RemoveNearbyWorkstation OtherActor))

(event Custom|SRV_AddNearbyWorkstation
  (params (PawnActor :type Object%20Object%20Reference))
  ;[1 1 1] Add this workstation to the player's nearby workstations.
  (CallFunction|AddNearbyWorkstation PawnActor))

(event Custom|SRV_RemoveNearbyWorkstation
  (params (PawnActor :type Object%20Object%20Reference))
  ;[1 1 1] Remove this workstation from the player's nearby workstations.
  (CallFunction|RemoveNearbyWorkstation PawnActor))

(fn ConstructionScript
  (|CallParentFunction)
  (Components|StaticMesh|SetStaticMesh (Variables|Default|GetActorMesh) (Variables|Default|GetMesh)) ; Set the static mesh.
  (Components|Sphere|SetSphereRadius (Variables|Settings|GetSphere) (Variables|Settings|GetRange) true) ; Update the range players can use this workbench from.
)

(fn AddNearbyWorkstation
  (params (Object :type Object%20Object%20Reference))
  (Networking|SwitchHasAuthority ; Is this running on the server?
    (:Authority
      (bind _aspawn (Utilities|Casting|CastToPawn Object) ; Is the overlapping actor a pawn?
        (:then
          (bind _manager (Class|BPintController|GetInventory(Message) (Pawn|GetController _aspawn))) ; Retrieve a reference to the player's inventory manager component.
          (Utilities|Array|Add (Variables|/Game/SGT/Blueprints/Components/C_Manager-Inventory.C_Manager-Inventory_C|GetNearbyWorkstations _manager) self) ; Add this workstation actor to the player's\nnearby workstations array.
          (return) ; Done.
        )
        (:CastFailed
          _)))
    (:Remote
      (CallFunction|SRVAddNearbyWorkstation Object) ; Run this function on the server.
    ))
  (return) ; Done.
)

(fn RemoveNearbyWorkstation
  (params (Object :type Object%20Object%20Reference))
  (Networking|SwitchHasAuthority ; Is this running on the server?
    (:Authority
      (bind _aspawn (Utilities|Casting|CastToPawn Object) ; Is the overlapping actor a pawn?
        (:then
          (bind _manager (Class|BPintController|GetInventory(Message) (Pawn|GetController _aspawn))) ; Retrieve a reference to the player's inventory manager component.
          (Utilities|Array|RemoveItem (Variables|/Game/SGT/Blueprints/Components/C_Manager-Inventory.C_Manager-Inventory_C|GetNearbyWorkstations _manager) self) ; Remove reference to this actor from the\nplayer's nearby workstations array.
          (return) ; Done.
        )
        (:CastFailed
          _)))
    (:Remote
      (CallFunction|SRVRemoveNearbyWorkstation Object) ; Run this function on the server.
    ))
  (return) ; Done.
)

(fn GetClass
  (return (Variables|Settings|GetClass)))