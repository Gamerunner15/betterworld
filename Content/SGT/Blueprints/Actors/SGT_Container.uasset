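; Lootable container actor with an inventory component, open/close sounds, lock info and a "(Locked)" name suffix.
; On BeginPlay the server gets loot row IDs for its lootable class from game mode spawner data.
; SetInventory applies the preset contents or rolls random loot table rows, re-picking whenever a spawn-chance check fails.
; Randomized contents can regenerate on a timer, which postpones the reset while the container is open.
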(event Custom|PlaySound
  (params (SoundToPlay :type Sound%20Wave%20Object%20Reference))
  (Audio|PlaySoundatLocation SoundToPlay (Transformation|GetActorLocation self) "0, 0, 0" 1.0 1.0 0.0 "/Game/SGT/Sounds/SA_SGT_DefaultAttenuation.SA_SGT_DefaultAttenuation" 0 0) ; Play input sound at actor location.
)

(event EventBeginPlay
  (Networking|SwitchHasAuthority ; Ensure this only runs on server.
    (:Authority
      (CallFunction|InitializeLoot) ; Initialize container loot based on settings.
    )))

(event EventUpdateInventory
  (params (ContainerInventory :type Array%20of%20Str%20SGT%20Inventory%20Entry%20Structures))
  (Variables|/Game/SGT/Blueprints/Components/C_Component-Inventory.C_Component-Inventory_C|SetInventory (Variables|ContainerSettings|GetComponent-Inventory) ContainerInventory) ; Update the container inventory.
)

(event EventSetIsOpen
  (params (State :type Boolean))
  (bind _output_get (Variables|ContainerSettings|SetIsOpen State)) ; Update container open state.
  (if _output_get ; Was this chest just set to open?
    (CallFunction|PlaySound (Variables|ContainerSettings|GetOpenSound)) ; Play chest open sound.
    (else
      (CallFunction|PlaySound (Variables|ContainerSettings|GetCloseSound)) ; Play chest close sound.
    )))

(fn ConstructionScript
  (|CallParentFunction)
  (Components|StaticMesh|SetStaticMesh (Variables|Default|GetActorMesh) (Variables|Default|GetMesh)) ; Set the static mesh.
  (Variables|Default|SetName (Variables|ContainerSettings|GetContainerName)) ; Set the actor name for interactive\nindication.
)

(fn SetInventory
  (Utilities|Array|Clear (Variables|/Game/SGT/Blueprints/Components/C_Component-Inventory.C_Component-Inventory_C|GetInventory (Variables|ContainerSettings|GetComponent-Inventory))) ; Ensure inventory is clear before\nprocessing.
  (Networking|SwitchHasAuthority ; Only set the inventory on the server.
    (:Authority
      (if (Variables|ContainerSettings|GetRandomizeContents) ; Do we want to randomize the contents of\nthis container using lootable classes? If\nnot, uses set inventory.
        (Utilities|Array|Clear (Variables|ContainerSettings|GetInventory)) ; Clear any previously set inventory.
        (if (Variables|ContainerSettings|GetNoLootFound) ; Does this container have an invalid or\nempty lootable class?
          (return) ; Done.
          (else
            (bind _output_get (Variables|ContainerSettings|SetItemCount (Math|Random|RandomIntegerinRange (Variables|ContainerSettings|GetMinItems) (Variables|ContainerSettings|GetMaxItems)))) ; Store randomly generated loot quantity\n(based on min and max item count) for\ncleaner use.
            (for _index (range 1 _output_get) ; For each loot item that needs to be\ngenerated...
              (bind _outrownames (DataTable|GetDataTableRowNames "/Game/SGT/Blueprints/Data/DT_SGT_LootTable.DT_SGT_LootTable" :!label _label)) ; Retrieve the data table rows from the lootable class table...
              (bind _returnvalue (Utilities|GetDataTableRow "/Game/SGT/Blueprints/Data/DT_SGT_LootTable.DT_SGT_LootTable" (Utilities|Array|Get(acopy) _outrownames (Utilities|Array|Get(acopy) (Variables|ContainerSettings|GetLootIDs) (Math|Random|RandomIntegerinRange 1 (Variables|ContainerSettings|GetLootCount))))) ; Pick a random item matching this lootable class and retrieve data from data table...
                (:then
                  (if (> (.ChanceToSpawn (Utilities|Struct|BreakStr_SGT_LootTable _returnvalue)) (Math|Random|RandomFloat)) ; Randomise percent and check against\nchance to generate. Should we generate\nthis item?
                    (Utilities|Array|Add (Variables|ContainerSettings|GetInventory) (Utilities|Struct|MakeStr_SGT_InventoryEntry (.Item (Utilities|Struct|BreakStr_SGT_LootTable _returnvalue)) (Math|Random|RandomIntegerinRange 1 (.MaximumQuantity (Utilities|Struct|BreakStr_SGT_LootTable _returnvalue))) 1.0)) ; Add to the container inventory.
                    (else
                      (goto _label))))
                (:RowNotFound
                  (goto _label)))))))
      (Variables|/Game/SGT/Blueprints/Components/C_Component-Inventory.C_Component-Inventory_C|SetInventory (Variables|ContainerSettings|GetComponent-Inventory) (Variables|ContainerSettings|GetInventory)) ; Set the inventory in the actor\ncomponent.
      (if (Variables|ContainerSettings|GetResetContentsOnCycle) ; Do we want to regenerate loot periodically?
        (Utilities|Time|SetTimerbyFunctionName 0 "CheckLoot" (Variables|ContainerSettings|GetContentsLifetime)) ; Set timer for loot lifetime check.
        (return) ; Done.
        (else
          (return) ; Done.
        )))
    (:Remote
      (return) ; Done.
    )))

(fn GetName
  (bind _name (|CallParentFunction))
  (if (Variables|ContainerSettings|GetLocked?) ; Is the container locked?
    (return (Utilities|Text|ToText(String) (Utilities|String|Append (Utilities|String|ToString(Text) _name) " (Locked)"))) ; Done.
    (else
      (return _name) ; Done.
    )))

(fn InitializeLoot
  (Variables|ContainerSettings|SetNoLootFound true) ; Set loot found control state to true.
  (bind _spawnerlootdata (Class|BPIntGameMode|GetSpawnerData(Message) (Game|GetGameMode))) ; Retrieve spawner data from game mode.
  (bind _array_element (Utilities|Array|ForEachLoopwithBreak _spawnerlootdata :!label _label) ; For each entry inthe spawner loot data array...
    (:LoopBody
      (if (Utilities|Enum|Equal(Enum) (.SpawnerClass (Utilities|Struct|BreakStr_SGT_LootTableIDs _array_element)) (Variables|ContainerSettings|GetLootableClass)) ; Does the current array element match\nthis spawner's class?
        (Variables|ContainerSettings|SetLootIDs (.RowIDs (Utilities|Struct|BreakStr_SGT_LootTableIDs _array_element))) ; Update the loot IDs.
        (goto _label Break)))
    (:Completed
      (Variables|ContainerSettings|SetNoLootFound (== (Utilities|Array|Length (Variables|ContainerSettings|GetLootIDs)) 0)) ; Set loot found control state based on\nlength of LootIDs array.
      (Variables|ContainerSettings|SetLootCount (- (Utilities|Array|Length (Variables|ContainerSettings|GetLootIDs)) 1)) ; Store number of loot items that match\nthis container's lootable class for\ncleaner use.
      (CallFunction|SetInventory) ; Set the intial container loot.
      (return))))

(fn CheckLoot
  (if (Variables|ContainerSettings|GetIsOpen) ; Is this container currently in use?
    (Utilities|Time|SetTimerbyFunctionName 0 "CheckLoot" 5.0) ; Set another check to happen in five seconds time.
    (return) ; Done.
    (else
      (CallFunction|SetInventory) ; Trigger inventory regeneration.
      (return) ; Done.
    )))

(fn GetInventory
  (return (Variables|/Game/SGT/Blueprints/Components/C_Component-Inventory.C_Component-Inventory_C|GetInventory (Variables|ContainerSettings|GetComponent-Inventory))))

(fn GetIsOpen
  (return (Variables|ContainerSettings|GetIsOpen)))

(fn GetLockInfo
  (return (Variables|ContainerSettings|GetLocked?) (Variables|ContainerSettings|GetLockID)))

(fn GetMaxStorage
  (return (Variables|ContainerSettings|GetMaximumStorageCount)))