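; Loot spawner actor that periodically scatters random SGT_Pickup items inside a box volume.
; On the server, it polls the game mode until the loot table is sorted, then caches row indices for its spawner class.
; Spawning rerolls DT_SGT_LootTable rows until a chance check passes, using line traces for ground placement.
; Timers drive respawn and expiry, with camper and detection spheres delaying them or despawning loot based on nearby characters.
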(event OnComponentEndOverlap(DetectionZone)
  (params (OverlappedComponent :type Primitive%20Component%20Object%20Reference) (OtherActor :type Actor%20Object%20Reference) (OtherComp :type Primitive%20Component%20Object%20Reference) (OtherBodyIndex :type Integer))
  ;[1 0.2 0.2 0.5] Trigger despawn check on player leaving detection zone.
  (Utilities|Casting|CastToCharacter OtherActor) ; Ensure it was a character that left the detection zone.
  (if (Variables|Settings|GetDespawnIfNoPlayersInRange) ; Is loot supposed to be removed if no players within range?
    (if (not (>= (Utilities|Array|Length (Collision|GetOverlappingActors (Variables|Settings|GetDetectionZone) "/Script/Engine.Character" :!class /Script/Engine.PrimitiveComponent)) 1)) ; Check if any other players are\nwithin range.
      (CallFunction|DespawnLoot) ; Despawn loot.
    )))

(event EventBeginPlay
  ;[1 0.2 0.2 0.5] Initialize this loot spawner.
  (CallFunction|Initialize))

(fn ConstructionScript
  (Components|Box|SetBoxExtent (Variables|Settings|GetSpawnVolume) (Variables|Settings|GetVolumeExtents) false) ; Update spawn volume size.
  (Transformation|SetRelativeLocation (Variables|Settings|GetSpawnVolume) (Math|Vector|MakeVector 0.0 0.0 (.Z (Math|Vector|BreakVector (Variables|Settings|GetVolumeExtents)))) false false) ; Set spawn volume above origin.
  (Components|Sphere|SetSphereRadius (Variables|Settings|GetDetectionZone) (Variables|Settings|GetMaximumPlayerDistance) false) ; Update detection zone size.
  (Components|Sphere|SetSphereRadius (Variables|Settings|GetCamperZone) (Variables|Settings|GetMinimumPlayerDistance) false) ; Update camper zone size.
)

(fn Initialize
  (Networking|SwitchHasAuthority ; Ensure this is running on the server.
    (:Authority
      (bind _state (Class|BPIntGameMode|GetLoottableState(Message) (Game|GetGameMode))) ; Retrieve loottable sorted state from\ngamemode.
      (if _state ; Has the loottable been sorted?
        (bind _spawnerlootdata (Class|BPIntGameMode|GetSpawnerData(Message) (Game|GetGameMode))) ; Retrieve spawner data from game mode.
        (bind _array_element (Utilities|Array|ForEachLoopwithBreak _spawnerlootdata :!label _label) ; For each entry inthe spawner loot data array...
          (:LoopBody
            (if (Utilities|Enum|Equal(Enum) (.SpawnerClass (Utilities|Struct|BreakStr_SGT_LootTableIDs _array_element)) (Variables|Settings|GetSpawnerClass)) ; Does the current array element match\nthis spawner's class?
              (Variables|Settings|SetLootIDs (.RowIDs (Utilities|Struct|BreakStr_SGT_LootTableIDs _array_element))) ; Update the loot IDs.
              (goto _label Break)))
          (:Completed
            (if (Variables|Settings|GetSpawnOnInitialize) ; Is loot supposed to be spawned initially?
              (CallFunction|SpawnLoot) ; Spawn loot.
              (else
                (Utilities|Time|SetTimerbyFunctionName 0 "SpawnTimer" (Variables|Settings|GetRespawnDelay)) ; Initiate the spawn timer.
              ))
            (return) ; Done.
          ))
        (else
          (Utilities|Time|SetTimerbyFunctionName 0 "Initialize" 0.25) ; Wait a short period and re-run initialize.
          (return) ; Done.
        )))
    (:Remote
      (return) ; Done.
    )))

(fn SpawnLoot
  (bind _returnvalue (Math|Random|RandomFloat))
  (for _array_element (Variables|Settings|GetSpawnedItems) ; For each item staored in the spawned\nitems array...
    (Utilities|IsValid _array_element ; Is this item still valid?
      (:Is%20Valid
        (Actor|DestroyActor _array_element) ; Remove old loot.
      )))
  (Utilities|Array|Clear (Variables|Settings|GetSpawnedItems)) ; Clear list of spawned items.
  (LocalVariables|SetItemCount (Math|Random|RandomIntegerinRange (Variables|Settings|GetMinimumItems) (Variables|Settings|GetMaximumItems))) ; Store randomly generated loot quantity\nfor cleaner use.
  (LocalVariables|SetLootCount (- (Utilities|Array|Length (Variables|Settings|GetLootIDs)) 1)) ; Store number of loot items that match this\nspawner class for cleaner use.
  (for _index (range 1 (LocalVariables|GetItemCount)) ; For each loot item that needs to be spawned...
    (bind _outrownames (DataTable|GetDataTableRowNames "/Game/SGT/Blueprints/Data/DT_SGT_LootTable.DT_SGT_LootTable" :!label _label)) ; Retrieve the data table rows from the spawner loot table...
    (bind _returnvalue_2 (Utilities|GetDataTableRow "/Game/SGT/Blueprints/Data/DT_SGT_LootTable.DT_SGT_LootTable" (Utilities|Array|Get(acopy) _outrownames (Utilities|Array|Get(acopy) (Variables|Settings|GetLootIDs) (Math|Random|RandomIntegerinRange 1 (LocalVariables|GetLootCount))))) ; Pick a random item matching this loot spawner class and retrieve data from data table...
      (:then
        (if (> (.ChanceToSpawn (Utilities|Struct|BreakStr_SGT_LootTable _returnvalue_2)) (Math|Random|RandomFloat)) ; Randomise percent and check against\nchance to spawn. Should we spawn this\nitem?
          (LocalVariables|SetLootData (.Item (Utilities|Struct|BreakStr_SGT_LootTable _returnvalue_2))) ; Store data for cleaner use.
          (LocalVariables|SetQuantity (Math|Random|RandomIntegerinRange 1 (.MaximumQuantity (Utilities|Struct|BreakStr_SGT_LootTable _returnvalue_2)))) ; Generate quantity within min and max\nand store for cleaner use.
          (bind _generatedlocation (CallFunction|GetLootLocation)) ; Generate randomised loot spawn location within spawn volume bounds.
          (bind _returnvalue_3 (Game|SpawnActorfromClass "/Game/SGT/Blueprints/Actors/SGT_Pickup.SGT_Pickup_C" (Math|Transform|MakeTransform _generatedlocation (Math|Rotator|MakeRotator _returnvalue _returnvalue 0.0)) "Undefined" 0 (LocalVariables|GetLootData) (LocalVariables|GetQuantity) 1.0 0)) ; Spawn item pickup actor.
          (Default|CreatePickup _returnvalue_3) ; Initiate data and create pickup.
          (Utilities|Array|Add (Variables|Settings|GetSpawnedItems) _returnvalue_3) ; Add loot item to the spawned items list.
          (else
            (goto _label))))
      (:RowNotFound
        (goto _label))))
  (Utilities|Time|SetTimerbyFunctionName 0 "SpawnTimer" (Variables|Settings|GetRespawnDelay)) ; Initiate respawn timer.
  (Utilities|Time|SetTimerbyFunctionName 0 "DespawnTimer" (Variables|Settings|GetLootLifetime)) ; Initiate despawn loop.
  (return) ; Done.
)

(fn DespawnLoot
  (for _array_element (Variables|Settings|GetSpawnedItems) ; For each item stored in the spawned\nitems array...
    (Utilities|IsValid _array_element ; Is this item still valid?
      (:Is%20Valid
        (Actor|DestroyActor _array_element) ; Remove old loot.
      )))
  (return) ; Done.
)

(fn SpawnTimer
  (if (and (Variables|Settings|GetProtectLootFromCampers) (>= (Utilities|Array|Length (Collision|GetOverlappingActors (Variables|Settings|GetCamperZone) "/Script/Engine.Character" :!class /Script/Engine.PrimitiveComponent)) 1)) ; Is camping protection enabled AND is there anyone in the camping zone?
    _
    (elif (and (Variables|Settings|GetOnlySpawnIfPlayersInRange) (< (Utilities|Array|Length (Collision|GetOverlappingActors (Variables|Settings|GetDetectionZone) "/Script/Engine.Character" :!class /Script/Engine.PrimitiveComponent)) 1)) ; Is loot not supposed to spawn when no players in range AND are there no players in range?
      _
      (else
        (CallFunction|SpawnLoot) ; Spawn loot.
        (return) ; Done.
      )))
  (Utilities|Time|SetTimerbyFunctionName 0 "SpawnTimer" (Variables|Settings|GetAdditionalDelay)) ; Add addition spawn delay.
  (return) ; Done.
)

(fn GetLootLocation
  (bind _spawnvolume (Variables|Settings|GetSpawnVolume))
  (bind (_origin _boxextent) (Collision|GetComponentBounds _spawnvolume))
  (bind _returnvalue (- _origin _boxextent))
  (bind _returnvalue_2 (+ _origin _boxextent))
  (bind (_x _y _z) (Math|Vector|BreakVector _returnvalue_2))
  (bind (_x_2 _y_2 _z_2) (Math|Vector|BreakVector _returnvalue))
  (LocalVariables|SetMaxZ _z) ; Store maximum Z value for\ncleaner use.
  (LocalVariables|SetMinZ _z_2) ; Store minimum Z value for\ncleaner use.
  (LocalVariables|SetRanX (Math|Random|RandomFloatinRange _x _x_2)) ; Store randomised X value for\ncleaner use.
  (LocalVariables|SetRanY (Math|Random|RandomFloatinRange _y _y_2)) ; Store randomised Y value for\ncleaner use.
  (bind (_outhit _returnvalue_3) (Collision|LineTraceByChannel (Math|Vector|MakeVector (LocalVariables|GetRanX) (LocalVariables|GetRanY) (LocalVariables|GetMaxZ)) (Math|Vector|MakeVector (LocalVariables|GetRanX) (LocalVariables|GetRanY) (LocalVariables|GetMinZ)) "TraceTypeQuery1" false 0 "None")) ; Perform a trace from max Z to min Z at spawn location to\nensure item is not spawning underground.
  (if _returnvalue_3 ; Was a hit detected?
    (LocalVariables|SetRanZ (.Z (Math|Vector|BreakVector (.Location (Collision|BreakHitResult _outhit))))) ; Use impact location to determine spawn Z value.
    (else
      (LocalVariables|SetRanZ (LocalVariables|GetMinZ)) ; As no hit was detected, just use the minimum Z value.
    ))
  (return (Math|Vector|MakeVector (LocalVariables|GetRanX) (LocalVariables|GetRanY) (LocalVariables|GetRanZ))) ; Done.
)

(fn DespawnTimer
  (if (>= (Utilities|Array|Length (Collision|GetOverlappingActors (Variables|Settings|GetCamperZone) "/Script/Engine.Character" :!class /Script/Engine.PrimitiveComponent)) 1) ; Are there any players in the camper zone?
    (Utilities|Time|SetTimerbyFunctionName 0 "DespawnTimer" (Variables|Settings|GetAdditionalDelay)) ; Retrigger this check after an additional delay.
    (return) ; Done.
    (else
      (CallFunction|DespawnLoot) ; Despawn current loot.
      (return) ; Done.
    )))