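; Survival game mode that tracks session changes and builds the loot lookup used by spawners.
; Player logins (after a short delay) and logouts call SessionState on the SurvivalGamestate, which per its comments handles singleplayer versus multiplayer.
; On authority BeginPlay, it sorts DT_SGT_LootTable row indices into per-spawner-class arrays, skipping "All" and seeding each with an ignored -1.
; Getters expose this data and its sorted flag.
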(event EventBeginPlay
  ;[0.2 1 0.2 0.5] Sort spawner loot data table into class arrays.
  (Networking|SwitchHasAuthority
    (:Authority
      (if (not (Variables|Default|GetLootTablesSorted))
        (CallFunction|InitializeLootTables)))))

(event EventPostLogin
  (params (NewPlayer :type Player%20Controller%20Object%20Reference))
  ;[0.2 1 0.2 0.5] Execute shortly after the player logins to the session.
  (Utilities|FlowControl|Delay 0.25) ; Wait for a short delay to allow casting on client.
  (bind _assurvival_gamestate (Utilities|Casting|CastToSurvivalGamestate (Game|GetGameState)))
  (Default|SessionState _assurvival_gamestate))

(event EventOnLogout
  (params (ExitingController :type Controller%20Object%20Reference))
  ;[0.2 1 0.2 0.5] Check if the game is now a singleplayer game or still multiplayer.
  (bind _assurvival_gamestate (Utilities|Casting|CastToSurvivalGamestate (Game|GetGameState)))
  (Default|SessionState _assurvival_gamestate))

(fn ConstructionScript)

(fn InitializeLootTables
  (Utilities|Array|Clear (Variables|Default|GetLootTableData)) ; Clear any data already present.
  (bind _enumvalue (|ForEachE_SGT_LootableClass) ; For each spawner class defined in\nE_LootTableClass
    (:LoopBody
      (bind _output_get (LocalVariables|SetSpawnerClass _enumvalue)) ; Store for cleaner use...
      (if (not (Utilities|Enum|Equal(Enum) _output_get "NewEnumerator0")) ; Is this class "All"?
        (Utilities|Array|Add (Variables|Default|GetLootTableData) (Utilities|Struct|MakeStr_SGT_LootTableIDs (LocalVariables|GetSpawnerClass) (Utilities|Array|MakeArray -1))) ; Make a new array entry for this spawner class. As UE cannot\nhandle empty arrays, so create array entry at index 0 with data\n-1 (will be ignored in use).
      ))
    (:then
      (bind _outrownames (DataTable|GetDataTableRowNames "/Game/SGT/Blueprints/Data/DT_SGT_LootTable.DT_SGT_LootTable")) ; Retrieve a list of all spawner loot defined by the loot table data\ntable.
      (for (_array_element _array_index) _outrownames ; For every entry in data table...
        (LocalVariables|SetArrayIndex _array_index) ; Store index for cleaner use...
        (bind _returnvalue (Utilities|GetDataTableRow "/Game/SGT/Blueprints/Data/DT_SGT_LootTable.DT_SGT_LootTable" _array_element) ; Retrieve appropriate data from data table.
          (:then
            (for (_array_element_2 _array_index_2) (Variables|Default|GetLootTableData) ; For every entry int he LootTableData array...
              (LocalVariables|SetArElement _array_element_2) ; Store data for cleaner use.
              (LocalVariables|SetArIndex _array_index_2) ; Store data for cleaner use.
              (if (Utilities|Array|ContainsItem (Utilities|Struct|BreakStr_SGT_LootTable _returnvalue) (.SpawnerClass (Utilities|Struct|BreakStr_SGT_LootTableIDs (LocalVariables|GetArElement)))) ; Does the data table data define this array spawner class as a match?
                (bind _output_get_2 (LocalVariables|SetRowIDs (.RowIDs (Utilities|Struct|BreakStr_SGT_LootTableIDs (LocalVariables|GetArElement))))) ; Store row IDs array for cleaner use.
                (Utilities|Array|Add _output_get_2 (LocalVariables|GetArrayIndex)) ; Add new match to Row IDs.
                (bind _structout (Utilities|Struct|SetmembersinStr_SGT_LootTableIDs (LocalVariables|GetArElement) (LocalVariables|GetRowIDs))) ; Update array element with new Row IDs array.
                (Utilities|Array|SetArrayElem (Variables|Default|GetLootTableData) (LocalVariables|GetArIndex) _structout) ; Set new data in LootTableData array.
              )))))
      (Variables|Default|SetLootTablesSorted true) ; Update sort state boolean.
      (return) ; Done.
    )))

(fn GetLoottableState
  (return (Variables|Default|GetLootTablesSorted)))

(fn GetSpawnerData
  (return (Variables|Default|GetLootTableData)))