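; Game state for the survival game that holds shared day/night cycle data and tracks whether the session is singleplayer.
; Setter events and getters expose days passed, calculated state and current and next curve selection.
; The TimeOfDay timeline sits behind a never-firing dummy branch so it can be handed out and driven externally by the TimeOfDay Manager.
; SessionState updates the singleplayer flag on authority from the player count.
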(event Custom|DummyEvent
  (if false ; Dummy branch. Will never fire.
    ;[1 0.2 0.2 0.5] !!!!!!!!!!!!!!!!!!!!!!! Do not delete !!!!!!!!!!!!!!!!!!!!!!!!
    ; !!!!!!!!!!!!!! Day/night cycle timeline !!!!!!!!!!!!!!!!
    ; !!!!!!! Controlled by TimeOfDay Manager !!!!!!!
    (Timeline|TimeOfDay Play)))

(event Custom|SessionState
  ;[1 0.2 0.2 0.5] Determine if this is still a singleplayer session or not.
  (Networking|SwitchHasAuthority
    (:Authority
      (bind _returnvalue (Class|GameMode|GetNumPlayers (Variables|Default|GetAuthorityGameMode)))
      (Variables|Default|SetIsSingleplayer (not (> _returnvalue 1))))))

(event EventSetCalculated
  (params (Calculated? :type Boolean))
  ;[1 0.2 0.2 0.5] Update calculated state bool.
  (Variables|TimeOfDay|SetCalculated Calculated?))

(event EventSetCurrentCurve
  (params (Curve :type Integer))
  ;[1 0.2 0.2 0.5] Update current curve.
  (Variables|Temperature|SetCurrentCurve Curve))

(event EventSetCurveChosen
  (params (Chosen? :type Boolean))
  ;[1 0.2 0.2 0.5] Update curve chosen state.
  (Variables|Temperature|SetNextCurveChosen Chosen?))

(event EventSetDaysPassed
  (params (DaysPassed :type Integer))
  ;[1 0.2 0.2 0.5] Update days passed.
  (Variables|TimeOfDay|SetDaysPassed DaysPassed))

(event EventSetNextCurve
  (params (Curve :type Integer))
  ;[1 0.2 0.2 0.5] Update next curve.
  (Variables|Temperature|SetNextCurve Curve))

(fn ConstructionScript)

(fn GetCalculated
  (return (Variables|TimeOfDay|GetCalculated)))

(fn GetCurrentCurve
  (return (Variables|Temperature|GetCurrentCurve)))

(fn GetCurveChosen
  (return (Variables|Temperature|GetNextCurveChosen)))

(fn GetDaysPassed
  (return (Variables|TimeOfDay|GetDaysPassed)))

(fn GetNextCurve
  (return (Variables|Temperature|GetNextCurve)))

(fn GetTimeline
  (return (Variables|Default|GetTimeOfDay)))