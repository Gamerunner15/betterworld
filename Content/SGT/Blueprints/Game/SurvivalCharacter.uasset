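; Survival game player character that holds stance, aim, view and death state behind setters and getters, and forwards damage to its controller.
; Setters write variables, and RepNotify functions apply flashlight light and emissive, modular equipment meshes, and ragdoll on death.
; Equipment pieces follow the body mesh through master pose.
; The owner's view hides the body when the camera overlaps the capsule, and head pieces in first person.
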(event OnComponentBeginOverlap(CameraCollision)
  (params (OverlappedComponent :type Primitive%20Component%20Object%20Reference) (OtherActor :type Actor%20Object%20Reference) (OtherComp :type Primitive%20Component%20Object%20Reference) (OtherBodyIndex :type Integer) (bFromSweep :type Boolean) (SweepResult :type Hit%20Result%20Structure%20%28by%20ref%29))
  ;[1 1 1] Control camera collision and player visibility.
  ;;[1 1 1] Hide player model if camera is inside of the capsule.
  (if (== OtherComp (Variables|Collision|GetCapsuleComponent))
    (CallFunction|HideMeshforPlayer true)))

(event OnComponentEndOverlap(CameraCollision)
  (params (OverlappedComponent :type Primitive%20Component%20Object%20Reference) (OtherActor :type Actor%20Object%20Reference) (OtherComp :type Primitive%20Component%20Object%20Reference) (OtherBodyIndex :type Integer))
  ;[1 1 1] Control camera collision and player visibility.
  ;;[1 1 1] Show player model once camera leaves the capsule.
  (if (== OtherComp (Variables|Collision|GetCapsuleComponent))
    (CallFunction|HideMeshforPlayer false)))

(event Custom|PlaySound
  (params (Sound :type Sound%20Base%20Object%20Reference) (Location :type Vector))
  (Audio|PlaySoundatLocation Sound Location "0, 0, 0" 1.0 1.0 0.0 "/Game/SGT/Sounds/SA_SGT_DefaultAttenuation.SA_SGT_DefaultAttenuation" 0 0))

(event EventSetEquipmentMesh
  (params (Type :type E_SGT_EquipmentType%20Enum :default "NewEnumerator0") (Mesh :type Skeletal%20Mesh%20Object%20Reference))
  (CallFunction|SetNewEquipment Type Mesh) ; Update equipment.
)

(event EventSetSprint
  (params (State :type Boolean))
  ;[1 1 1] Control character states.
  (Variables|Character|Data|Movement|SetIsSprinting State) ; Set sprint state.
)

(event EventSetProne
  (params (ProneState :type Boolean))
  ;[1 1 1] Control character states.
  (Variables|Character|Data|Movement|SetIsProne ProneState) ; Set prone state.
)

(event EventSetViewMode
  (params (State :type Boolean))
  ;[1 1 1] Control character states.
  (bind _output_get (Variables|Character|SetIsFirstPerson State)) ; Set first person state.
  (Class|PrimitiveComponent|SetOwnerNoSee (Variables|CharacterMeshes|GetE_Head) _output_get) ; Hide/unhide player head and helmet model.
)

(event EventSetAim
  (params (State :type Boolean))
  ;[1 1 1] Control character states.
  (Variables|Character|Data|Movement|SetIsAiming State) ; Set aim state.
)

(event EventShowChestlight
  (params (Enable :type Boolean))
  ;[1 1 1] Control flashlight.
  (Variables|Flashlight|Data|SetShowFlashlight Enable))

(event EventResetMesh
  ;[1 1 1] Control camera collision and player visibility.
  ;;[1 1 1] Show player model once camera leaves the capsule.
  (CallFunction|HideMeshforPlayer false))

(event EventToggleFlashlight
  (params (TurnOn :type Boolean))
  ;[1 1 1] Control flashlight.
  (Variables|Flashlight|Data|SetFlashlightOn TurnOn))

(event EventTriggerSound
  (params (Sound :type Sound%20Base%20Object%20Reference) (Location :type Vector :default "0, 0, 0"))
  (CallFunction|PlaySound Sound Location))

(event EventBeginPlay
  (CallFunction|GetFlashlightMaterial) ; Get light material from flashlight.
  (Class|SkinnedMeshComponent|SetMasterPoseComponent (Variables|CharacterMeshes|GetE_Head) (Variables|Character|GetMesh) false) ; Update master pose for each equipment piece.
)

(event EventSetCrouch
  (params (CrouchState :type Boolean))
  ;[1 1 1] Control character states.
  (Variables|Character|Data|Movement|SetIsCrouching CrouchState) ; Set crouch state.
)

(event EventSetLootable
  (params (Lootable :type SGT%20Container%20Object%20Reference))
  ;[1 1 1] Control character states.
  (Variables|Character|SetLootableInventory Lootable) ; Set player lootable inventory.
)

(event EventGetProneAnimState
  (params (NewState :type Boolean))
  ;[1 1 1] Control character states.
  (Variables|Character|Data|Movement|SetProneAnimDone NewState) ; Set prone anim state.
)

(event EventSetIsDead
  (params (State :type Boolean))
  ;[1 1 1] Control character states.
  (Variables|Character|Data|SetIsDead State) ; Set player death state.
)

(event EventSetFlashlightMat
  (params (Intensity :type Float%20%28single-precision%29) (Emissive :type Float%20%28single-precision%29))
  ;[1 1 1] Control flashlight.
  (Variables|Flashlight|Data|SetFlashlightIntensity Intensity) ; Update flashlight intensity.
  (Variables|Flashlight|Data|SetFlashlightEmissive Emissive) ; Update flashlight emissive level.
)

(event EventDamageEvent
  (params (Amount :type Float%20%28single-precision%29) (Type :type Damage%20Type%20Class%20Reference))
  ;[1 1 1] Called on character damage event.
  (Game|Damage|ApplyDamage (Pawn|GetController self) Amount 0 0 Type) ; Call damage event on controller.
)

(event EventGetCrouchAnimState
  (params (NewState :type Boolean))
  ;[1 1 1] Control character states.
  (Variables|Character|Data|Movement|SetCrouchAnimDone NewState) ; Set crouch anim state.
)

(fn ConstructionScript)

(fn OnRepIsDead
  (if (Variables|Character|Data|GetIsDead) ; Is this character dead?
    (Physics|SetSimulatePhysics (Variables|Character|GetMesh) true) ; Enable ragdoll.
    (Class|PrimitiveComponent|WakeAllRigidBodies (Variables|Character|GetMesh)) ; Wake up all rigid bodies for better interaction with dead bodies.
    (Collision|SetCollisionEnabled (Variables|Collision|GetCapsuleComponent) "NoCollision") ; Disable capsule collision for better interaction with dead bodies.
    (return) ; Done.
    (else
      (return) ; Done.
    )))

(fn OnRepShowFlashlight
  (Rendering|SetVisibility (Variables|Flashlight|Components|GetFlashlight) (Variables|Flashlight|Data|GetShowFlashlight) false) ; Update the flashlight visibility.
  (return) ; Done.
)

(fn OnRepFlashlighton
  (if (Variables|Flashlight|Data|GetFlashlightOn) ; Are we turning the flashlight on or off?
    (Rendering|Components|Light|SetIntensity (Variables|Flashlight|Components|GetSpotLight) (Variables|Flashlight|Data|GetFlashlightIntensity)) ; Set flashlight to on.
    (Rendering|Material|SetScalarParameterValue (Variables|Flashlight|Data|GetFlashlightScreen) "EmissiveLevel" (Variables|Flashlight|Data|GetFlashlightEmissive) :!class /Script/Engine.MaterialInstanceDynamic) ; Set emissive effect to 5.
    (return) ; Done.
    (else
      (Rendering|Components|Light|SetIntensity (Variables|Flashlight|Components|GetSpotLight) 0.0) ; Set flashlight to off.
      (Rendering|Material|SetScalarParameterValue (Variables|Flashlight|Data|GetFlashlightScreen) "EmissiveLevel" 0.0 :!class /Script/Engine.MaterialInstanceDynamic) ; Reset emissive effect to 0.
      (return) ; Done.
    )))

(fn GetFlashlightMaterial
  (bind _returnvalue (Rendering|Material|CreateDynamicMaterialInstance (Variables|Flashlight|Components|GetFlashlight) 1 "/Game/SGT/Materials/Flashlight/M_SGT_ScreenMat.M_SGT_ScreenMat" "None" :!class /Script/Engine.PrimitiveComponent)) ; Create a dynamic version of the material used for the light part of the flashlight.
  (Variables|Flashlight|Data|SetFlashlightScreen _returnvalue) ; Save instance as reference for later use.
  (return) ; Done.
)

(fn SetNewEquipment
  (params (Selection :type E_SGT_EquipmentType%20Enum :default "NewEnumerator0") (NewParam :type Skeletal%20Mesh%20Object%20Reference))
  (LocalVariables|SetNewMesh NewParam)
  (switch Utilities|FlowControl|Switch|SwitchonE_SGT_EquipmentType Selection
    (:NewEnumerator0
      (Variables|MeshReferences|SetBagSK (LocalVariables|GetNewMesh)))
    (:NewEnumerator8
      (Variables|MeshReferences|SetHeadSK (LocalVariables|GetNewMesh)))
    (:NewEnumerator1
      (Variables|MeshReferences|SetTorsoSK (LocalVariables|GetNewMesh)))
    (:NewEnumerator4
      (Variables|MeshReferences|SetLHandSK (LocalVariables|GetNewMesh)))
    (:NewEnumerator2
      (Variables|MeshReferences|SetLLegSK (LocalVariables|GetNewMesh)))
    (:NewEnumerator3
      (Variables|MeshReferences|SetLFootSK (LocalVariables|GetNewMesh)))
    (:NewEnumerator5
      (Variables|MeshReferences|SetRHandSK (LocalVariables|GetNewMesh)))
    (:NewEnumerator6
      (Variables|MeshReferences|SetRLegSK (LocalVariables|GetNewMesh)))
    (:NewEnumerator7
      (Variables|MeshReferences|SetRFootSK (LocalVariables|GetNewMesh)))))

(fn OnRepRFootSK
  (Class|SkinnedMeshComponent|SetSkeletalMesh (Variables|CharacterMeshes|GetE_RightFoot) (Variables|MeshReferences|GetRFootSK) true)
  (Class|SkinnedMeshComponent|SetMasterPoseComponent (Variables|CharacterMeshes|GetE_RightFoot) (Variables|Character|GetMesh) false))

(fn OnRepRLegSK
  (Class|SkinnedMeshComponent|SetSkeletalMesh (Variables|CharacterMeshes|GetE_RightLeg) (Variables|MeshReferences|GetRLegSK) true)
  (Class|SkinnedMeshComponent|SetMasterPoseComponent (Variables|CharacterMeshes|GetE_RightLeg) (Variables|Character|GetMesh) false))

(fn OnRepRHandSK
  (Class|SkinnedMeshComponent|SetSkeletalMesh (Variables|CharacterMeshes|GetE_RightHand) (Variables|MeshReferences|GetRHandSK) true)
  (Class|SkinnedMeshComponent|SetMasterPoseComponent (Variables|CharacterMeshes|GetE_RightHand) (Variables|Character|GetMesh) false))

(fn OnRepLFootSK
  (Class|SkinnedMeshComponent|SetSkeletalMesh (Variables|CharacterMeshes|GetE_LeftFoot) (Variables|MeshReferences|GetLFootSK) true)
  (Class|SkinnedMeshComponent|SetMasterPoseComponent (Variables|CharacterMeshes|GetE_LeftFoot) (Variables|Character|GetMesh) false))

(fn OnRepLLegSK
  (Class|SkinnedMeshComponent|SetSkeletalMesh (Variables|CharacterMeshes|GetE_LeftLeg) (Variables|MeshReferences|GetLLegSK) true)
  (Class|SkinnedMeshComponent|SetMasterPoseComponent (Variables|CharacterMeshes|GetE_LeftLeg) (Variables|Character|GetMesh) false))

(fn OnRepLHandSK
  (Class|SkinnedMeshComponent|SetSkeletalMesh (Variables|CharacterMeshes|GetE_LeftHand) (Variables|MeshReferences|GetLHandSK) true)
  (Class|SkinnedMeshComponent|SetMasterPoseComponent (Variables|CharacterMeshes|GetE_LeftHand) (Variables|Character|GetMesh) false))

(fn OnRepTorsoSK
  (Class|SkinnedMeshComponent|SetSkeletalMesh (Variables|CharacterMeshes|GetE_Torso) (Variables|MeshReferences|GetTorsoSK) true)
  (Class|SkinnedMeshComponent|SetMasterPoseComponent (Variables|CharacterMeshes|GetE_Torso) (Variables|Character|GetMesh) false))

(fn OnRepHeadSK
  (Class|SkinnedMeshComponent|SetSkeletalMesh (Variables|CharacterMeshes|GetE_Head) (Variables|MeshReferences|GetHeadSK) true)
  (Class|SkinnedMeshComponent|SetMasterPoseComponent (Variables|CharacterMeshes|GetE_Head) (Variables|Character|GetMesh) false))

(fn OnRepBagSK
  (Class|SkinnedMeshComponent|SetSkeletalMesh (Variables|CharacterMeshes|GetE_Bag) (Variables|MeshReferences|GetBagSK) true)
  (Class|SkinnedMeshComponent|SetMasterPoseComponent (Variables|CharacterMeshes|GetE_Bag) (Variables|Character|GetMesh) false))

(fn HideMeshforPlayer
  (params (Hide? :type Boolean))
  (bind _mesh (Variables|Character|GetMesh))
  (LocalVariables|SetState Hide?)
  (Class|PrimitiveComponent|SetOwnerNoSee _mesh (LocalVariables|GetState))
  (for _array_element (Components|GetChildrenComponents _mesh true)
    (bind _asstatic_mesh_component (Utilities|Casting|CastToStaticMeshComponent _array_element)
      (:then
        (Class|PrimitiveComponent|SetOwnerNoSee _asstatic_mesh_component (LocalVariables|GetState)))
      (:CastFailed
        (bind _asskeletal_mesh_component (Utilities|Casting|CastToSkeletalMeshComponent _array_element))
        (Class|PrimitiveComponent|SetOwnerNoSee _asskeletal_mesh_component (LocalVariables|GetState))))))

(fn GetActorMeshComponent
  (return (Variables|Character|GetMesh)))

(fn GetAim
  (return (Variables|Character|Data|Movement|GetIsAiming)))

(fn GetCamera
  (return (Variables|Character|Components|Camera|GetPlayerCamera) (Variables|Character|Components|Camera|GetCameraBoom) (Variables|Character|Components|Camera|GetCameraCollision)))

(fn GetCrouch
  (return (Variables|Character|Data|Movement|GetIsCrouching)))

(fn GetEquipmentMesh
  (params (Type :type E_SGT_EquipmentType%20Enum :default "NewEnumerator0"))
  ;[1 1 1] EQUIPMENT ENUM REF
  (switch Utilities|FlowControl|Switch|SwitchonE_SGT_EquipmentType Type
    (:NewEnumerator0
      (return (Variables|MeshReferences|GetBagSK)))
    (:NewEnumerator8
      (return (Variables|MeshReferences|GetHeadSK)))
    (:NewEnumerator1
      (return (Variables|MeshReferences|GetTorsoSK)))
    (:NewEnumerator4
      (return (Variables|MeshReferences|GetLHandSK)))
    (:NewEnumerator2
      (return (Variables|MeshReferences|GetLLegSK)))
    (:NewEnumerator3
      (return (Variables|MeshReferences|GetLFootSK)))
    (:NewEnumerator5
      (return (Variables|MeshReferences|GetRHandSK)))
    (:NewEnumerator6
      (return (Variables|MeshReferences|GetRLegSK)))
    (:NewEnumerator7
      (return (Variables|MeshReferences|GetRFootSK)))))

(fn GetHeadLocation
  (return (Variables|Character|Components|Head|GetPlayerHeadLocation)))

(fn GetLifeState
  (return (Variables|Character|Data|GetIsDead)))

(fn GetLootable
  (return (Variables|Character|GetLootableInventory)))

(fn GetName
  (return "Some Dead Guy"))

(fn GetPlayerMesh
  (return (Variables|Character|GetMesh)))

(fn GetProne
  (return (Variables|Character|Data|Movement|GetIsProne)))

(fn GetViewMode
  (return (Variables|Character|GetIsFirstPerson)))

(fn ParseCrouchAnimState
  (return (Variables|Character|Data|Movement|GetCrouchAnimDone)))

(fn ParseFlashlightState
  (return (Variables|Flashlight|Data|GetFlashlightOn)))

(fn ParseProneAnimState
  (return (Variables|Character|Data|Movement|GetProneAnimDone)))