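; Main menu controller that sets up the front-end menu screen when play begins.
; BeginPlay runs Initialize, which clears existing widgets, adds W_SGT_MainMenu to the viewport, and focuses it in game-and-UI input with the mouse locked and cursor visible.
; It then calls DestroySession on itself, so any existing online session is torn down on arrival at the menu.
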(event EventBeginPlay
  (CallFunction|Initialize)
  (|DestroySession self))

(fn ConstructionScript)

(fn Initialize
  (Viewport|RemoveAllWidgets) ; Remove any pre-existing widgets.
  (bind _returnvalue (UserInterface|CreateWidget "/Game/SGT/Blueprints/MainMenu/W_SGT_MainMenu.W_SGT_MainMenu_C" (Game|GetPlayerController 0))) ; Create the main menu widget.
  (UserInterface|Viewport|AddtoViewport _returnvalue 0) ; Add the main menu to the current viewport.
  (Input|SetInputModeGameandUI (Game|GetPlayerController 0) _returnvalue "LockAlways" false)
  (Variables|/Script/Engine.PlayerController|SetbShowMouseCursor (Game|GetPlayerController 0) true) ; Display the mouse cursor.
  (return))