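; AI loot component that gives its owning actor a lootable inventory, generated only on the server.
; It uses either a supplied inventory or random DT_SGT_LootTable rows matching its spawner class via game mode data, re-rolling failed spawn-chance checks.
; Items go into a hidden spawned SGT_Container, set as the owner's lootable.
; After the loot lifetime, a timer destroys the container, retrying each second while it is open.
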(event Custom|GenerateLoot
  (params (RandomizeLoot? :type Boolean) (SetInventory :type Array%20of%20Str%20SGT%20Inventory%20Entry%20Structures))
  (CallFunction|MakeAILoot RandomizeLoot? SetInventory) ; Make the loot for this actor.
)

(event Custom|RemoveLoot
  (bind _state (Class|BPIntContainer|GetIsOpen(Message) (Variables|LootGenerationSettings|GetLootContainer)))
  (if _state
    (Utilities|Time|SetTimerbyFunctionName 0 "RemoveLoot" 1.0) ; Setup timer to check after loot lifetime if loot can be removed from world.
    (else
      (Actor|DestroyActor (Variables|LootGenerationSettings|GetLootContainer)))))

(fn MakeAILoot
  (params (RandomizeLoot? :type Boolean) (SetInventory :type Array%20of%20Str%20SGT%20Inventory%20Entry%20Structures))
  (LocalVariables|SetRandomizeLoot RandomizeLoot?) ; Store input for cleaner use.
  (LocalVariables|SetInventoryToUse SetInventory) ; Store input for cleaner use.
  (if (Ability|HasAuthority (Components|GetOwner)) ; Ensure this is running on the server.
    (if (LocalVariables|GetRandomizeLoot) ; Do we want to randomize loot for this AI?
      (bind _spawnerlootdata (Class|BPIntGameMode|GetSpawnerData(Message) (Game|GetGameMode))) ; Retrieve spawner data from game mode.
      (bind _array_element (Utilities|Array|ForEachLoopwithBreak _spawnerlootdata :!label _label) ; For each entry inthe spawner loot data array...
        (:LoopBody
          (if (Utilities|Enum|Equal(Enum) (.SpawnerClass (Utilities|Struct|BreakStr_SGT_LootTableIDs _array_element)) (Variables|LootGenerationSettings|GetSpawnerClass)) ; Does the current array element match\nthis spawner's class?
            (Variables|LootGenerationSettings|SetLootIDs (.RowIDs (Utilities|Struct|BreakStr_SGT_LootTableIDs _array_element))) ; Update the loot IDs.
            (goto _label Break)))
        (:Completed
          (Variables|LootGenerationSettings|SetItemCount (Math|Random|RandomIntegerinRange (Variables|LootGenerationSettings|GetMinimumItems) (Variables|LootGenerationSettings|GetMaximumItems))) ; Store randomly generated loot\nquantity for cleaner use.
          (Variables|LootGenerationSettings|SetLootCount (- (Utilities|Array|Length (Variables|LootGenerationSettings|GetLootIDs)) 1)) ; Store number of loot items that match\nthis spawner class for cleaner use.
          (for _index (range 1 (Variables|LootGenerationSettings|GetItemCount)) ; For each loot item that needs to be spawned...
            (bind _outrownames (DataTable|GetDataTableRowNames "/Game/SGT/Blueprints/Data/DT_SGT_LootTable.DT_SGT_LootTable" :!label _label_2)) ; Retrieve the data table rows from the spawner loot table...
            (bind _returnvalue (Utilities|GetDataTableRow "/Game/SGT/Blueprints/Data/DT_SGT_LootTable.DT_SGT_LootTable" (Utilities|Array|Get(acopy) _outrownames (Utilities|Array|Get(acopy) (Variables|LootGenerationSettings|GetLootIDs) (Math|Random|RandomIntegerinRange 1 (Variables|LootGenerationSettings|GetLootCount))))) ; Pick a random item matching this loot spawner class and retrieve data from data table...
              (:then
                (if (> (.ChanceToSpawn (Utilities|Struct|BreakStr_SGT_LootTable _returnvalue)) (Math|Random|RandomFloat)) ; Randomise percent and check against\nchance to spawn. Should we spawn this\nitem?
                  (Utilities|Array|Add (Variables|LootGenerationSettings|GetInventory) (Utilities|Struct|MakeStr_SGT_InventoryEntry (.Item (Utilities|Struct|BreakStr_SGT_LootTable _returnvalue)) (Math|Random|RandomIntegerinRange 1 (.MaximumQuantity (Utilities|Struct|BreakStr_SGT_LootTable _returnvalue))) 1.0)) ; Add to the container inventory.
                  (else
                    (goto _label_2))))
              (:RowNotFound
                (goto _label_2))))
          (bind _returnvalue_2 (Game|SpawnActorfromClass "/Game/SGT/Blueprints/Actors/SGT_Container.SGT_Container_C" (Math|Transform|MakeTransform "0.000000,0.000000,0.000000") "Undefined" 0 0 :!label _label_3)) ; Spawn an invisible container to hold the player's loot.
          (bind _output_get (Variables|LootGenerationSettings|SetLootContainer _returnvalue_2)) ; Update reference to loot container.
          (Rendering|SetActorHiddenInGame _output_get true) ; Ensure that loot container is hidden in game.
          (Utilities|Time|SetTimerbyFunctionName 0 "RemoveLoot" (Variables|LootGenerationSettings|GetLootLifetime)) ; Setup timer to check after loot lifetime if loot can be removed from world.
          (Default|UpdateInventory (Variables|LootGenerationSettings|GetLootContainer) (Variables|LootGenerationSettings|GetInventory)) ; Update loot container inventory.
          (Class|BPIntCharacter|SetLootable(Message) (Components|GetOwner) (Variables|LootGenerationSettings|GetLootContainer)) ; Set the lootable object for the character.
          (return) ; Done.
        ))
      (else
        (Variables|LootGenerationSettings|SetInventory (LocalVariables|GetInventoryToUse)) ; Use manually set inventory for lootable inventory.
        (goto _label_3)))
    (else
      (return) ; Done.
    )))