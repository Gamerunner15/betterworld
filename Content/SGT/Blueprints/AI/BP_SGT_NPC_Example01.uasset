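; Example SGT enemy NPC that chases and shoots players, displays its health as text, and ragdolls with generated loot on death.
; PawnSensing moves it toward seen pawns; within range, a forward eye trace confirms a living character before delayed shots deal damage through message calls.
; A looping timer recolors the head's dynamic material by target and attack state.
; Mostly stubbed getters expose life, aim, mesh and loot state.
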(event OnSeePawn(PawnSensing)
  (params (Pawn :type Pawn%20Object%20Reference))
  ;[1 1 1] AI sense player by sight logic.
  (if (not (Variables|AISettings|GetIsDead)) ; Is the AI still alive?
    (Variables|AISettings|SetSensedPawn Pawn) ; Store data for cleaner use.
    (if (not (Utilities|Array|ContainsItem (Variables|AISettings|GetDeadPlayers) (Variables|AISettings|GetSensedPawn))) ; Is the sensed pawn already dead?
      (if (Variables|AISettings|GetAttacking) ; Is the NPC already attacking?
        (if (< (Transformation|GetDistanceTo (Variables|AISettings|GetSensedPawn)) 6e+02) ; Is the sensed pawn within 600 units?
          (bind (_playerfound_ _player) (CallFunction|EyeTrace :!label _label)) ; Can this AI see a player?
          (if _playerfound_ ; Was a player spotted?
            (Variables|AISettings|SetPlayer _player) ; Set reference to player for use.
            (Components|Movement|StopMovementImmediately (Variables|Character|GetCharacterMovement)) ; Stop actor from moving.
            (CallFunction|FireWeapon) ; Fire weapon at player.
            (Variables|AISettings|SetAttacking true) ; Update attacking state bool.
          )
          (else
            (AI|Navigation|SimpleMovetoActor (Pawn|GetController) (Variables|AISettings|GetSensedPawn) :!label _label_2) ; Move towards the sensed pawn.
            (if (< (Transformation|GetDistanceTo (Variables|AISettings|GetSensedPawn)) 6e+02) ; Is the sensed pawn within 600 units?
              (goto _label))))
        (else
          (goto _label_2))))))

(event Custom|Die
  ;[1 1 1] Kill AI character and set to ragdoll.
  (Physics|SetSimulatePhysics (Variables|Character|GetMesh) true) ; Enable ragdoll.
  (Class|PrimitiveComponent|WakeAllRigidBodies (Variables|Character|GetMesh)) ; Wake up all rigid bodies for better interaction with dead bodies.
  (Collision|SetCollisionEnabled (Variables|Collision|GetCapsuleComponent) "NoCollision") ; Disable capsule collision for better interaction with dead bodies.
  (Variables|AISettings|SetIsDead true) ; Set dead state.
)

(event Custom|UpdateHealth
  (params (Value :type Float%20%28double-precision%29))
  (Rendering|Components|TextRender|SetText (Variables|AISettings|GetTextRender) (Utilities|Text|ToText(Float) Value "HalfToEven")) ; Update health text render.
)

(event Custom|WeaponShot
  (bind _weapon (Variables|AISettings|GetWeapon))
  ;[1 1 1] Visual weapon fire event.
  (Niagara|SpawnSystematLocation "/Game/SGT/Effects/ParticleSystems/P_SGT_GunMuzzleFlare.P_SGT_GunMuzzleFlare" (Transformation|GetSocketLocation _weapon "Muzzle") (Transformation|GetWorldRotation _weapon))
  (Audio|PlaySoundatLocation "/Game/SGT/Sounds/Weapons/S_SGT_Weapons_ShotgunFire.S_SGT_Weapons_ShotgunFire" (Transformation|GetWorldLocation (Variables|AISettings|GetWeapon)) "0, 0, 0" 1.0 1.0 0.0 0 0 0 0) ; Play gunshot sound.
)

(event Custom|FireWeapon
  (bind _player (Variables|AISettings|GetPlayer))
  (bind (_ascharacter _bsuccess) (Utilities|Casting|CastToCharacter _player))
  ;[1 1 1] Fire weapon, spawn muzzle flash, apply damage and check for player death.
  (Utilities|FlowControl|Delay 0.5) ; Delay weapon fire event.
  (if (Variables|AISettings|GetAttacking) ; Ensure the NPC is still set to attacking\nafter delay.
    (CallFunction|WeaponShot) ; Shoot weapon.
    (if _bsuccess
      (Class|BPIntCharacter|DamageEvent(Message) _ascharacter 15.0 "/Script/Engine.DamageType") ; Call character damage event.
      (bind _isdead (Class|BPintController|GetLifeState(Message) (Pawn|GetController _ascharacter))) ; Retrieve character life state.
      (if _isdead ; Is the character dead?
        (Variables|AISettings|SetAttacking false) ; Update attackig state bool.
      ))))

(event EventSetLootable
  (params (Lootable :type SGT%20Container%20Object%20Reference))
  (Variables|AISettings|SetLootableInventory Lootable) ; Set character's lootable inventory.
)

(event EventDamageEvent
  (params (Amount :type Float%20%28double-precision%29) (Type :type Damage%20Type%20Class%20Reference))
  (Game|Damage|ApplyDamage self Amount 0 0 Type) ; Apply input damage amount and type to NPC.
)

(event Game|Damage|EventAnyDamage
  (params (Damage :type Float%20%28single-precision%29) (DamageType :type Damage%20Type%20Object%20Reference) (InstigatedBy :type Controller%20Object%20Reference) (DamageCauser :type Actor%20Object%20Reference))
  ;[1 1 1] Receive damage event.
  (bind _output_get (Variables|AISettings|SetHealth (- (Variables|AISettings|GetHealth) Damage))) ; Update health.
  (CallFunction|UpdateHealth _output_get)
  (if (<= (Variables|AISettings|GetHealth) 0.0) ; Is this AI out of health?
    (CallFunction|Die) ; Call death event.
    (Default|GenerateLoot (Variables|AISettings|GetBP_AI_RNGLootComponent) (Variables|AISettings|GetGenerateRandomLoot) (Variables|AISettings|GetInventory))))

(event EventBeginPlay
  ;[1 1 1] Event begin play.
  (CallFunction|Initialize) ; Initialize AI Actor.
  (Rendering|Components|TextRender|SetText (Variables|AISettings|GetTextRender) (Utilities|Text|ToText(Float) (Variables|AISettings|GetHealth) "HalfToEven")) ; Set initial health value as text render text.
)

(fn ConstructionScript)

(fn EyeTrace
  (bind _eyes (Variables|AISettings|GetEyes))
  (bind _returnvalue (Transformation|GetWorldLocation _eyes))
  (bind _outhit (Collision|LineTraceByChannel _returnvalue (+ _returnvalue (* (Transformation|GetActorForwardVector self) (Variables|AISettings|GetVisionRange))) "TraceTypeQuery1" false 0 "None")) ; Trace from eyes to point defined by forward vector and range.
  (bind _ascharacter (Utilities|Casting|CastToCharacter (.HitActor (Collision|BreakHitResult _outhit))) ; Is the actor hit a character?
    (:then
      (bind _isdead (Class|BPintController|GetLifeState(Message) (Pawn|GetController _ascharacter))) ; Retrieve the life state from the character's controller.
      (if _isdead ; Is this character alive?
        _
        (else
          (return true (.HitActor (Collision|BreakHitResult _outhit))) ; Done.
        )))
    (:CastFailed
      _))
  (return false 0) ; Done.
)

(fn UpdateMaterial
  (Utilities|IsValid (Variables|AISettings|GetPlayer) ; Is there a valid player?
    (:Is%20Valid
      (if (Variables|AISettings|GetAttacking) ; Is this actor attacking?
        (Rendering|Material|SetVectorParameterValue (Variables|AISettings|GetNPCMaterial) "Color" "(R=1.000000,G=0.000000,B=0.000000,A=1.000000)" :!class /Script/Engine.MaterialInstanceDynamic) ; Set body color to red.
        (else
          (Rendering|Material|SetVectorParameterValue (Variables|AISettings|GetNPCMaterial) "Color" "(R=1.000000,G=1.000000,B=0.000000,A=1.000000)" :!class /Script/Engine.MaterialInstanceDynamic) ; Set bodycolor to yellow.
        )))
    (:Is%20Not%20Valid
      (Rendering|Material|SetVectorParameterValue (Variables|AISettings|GetNPCMaterial) "Color" "(R=0.183480,G=1.000000,B=0.000000,A=1.000000)" :!class /Script/Engine.MaterialInstanceDynamic) ; Set bodycolor to green.
    ))
  (return) ; Done.
)

(fn Initialize
  (bind _returnvalue (Rendering|Material|CreateDynamicMaterialInstance (Variables|AISettings|GetHead) 0 "/Game/SGT/Materials/Character/Parents/M_SGT_Mannequin_Head.M_SGT_Mannequin_Head" "None" :!class /Script/Engine.PrimitiveComponent)) ; Retrieve dynamic instance of NPC head material.
  (Variables|AISettings|SetNPCMaterial _returnvalue) ; Store a reference to the dynamic material.
  (Utilities|Time|SetTimerbyFunctionName 0 "UpdateMaterial" 0.05 true) ; Start material update timer.
  (return) ; Done.
)

(fn GetActorMeshComponent
  (return (Variables|Character|GetMesh)))

(fn GetAim
  (return (Variables|AISettings|GetAttacking)))

(fn GetCamera
  (return 0 0 0))

(fn GetCrouch
  (return false))

(fn GetEquipmentMesh
  (params (Type :type E_SGT_EquipmentType%20Enum :default "NewEnumerator0"))
  (return 0))

(fn GetHeadLocation
  (return 0))

(fn GetLifeState
  (return (Variables|AISettings|GetIsDead)))

(fn GetLootable
  (return (Variables|AISettings|GetLootableInventory)))

(fn GetName
  (return ""))

(fn GetPlayerMesh
  (return 0))

(fn GetProne
  (return false))

(fn GetViewMode
  (return false))

(fn ParseCrouchAnimState
  (return false))

(fn ParseFlashlightState
  (return false))

(fn ParseProneAnimState
  (return false))