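; Player health manager component that handles damage, healing, decay, regeneration and death, initialized with a PlayerController.
; Looping timers drive server-only decay, delayed regeneration and optional fall checks, which apply damage based on drop height.
; Incoming damage is scaled by the inventory manager's armor impact when that system is enabled.
; Health changes feed UpdateHealth, which toggles the low-health effect, updates the HUD manager and tells the controller to kill the player at zero.
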(event Custom|Decay
  ;[1 0.2 0.2 0.5] Lower the player health by 1/5 of the health drain (happens 5x a second).
  (Utilities|SwitchHasAuthority ; Ensure this only runs on the server.
    (:Authority
      (Variables|HealthSettings|SetPlayerHealth (Math|Float|Clamp(Float) (- (Variables|HealthSettings|GetPlayerHealth) (/ (Variables|HealthSettings|GetHealthDrain) 5.0)) 0.0 (Variables|HealthSettings|GetMaxPlayerHealth))) ; Update health value.
      (HealthSystem|UpdateHealth) ; Run health update.
    )))

(event Custom|SetDecay
  (params (NewAmount :type Float%20%28single-precision%29))
  ;[1 0.2 0.2 0.5] Adjust health drain amount to incorporate new input.
  (Variables|HealthSettings|SetHealthDrain (+ (Variables|HealthSettings|GetHealthDrain) NewAmount)) ; Update health drain.
  (HealthSystem|CheckDrain) ; Run health drain update.
)

(event Custom|TakeDamage
  (params (Amount :type Float%20%28single-precision%29))
  ;[1 0.2 0.2 0.5] Lower health by damage amount.
  (Utilities|Time|ClearTimerbyFunctionName 0 "Regeneration") ; Ensure regeneration is turned off.
  (CallFunction|DamageEvent Amount) ; Execute damage event.
  (Utilities|FlowControl|RetriggerableDelay (Variables|HealthSettings|GetRegenerationDelay)) ; Start regen delay everytime damage is received.
  (bind _isdead (Class|BPintController|GetLifeState(Message) (Variables|HealthSettings|GetPlayerController))) ; Retrieve current life state from the controller.
  (if (and (not _isdead) (Variables|HealthSettings|GetRegenerativeHealth)) ; Is the player still alive AND is health\nregeneration enabled?
    (Utilities|Time|SetTimerbyFunctionName 0 "Regeneration" 1.0 true) ; Start health regen loop.
  ))

(event Custom|UpdateHUD
  (params (Health :type Float%20%28single-precision%29))
  (bind _hudmanager (Variables|HealthSettings|GetHUDManager))
  ;[0.2 1 0.2 0.5] Update player HUD.
  (Utilities|IsValid _hudmanager ; Is the HUD manager valid?
    (:Is%20Valid
      (Variables|/Game/SGT/Blueprints/Components/C_Manager-HUD.C_Manager-HUD_C|SetHealth _hudmanager Health) ; Update player HUD.
    )))

(event Custom|FallCheck
  ;[1 0.2 0.2 0.5] Check for player falling.
  (Utilities|SwitchHasAuthority ; Ensure this only runs on the server.
    (:Authority
      (FallingDamage|CheckforFall) ; Determine if player is falling.
    )))

(event Custom|AddHealth
  (params (AmountToAdd :type Float%20%28single-precision%29))
  ;[1 0.2 0.2 0.5] Take input health and add to current health, clamping within max.
  (Variables|HealthSettings|SetPlayerHealth (Math|Float|Clamp(Float) (+ (Variables|HealthSettings|GetPlayerHealth) AmountToAdd) 0.0 (Variables|HealthSettings|GetMaxPlayerHealth))) ; Update health value.
  (HealthSystem|UpdateHealth) ; Run health update.
)

(event Custom|ResetDecay
  ;[1 0.2 0.2 0.5] Disable health decay.
  (Variables|HealthSettings|SetHealthDrain 0.0) ; Update health drain.
  (HealthSystem|CheckDrain) ; Run health drain update.
)

(event Custom|Regeneration
  ;[1 0.2 0.2 0.5] Execute health regeneration sequence.
  (Utilities|SwitchHasAuthority ; Ensure this only runs on the server.
    (:Authority
      (if (not (Variables|HealthSettings|GetDecayActive)) ; Is health decay currently active?
        (if (< (Variables|HealthSettings|GetPlayerHealth) (Variables|HealthSettings|GetMaxPlayerHealth)) ; Is health regen required?
          (CallFunction|AddHealth (Variables|HealthSettings|GetRegenerationRate)) ; Add regen amount.
        )))))

(event EventInitialize
  (params (PlayerController :type Player%20Controller%20Object%20Reference))
  ;[0.2 1 0.2 0.5] Initialize health system.
  (bind _output_get (Variables|HealthSettings|SetPlayerController PlayerController)) ; Store a reference to the player controller.
  (bind _ascharacter (Utilities|Casting|CastToCharacter (Pawn|GetControlledPawn _output_get))) ; Check if the pawn is a derivative of the base character class.
  (Variables|HealthSettings|SetControlledChar _ascharacter) ; Set reference to base character class.
  (bind (_no_hud _hudcomponent _novisualeffects _visualeffectscomponent) (CallFunction|CommonComponents (Variables|HealthSettings|GetPlayerController) true false)) ; Retrieve common components from player controller.
  (if _no_hud ; Was there no HUD manager found?
    _
    (else
      (Variables|HealthSettings|SetHUDManager _hudcomponent) ; Set reference to HUD manager.
    ))
  (if _novisualeffects ; Was there no visual feedback manager\nfound in the player controller?
    (Variables|HealthSettings|SetLowHealthVisualEffect "NewEnumerator11") ; As no valid visual feedback manager was found,\nforce effect to none.
    (else
      (Variables|HealthSettings|SetVisualFeedbackManager _visualeffectscomponent) ; Set reference to Visual Feedback manager.
    ))
  (Variables|HealthSettings|SetPlayerHealth (Variables|HealthSettings|GetMaxPlayerHealth)) ; Ensure health is set to max on startup.
  (Variables|HealthSettings|SetHealthDrain 0.0) ; Ensure health drain is 0 on startup.
  (HealthSystem|UpdateHealth) ; Run health update.
  (HealthSystem|CheckDrain) ; Run health drain update.
  (if (Variables|FallingDamageSettings|GetEnableFallingDamage) ; Is falling damage enabled?
    (Utilities|Time|SetTimerbyFunctionName 0 "FallCheck" 0.05 true) ; Start falling check loop.
  )
  (if (Variables|HealthSettings|GetRegenerativeHealth) ; Is health regeneration enabled?
    (Utilities|Time|SetTimerbyFunctionName 0 "Regeneration" 1.0 true) ; Start health regen loop.
  ))

(event EventReset
  ;[0.2 1 0.2 0.5] Force reset prior to death.
  (Utilities|Time|ClearandInvalidateTimerbyHandle (Variables|HealthSettings|GetDecayTimer)) ; Force stop the decay timer.
  (Variables|HealthSettings|SetDecayActive false) ; Reset decay active state bool.
  (Variables|HealthSettings|SetPlayerHealth (Variables|HealthSettings|GetMaxPlayerHealth)) ; Reset player health level.
  (Variables|HealthSettings|SetHealthDrain 0.0) ; Reset health drain amount.
  (Utilities|Time|ClearTimerbyFunctionName 0 "Regeneration") ; Ensure regeneration is turned off.
)

(fn CheckforFall
  (bind _controlledchar (Variables|HealthSettings|GetControlledChar))
  (bind _charactermovement (Variables|/Script/Engine.Character|GetCharacterMovement _controlledchar))
  (if (and (Utilities|Enum|Equal(Enum) (Variables|/Script/Engine.CharacterMovementComponent|GetMovementMode _charactermovement) "MOVE_Falling") (< (.Z (Math|Vector|BreakVector (Variables|/Script/Engine.MovementComponent|GetVelocity _charactermovement))) 0.0)) ; Is the player falling both in state and direction?
    (if (Variables|FallingDamageSettings|GetIsFalling) ; Was the player already falling?
      _
      (else
        (Variables|FallingDamageSettings|SetFallStartZ (Utilities|GetCharZ)) ; Set starting Z value for fall.
        (Variables|FallingDamageSettings|SetIsFalling true) ; Set falling state to true.
      ))
    (return) ; Done.
    (elif (Variables|FallingDamageSettings|GetIsFalling) ; Was the player falling last time?
      (Variables|FallingDamageSettings|SetIsFalling false) ; Set falling state to false.
      (FallingDamage|CalcFallDamage) ; Calculate and apply falling damage.
      (return) ; Done.
      (else
        (return) ; Done.
      ))))

(fn CalcFallDamage
  (bind _output_get (LocalVariables|SetFallHeight (+ (- (Variables|FallingDamageSettings|GetFallStartZ) (Utilities|GetCharZ)) (Variables|FallingDamageSettings|GetFallHeightOffset)))) ; Update fall height.
  (if (> _output_get (Variables|FallingDamageSettings|GetSafeFallDistance)) ; Did the player fall enough to receive damage?
    (Game|Damage|ApplyDamage (Variables|HealthSettings|GetPlayerController) (* (/ (- (LocalVariables|GetFallHeight) (Variables|FallingDamageSettings|GetSafeFallDistance)) 1e+02) (Variables|FallingDamageSettings|GetFallDamageRate)) 0 0) ; Apply damage based on multiplier and fall distance.
    (return) ; Done.
    (else
      (return) ; Done.
    )))

(fn CheckDrain
  (if (Math|Float|NearlyEqual(Float) (Variables|HealthSettings|GetHealthDrain) 0.0 0.0005) ; Is the health drain currently equal or less than 5/1000ths of a unit?
    (Utilities|Time|ClearandInvalidateTimerbyHandle (Variables|HealthSettings|GetDecayTimer)) ; If yes, stop the health drain.
    (Variables|HealthSettings|SetDecayActive false) ; Update bool to reflect decay state.
    (return) ; Done.
    (elif (Variables|HealthSettings|GetDecayActive) ; Check if decay is already active.
      (return) ; Done.
      (else
        (Variables|HealthSettings|SetDecayActive true) ; Update bool to reflect decay state.
        (bind _returnvalue (Utilities|Time|SetTimerbyFunctionName 0 "Decay" 0.2 true)) ; Initiate health decay loop.
        (Variables|HealthSettings|SetDecayTimer _returnvalue) ; Store reference to timer for later use.
        (return) ; Done.
      ))))

(fn UpdateHealth
  (bind _playercontroller (Variables|HealthSettings|GetPlayerController))
  (Utilities|IsValid _playercontroller ; Is the player controller reference valid?
    (:Is%20Valid
      (bind _isdead (Class|BPintController|GetLifeState(Message) _playercontroller)) ; Return current life state of the player.
      (if _isdead ; Is the player dead?
        (return) ; Done.
        (else
          (CallFunction|UpdateVisualEffect) ; Run visual effect update.
          (CallFunction|UpdateHUD (/ (Variables|HealthSettings|GetPlayerHealth) (Variables|HealthSettings|GetMaxPlayerHealth))) ; Update player's HUD.
          (if (<= (Variables|HealthSettings|GetPlayerHealth) 0.0) ; Does the player have any health?
            (Variables|HealthSettings|SetHealthDrain 0.0) ; Reset health drain to 0.
            (Class|BPintController|SetKillPlayer(Message) (Variables|HealthSettings|GetPlayerController)) ; Trigger player death.
            (return)
            (else
              (return) ; Done.
            )))))
    (:Is%20Not%20Valid
      (return) ; Done.
    )))

(fn DamageEvent
  (params (DamageAmount :type Float%20%28single-precision%29))
  (LocalVariables|SetInputDamage DamageAmount) ; Store input damage for cleaner use.
  (bind _manager (Class|BPintController|GetInventory(Message) (Variables|HealthSettings|GetPlayerController))) ; Retrieve a reference the inventory manager.
  (Utilities|IsValid _manager ; Does the player controller have an inventory manager?
    (:Is%20Valid
      (if (Variables|/Game/SGT/Blueprints/Components/C_Manager-Inventory.C_Manager-Inventory_C|GetUseArmorSystem _manager) ; Are we supposed to consider armor?
        (bind _currentrating (Default|GetArmorImpact _manager)) ; Retrieve the armor rating impact.
        (LocalVariables|SetInputDamage (* _currentrating (LocalVariables|GetInputDamage))) ; Update the input damage after adjusting for armor.
      ))
    (:Is%20Not%20Valid
      _))
  (Variables|HealthSettings|SetPlayerHealth (- (Variables|HealthSettings|GetPlayerHealth) (LocalVariables|GetInputDamage))) ; Update health value.
  (HealthSystem|UpdateHealth) ; Run health update.
  (return) ; Done.
)

(fn UpdateVisualEffect
  (if (Utilities|Enum|NotEqual(Enum) (Variables|HealthSettings|GetLowHealthVisualEffect) "NewEnumerator11") ; Is a visual effect enabled?
    (if (Variables|HealthSettings|GetVisualEffectActive) ; Is the visual effect currently active?
      (if (<= (Variables|HealthSettings|GetPlayerHealth) (Variables|HealthSettings|GetVisualEffectThreshold)) ; Is the player's water below the visual effect threshold level?
        _
        (else
          (Default|EffectControl (Variables|HealthSettings|GetVisualFeedbackManager) (Variables|HealthSettings|GetLowHealthVisualEffect) true) ; Begin the sequence to turn the visual effect off.
          (Variables|HealthSettings|SetVisualEffectActive false) ; Update visual effect state bool.
          (return) ; Done.
        ))
      (elif (> (Variables|HealthSettings|GetPlayerHealth) (Variables|HealthSettings|GetVisualEffectThreshold)) ; Is the player's water above the visual effect threshold level?
        _
        (else
          (Default|EffectControl (Variables|HealthSettings|GetVisualFeedbackManager) (Variables|HealthSettings|GetLowHealthVisualEffect) false) ; Begin the sequence to turn the visual effect on.
          (Variables|HealthSettings|SetVisualEffectActive true) ; Update visual effect state bool.
          (return) ; Done.
        )))
    (return) ; Done.
    (else
      (return) ; Done.
    )))