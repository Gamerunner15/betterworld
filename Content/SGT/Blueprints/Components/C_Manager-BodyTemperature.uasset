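; Player controller component that tracks body temperature and applies heatstroke or hypothermia past set thresholds.
; Looping timers on the server drift temperature toward the TimeOfDay manager's world temperature or an active volume's temperature, and deal damage during extremes.
; UpdateTemperature switches states and drives the optional HUD, visual effect, stamina cap and thirst (heatstroke only) managers found at Initialize.
; State flags prevent stacking stamina and thirst modifiers.
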(event Custom|UpdateHUD
  (params (Temperature :type Float%20%28double-precision%29))
  (bind _hudmanager (Variables|BodyTemperatureSettings|GetHUDManager))
  ;[0.2 1 0.2 0.5] Update player HUD.
  (if (not (Variables|BodyTemperatureSettings|GetDisableSystem)) ; DEBUG: Is the body temperature\nsystem set to disabled?
    (Utilities|IsValid _hudmanager ; Is there a valid HUD manager?
      (:Is%20Valid
        (Variables|/Game/SGT/Blueprints/Components/C_Manager-HUD.C_Manager-HUD_C|SetTempBody _hudmanager Temperature) ; Update body temperature on HUD.
      ))))

(event Custom|VolumeTriggered
  (params (Temperature :type Float%20%28double-precision%29) (Delay :type Float%20%28double-precision%29) (Percent :type Float%20%28double-precision%29))
  ;[1 0.2 0.2 0.5] Triggered volume sequences.
  (if (not (Variables|BodyTemperatureSettings|GetDisableSystem)) ; DEBUG: Is the body temperature\nsystem set to disabled?
    (Variables|BodyTemperatureSettings|SetVolumeTemperature Temperature) ; Store input for cleaner use.
    (Variables|BodyTemperatureSettings|SetUpdateRatio Percent) ; Store input for cleaner use.
    (Variables|BodyTemperatureSettings|SetInVolume true) ; Set volume active state bool.
    (bind _returnvalue (Utilities|Time|SetTimerbyFunctionName 0 "VolumeUpdate" Delay true)) ; Initiate volume update timer.
    (Variables|BodyTemperatureSettings|SetVolumeTimer _returnvalue) ; Store a reference to the volume update timer for future cancellation.
  ))

(event Custom|RunUpdate
  ;[1 0.2 0.2 0.5] Initiate update timer to account for world temperature.
  (if (not (Variables|BodyTemperatureSettings|GetDisableSystem)) ; DEBUG: Is the body temperature\nsystem set to disabled?
    (Utilities|SwitchHasAuthority
      (:Authority
        (bind _returnvalue (Utilities|Time|SetTimerbyFunctionName 0 "UpdateTemperature" (/ 1.0 (Math|Conversions|ToFloat(Integer) (Variables|BodyTemperatureSettings|GetUpdateFrequency))) true)) ; Begin update loop.
        (Variables|BodyTemperatureSettings|SetUpdateTimer _returnvalue) ; Store reference to the update timer.
        (Variables|BodyTemperatureSettings|SetUpdateRunning true) ; Set update running state bool.
      ))))

(event Custom|AddHeat
  (params (AmoutToAdd :type Float%20%28double-precision%29))
  ;[1 0.2 0.2 0.5] Take input 'heat' and add to the current temperature.
  (if (not (Variables|BodyTemperatureSettings|GetDisableSystem)) ; DEBUG: Is the body temperature\nsystem set to disabled?
    (Variables|BodyTemperatureSettings|SetPlayerTemperature (+ (Variables|BodyTemperatureSettings|GetPlayerTemperature) AmoutToAdd)) ; Update body temperature.
  ))

(event Custom|ExtremeTemperatures
  ;[1 0.2 0.2 0.5] Apply appropriate damage based on heatstroke/hypothermia state.
  (if (not (Variables|BodyTemperatureSettings|GetDisableSystem)) ; DEBUG: Is the body temperature\nsystem set to disabled?
    (Utilities|SwitchHasAuthority ; Ensure this only runs on the server.
      (:Authority
        (if (Variables|HeatstrokeSettings|GetHeatstrokeActive) ; Is heatstroke active?
          (Game|Damage|ApplyDamage (Variables|BodyTemperatureSettings|GetPlayerController) (* (Variables|HeatstrokeSettings|GetDamage-Heatstroke) (/ 1.0 (Math|Conversions|ToFloat(Integer) (Variables|BodyTemperatureSettings|GetUpdateFrequency)))) 0 0 "/Game/SGT/Blueprints/Misc/Damage_Statistical.Damage_Statistical_C") ; Apply appropriate damage.
          (CallFunction|UpdateTemperature) ; Run temperature update.
          (elif (Variables|HypothermiaSettings|GetHypothermiaActive) ; Is hypothermia active?
            (Game|Damage|ApplyDamage (Variables|BodyTemperatureSettings|GetPlayerController) (* (Variables|HypothermiaSettings|GetDamage-Hypothermia) (/ 1.0 (Math|Conversions|ToFloat(Integer) (Variables|BodyTemperatureSettings|GetUpdateFrequency)))) 0 0 "/Game/SGT/Blueprints/Misc/Damage_Statistical.Damage_Statistical_C") ; Apply appropriate damage.
            (CallFunction|UpdateTemperature) ; Run temperature update.
            (else
              (Utilities|Time|ClearandInvalidateTimerbyHandle (Variables|BodyTemperatureSettings|GetExtremeTempTimer)) ; Cancel extreme temp timer.
            )))))))

(event Custom|VolumeStop
  ;[1 0.2 0.2 0.5] Triggered volume sequences.
  (if (not (Variables|BodyTemperatureSettings|GetDisableSystem)) ; DEBUG: Is the body temperature\nsystem set to disabled?
    (Variables|BodyTemperatureSettings|SetInVolume false) ; Set volume active state bool.
  ))

(event EventVolumeExit
  ;[1 0.2 0.2 0.5] End volume sequence.
  (if (not (Variables|BodyTemperatureSettings|GetDisableSystem)) ; DEBUG: Is the body temperature\nsystem set to disabled?
    (Utilities|SwitchHasAuthority ; Ensure this only runs on the server.
      (:Authority
        (CallFunction|VolumeStop) ; Stop the temperature volume loop.
      ))))

(event EventInitialize
  (params (PlayerController :type Player%20Controller%20Object%20Reference))
  ;[0.2 1 0.2 0.5] Initialize body temperature system.
  (if (not (Variables|BodyTemperatureSettings|GetDisableSystem)) ; DEBUG: Is the body temperature\nsystem set to disabled?
    (Variables|BodyTemperatureSettings|SetPlayerController PlayerController) ; Set reference to controller.
    (bind (_no_hud _hudcomponent _novisualeffects _visualeffectscomponent _nostamina _staminacomponent) (CallFunction|CommonComponents (Variables|BodyTemperatureSettings|GetPlayerController) (or (Utilities|Enum|NotEqual(Enum) (Variables|HeatstrokeSettings|GetVisualEffect-Heatstroke) "NewEnumerator11") (Utilities|Enum|NotEqual(Enum) (Variables|HypothermiaSettings|GetVisualEffect-Hypothermia) "NewEnumerator11")) (or (Variables|HeatstrokeSettings|GetLimitStamina-Heatstroke) (Variables|HypothermiaSettings|GetLimitStamina-Hypothermia)))) ; Retrieve common components from player controller.
    (if _no_hud ; Was there no HUD manager found?
      _
      (else
        (Variables|BodyTemperatureSettings|SetHUDManager _hudcomponent) ; Set reference to HUD manager.
      ))
    (if _novisualeffects ; Was there no visual feedback manager\nfound in the player controller?
      (Variables|HeatstrokeSettings|SetVisualEffect-Heatstroke "NewEnumerator11") ; As no valid visual feedback manager was found,\nforce effect to none.
      (Variables|HypothermiaSettings|SetVisualEffect-Hypothermia "NewEnumerator11") ; As no valid visual feedback manager was found,\nforce effect to none.
      (else
        (Variables|BodyTemperatureSettings|SetVisualFeedbackManager _visualeffectscomponent) ; Set reference to Visual Feedback manager.
      ))
    (if _nostamina ; Was there no stamina manager found\nin the player controller?
      (Variables|HeatstrokeSettings|SetLimitStamina-Heatstroke false) ; As no valid stamina manager exists,\nforce LimitStamina to false.
      (Variables|HypothermiaSettings|SetLimitStamina-Hypothermia false) ; As no valid stamina manager exists,\nforce LimitStamina to false.
      (else
        (Variables|BodyTemperatureSettings|SetStaminaManager _staminacomponent) ; Set reference to Stamina manager.
      ))
    (Utilities|IsValid (Actor|GetComponentbyClass (Variables|BodyTemperatureSettings|GetPlayerController) "/Game/SGT/Blueprints/Components/C_Manager-TimeOfDay.C_Manager-TimeOfDay_C") ; Does the player have a valide time of day\ncomponent attach to their controller?
      (:Is%20Valid
        (bind _output_get (Variables|BodyTemperatureSettings|SetTimeOfDayManager (Actor|GetComponentbyClass (Variables|BodyTemperatureSettings|GetPlayerController) "/Game/SGT/Blueprints/Components/C_Manager-TimeOfDay.C_Manager-TimeOfDay_C"))) ; Store reference to time of day manager.
        (Variables|BodyTemperatureSettings|SetUseWorldTemperature (Variables|/Game/SGT/Blueprints/Components/C_Manager-TimeOfDay.C_Manager-TimeOfDay_C|GetUseWorldTemperature _output_get)) ; Set world temperature use state bool.
      )
      (:Is%20Not%20Valid
        (Variables|BodyTemperatureSettings|SetUseWorldTemperature false) ; No time of day manager, thus no world temperature.
      ))
    (Utilities|IsValid (Actor|GetComponentbyClass (Variables|BodyTemperatureSettings|GetPlayerController) "/Game/SGT/Blueprints/Components/C_Manager-Thirst.C_Manager-Thirst_C") ; Does the player have a valid thirst\ncomponent attach to their controller?
      (:Is%20Valid
        (Variables|BodyTemperatureSettings|SetThirstManager (Actor|GetComponentbyClass (Variables|BodyTemperatureSettings|GetPlayerController) "/Game/SGT/Blueprints/Components/C_Manager-Thirst.C_Manager-Thirst_C")) ; Store reference to thirst manager.
        (Variables|HeatstrokeSettings|SetIncreaseThirst true) ; Update increase thirst state bool.
      )
      (:Is%20Not%20Valid
        (Variables|HeatstrokeSettings|SetIncreaseThirst false) ; Update increase thirst state bool.
      ))
    (Variables|BodyTemperatureSettings|SetPlayerTemperature (Variables|BodyTemperatureSettings|GetNormalTemperature)) ; Set initial player temperature.
    (if (Variables|BodyTemperatureSettings|GetUseWorldTemperature) ; Is world temperature meant to impact\nbody temperature?
      (CallFunction|RunUpdate) ; Run update for world temperature.
      (else
        (Variables|BodyTemperatureSettings|SetUpdateRunning false) ; Set update running state bool.
        (CallFunction|UpdateTemperature)))))

(event EventReset
  ;[0.2 1 0.2 0.5] Reset body temperature system
  (if (not (Variables|BodyTemperatureSettings|GetDisableSystem)) ; DEBUG: Is the body temperature\nsystem set to disabled?
    (Utilities|Time|ClearandInvalidateTimerbyHandle (Variables|BodyTemperatureSettings|GetUpdateTimer)) ; Force stop the update timer.
    (Utilities|Time|ClearandInvalidateTimerbyHandle (Variables|BodyTemperatureSettings|GetExtremeTempTimer)) ; Force stop the extreme temp timer.
    (Variables|BodyTemperatureSettings|SetUpdateRunning false) ; Reset update running state bool.
    (Variables|HeatstrokeSettings|SetHeatstrokeActive false) ; Reset heatstroke active state bool.
    (Variables|HypothermiaSettings|SetHypothermiaActive false) ; Reset hypothermia active state bool.
    (Variables|BodyTemperatureSettings|SetPlayerTemperature (Variables|BodyTemperatureSettings|GetNormalTemperature)) ; Reset player temperature value.
  ))

(event EventVolumeEvent
  (params (Temperature :type Float%20%28double-precision%29) (Delay :type Float%20%28double-precision%29) (Percent :type Float%20%28double-precision%29))
  ;[1 0.2 0.2 0.5] Volume triggered sequence.
  (if (not (Variables|BodyTemperatureSettings|GetDisableSystem)) ; DEBUG: Is the body temperature\nsystem set to disabled?
    (Utilities|SwitchHasAuthority ; Ensure this only runs on the server.
      (:Authority
        (CallFunction|VolumeTriggered Temperature Delay Percent) ; Trigger the temperature volume event.
      ))))

(fn UpdateTemperature
  (bind _playercontroller (Variables|BodyTemperatureSettings|GetPlayerController))
  (bind _hudmanager (Variables|BodyTemperatureSettings|GetHUDManager))
  (bind _hudmanager_2 (Variables|BodyTemperatureSettings|GetHUDManager))
  (Utilities|IsValid _playercontroller ; Valid player controller?
    (:Is%20Valid
      (bind _isdead (Class|BPintController|GetLifeState(Message) _playercontroller)) ; Get the current life state from the controller via interface.
      (if _isdead ; Is the player dead?
        (return) ; As player is dead, do nothing.
        (else
          (CallFunction|UpdateVisualEffect) ; Run visual effect update.
          (if (>= (Variables|BodyTemperatureSettings|GetPlayerTemperature) (Variables|HeatstrokeSettings|GetThreshold-Heatstroke)) ; Is the player temperature above the\nheatstroke threshold?
            (if (Variables|HeatstrokeSettings|GetHeatstrokeActive) ; Is heatstroke already active?
              _
              (else
                (CallFunction|ActivateExtremeTemp true)
                (Utilities|IsValid _hudmanager ; Is the HUD manager reference valid?
                  (:Is%20Valid
                    (Default|UpdateFeedback _hudmanager "You are overheating. Find a way to cooldown.") ; Provide feedback to player.
                  )
                  (:Is%20Not%20Valid
                    _))
                (if (Variables|HeatstrokeSettings|GetIncreaseThirst) ; Do we need to increase the player's thirst rate?
                  (CallFunction|AlterThirst (Variables|HeatstrokeSettings|GetIncreasedThirstRate)))))
            (if (Variables|HeatstrokeSettings|GetLimitStamina-Heatstroke) ; Should the player's stamina be limited if they are dehydrated?
              (CallFunction|LimitStamina true false))
            (elif (<= (Variables|BodyTemperatureSettings|GetPlayerTemperature) (Variables|HypothermiaSettings|GetThreshold-Hypothermia)) ; Is the player temperature below the\nhypothermia threshold?
              (if (Variables|HypothermiaSettings|GetHypothermiaActive) ; Is the player temperature below the\nhypothermia threshold?
                _
                (else
                  (CallFunction|ActivateExtremeTemp false)
                  (Utilities|IsValid _hudmanager_2 ; Is the HUD manager reference valid?
                    (:Is%20Valid
                      (Default|UpdateFeedback _hudmanager_2 "You are freezing. Find a way to heat up.") ; Provide feedback to player.
                    )
                    (:Is%20Not%20Valid
                      _))
                  (if (Variables|HypothermiaSettings|GetLimitStamina-Hypothermia) ; Should the player's stamina be limited if they are dehydrated?
                    (CallFunction|LimitStamina false true))))
              (else
                (if (Variables|HeatstrokeSettings|GetHeatstrokeActive) ; Is heatstroke already active?
                  (CallFunction|AlterThirst (- 0.0 (Variables|HeatstrokeSettings|GetIncreasedThirstRate))))
                (if (or (Variables|HypothermiaSettings|GetLimitStamina-Hypothermia) (Variables|HeatstrokeSettings|GetLimitStamina-Heatstroke)) ; Should the player's stamina be limited if they are dehydrated?
                  (CallFunction|LimitStamina false false))
                (Variables|HeatstrokeSettings|SetHeatstrokeActive false) ; Update heatstroke state bool.
                (Variables|HypothermiaSettings|SetHypothermiaActive false) ; Update hypothermia state bool.
              )))
          (if (Variables|BodyTemperatureSettings|GetInVolume) ; Is the player currently in a temperature volume?
            _
            (else
              (Variables|BodyTemperatureSettings|SetPlayerTemperature (+ (CallFunction|GetUpdateAmount) (Variables|BodyTemperatureSettings|GetPlayerTemperature))) ; Update player temperature.
            ))
          (CallFunction|UpdateHUD (Variables|BodyTemperatureSettings|GetPlayerTemperature)) ; Parse player temperature to the HUD manager.
          (return) ; Done.
        )))
    (:Is%20Not%20Valid
      (return) ; Done.
    )))

(fn GetUpdateAmount
  (if (Variables|BodyTemperatureSettings|GetUseWorldTemperature)
    (return (/ (* (- (Variables|/Game/SGT/Blueprints/Components/C_Manager-TimeOfDay.C_Manager-TimeOfDay_C|GetCurrentTemperature (Variables|BodyTemperatureSettings|GetTimeOfDayManager)) (Variables|BodyTemperatureSettings|GetPlayerTemperature)) (Variables|BodyTemperatureSettings|GetWorldTemperatureInfluence)) (Math|Conversions|ToFloat(Integer) (Variables|BodyTemperatureSettings|GetUpdateFrequency))))
    (else
      (return 0.0))))

(fn UpdateVisualEffect
  (if (or (Utilities|Enum|NotEqual(Enum) (Variables|HeatstrokeSettings|GetVisualEffect-Heatstroke) "NewEnumerator11") (Utilities|Enum|NotEqual(Enum) (Variables|HypothermiaSettings|GetVisualEffect-Hypothermia) "NewEnumerator11")) ; Is a visual effect enabled for either heatstroke or hypothermia?
    (if (Variables|HeatstrokeSettings|GetHeatstrokeVisualActive) ; Is the visual effect currently active?
      (if (>= (Variables|BodyTemperatureSettings|GetPlayerTemperature) (Variables|HeatstrokeSettings|GetThreshold-Heatstroke)) ; Is the player temperature above the\nheatstroke threshold?
        _
        (else
          (Default|EffectControl (Variables|BodyTemperatureSettings|GetVisualFeedbackManager) (Variables|HeatstrokeSettings|GetVisualEffect-Heatstroke) true) ; Begin the sequence to turn the visual effect off.
          (Variables|HeatstrokeSettings|SetHeatstrokeVisualActive false) ; Update visual effect state bool.
          (return) ; Done.
        ))
      (elif (Variables|HypothermiaSettings|GetHypothermiaVisualActive) ; Is the visual effect currently active?
        (if (<= (Variables|BodyTemperatureSettings|GetPlayerTemperature) (Variables|HypothermiaSettings|GetThreshold-Hypothermia)) ; Is the player temperature below the\nhypothermia threshold?
          _
          (else
            (Default|EffectControl (Variables|BodyTemperatureSettings|GetVisualFeedbackManager) (Variables|HypothermiaSettings|GetVisualEffect-Hypothermia) true) ; Begin the sequence to turn the visual effect off.
            (Variables|HypothermiaSettings|SetHypothermiaVisualActive false) ; Update visual effect state bool.
            (return) ; Done.
          ))
        (elif (and (> (Variables|BodyTemperatureSettings|GetPlayerTemperature) (Variables|HypothermiaSettings|GetThreshold-Hypothermia)) (< (Variables|BodyTemperatureSettings|GetPlayerTemperature) (Variables|HeatstrokeSettings|GetThreshold-Heatstroke))) ; Is the player temperature within safe\nlevels?
          (return) ; Done.
          (elif (>= (Variables|BodyTemperatureSettings|GetPlayerTemperature) (Variables|HeatstrokeSettings|GetThreshold-Heatstroke)) ; Is the player temperature above the\nheatstroke threshold?
            (Default|EffectControl (Variables|BodyTemperatureSettings|GetVisualFeedbackManager) (Variables|HeatstrokeSettings|GetVisualEffect-Heatstroke) false) ; Begin the sequence to turn the visual effect on.
            (Variables|HeatstrokeSettings|SetHeatstrokeVisualActive true) ; Update visual effect state bool.
            (return) ; Done.
            (elif (<= (Variables|BodyTemperatureSettings|GetPlayerTemperature) (Variables|HypothermiaSettings|GetThreshold-Hypothermia)) ; Is the player temperature below the\nhypothermia threshold?
              (Default|EffectControl (Variables|BodyTemperatureSettings|GetVisualFeedbackManager) (Variables|HypothermiaSettings|GetVisualEffect-Hypothermia) false) ; Begin the sequence to turn the visual effect on.
              (Variables|HypothermiaSettings|SetHypothermiaVisualActive true) ; Update visual effect state bool.
              (return) ; Done.
              (else
                (return) ; Done.
              ))))))
    (return) ; Done.
    (else
      (return) ; Done.
    )))

(fn ActivateExtremeTemp
  (params (Heatstroke? :type Boolean))
  (bind _output_get (Variables|HeatstrokeSettings|SetHeatstrokeActive Heatstroke?)) ; Update heatstroke state bool.
  (Variables|HypothermiaSettings|SetHypothermiaActive (not _output_get)) ; Update hypothermia state bool.
  (bind _returnvalue (Utilities|Time|SetTimerbyFunctionName 0 "ExtremeTemperatures" (/ 1.0 (Math|Conversions|ToFloat(Integer) (Variables|BodyTemperatureSettings|GetUpdateFrequency))) true)) ; Start the extreme temperatures timer.
  (Variables|BodyTemperatureSettings|SetExtremeTempTimer _returnvalue) ; Set a reference to the extreme temperatures timer.
  (return) ; Done.
)

(fn LimitStamina
  (params (Heatstroke? :type Boolean) (Hypothermia? :type Boolean))
  (if Heatstroke?
    (if (Variables|HypothermiaSettings|GetHypothermiaStaminaLimited) ; Is stamina already limited because of hypothermia?
      (Default|RaiseCap (Variables|BodyTemperatureSettings|GetStaminaManager) (Variables|HypothermiaSettings|GetStaminaReduction-Hypothermia)) ; Raise the player's stamina cap to ensure we don't double up on capping.
      (Variables|HypothermiaSettings|SetHypothermiaStaminaLimited false) ; Update limited stamina state bool.
    )
    (if (Variables|HeatstrokeSettings|GetHeatstrokeStaminaLimited) ; Is stamina already limited because of heatstroke?
      (return) ; Done.
      (else
        (Default|LowerCap (Variables|BodyTemperatureSettings|GetStaminaManager) (Variables|HeatstrokeSettings|GetStaminaReduction-Heatstroke)) ; Lower the player's stamina cap.
        (Variables|HeatstrokeSettings|SetHeatstrokeStaminaLimited true) ; Update limited stamina state bool.
        (return) ; Done.
      ))
    (elif Hypothermia?
      (if (Variables|HeatstrokeSettings|GetHeatstrokeStaminaLimited) ; Is stamina already limited because of heatstroke?
        (Default|RaiseCap (Variables|BodyTemperatureSettings|GetStaminaManager) (Variables|HeatstrokeSettings|GetStaminaReduction-Heatstroke)) ; Raise the player's stamina cap to ensure we don't double up on capping.
        (Variables|HeatstrokeSettings|SetHeatstrokeStaminaLimited false) ; Update limited stamina state bool.
      )
      (if (Variables|HypothermiaSettings|GetHypothermiaStaminaLimited) ; Is stamina already limited because of heatstroke?
        (return) ; Done.
        (else
          (Default|LowerCap (Variables|BodyTemperatureSettings|GetStaminaManager) (Variables|HypothermiaSettings|GetStaminaReduction-Hypothermia)) ; Lower the player's stamina cap.
          (Variables|HypothermiaSettings|SetHypothermiaStaminaLimited true) ; Update limited stamina state bool.
          (return) ; Done.
        ))
      (else
        (if (Variables|HypothermiaSettings|GetHypothermiaStaminaLimited) ; Is stamina already limited because of hypothermia?
          (Default|RaiseCap (Variables|BodyTemperatureSettings|GetStaminaManager) (Variables|HypothermiaSettings|GetStaminaReduction-Hypothermia)) ; Raise the player's stamina cap to ensure we don't double up on capping.
          (Variables|HypothermiaSettings|SetHypothermiaStaminaLimited false) ; Update limited stamina state bool.
        )
        (if (Variables|HeatstrokeSettings|GetHeatstrokeStaminaLimited) ; Is stamina already limited because of heatstroke?
          (Default|RaiseCap (Variables|BodyTemperatureSettings|GetStaminaManager) (Variables|HeatstrokeSettings|GetStaminaReduction-Heatstroke)) ; Raise the player's stamina cap to ensure we don't double up on capping.
          (Variables|HeatstrokeSettings|SetHeatstrokeStaminaLimited false) ; Update limited stamina state bool.
        )
        (return) ; Done.
      ))))

(fn AlterThirst
  (params (Amount :type Float%20%28double-precision%29))
  (bind _output_get (LocalVariables|SetInput Amount))
  (if (< _output_get 0.0)
    (if (Variables|HeatstrokeSettings|GetThirstIsIncreased) ; Is thirst currently increased?
      (Default|AddtoMultiplier (Variables|BodyTemperatureSettings|GetThirstManager) (LocalVariables|GetInput)) ; Reduce thirst multiplier.
      (Variables|HeatstrokeSettings|SetThirstIsIncreased false) ; Update thirst increased state bool.
      (return) ; Done.
      (else
        _))
    (elif (Variables|HeatstrokeSettings|GetThirstIsIncreased) ; Is thirst already increased?
      _
      (else
        (Default|AddtoMultiplier (Variables|BodyTemperatureSettings|GetThirstManager) (LocalVariables|GetInput)) ; Increase thirst multiplier.
        (Variables|HeatstrokeSettings|SetThirstIsIncreased true) ; Update thirst increased state bool.
        (return) ; Done.
      )))
  (return) ; Done.
)

(fn AddTemperature
  (params (Amount :type Float%20%28double-precision%29))
  (Utilities|FlowControl|DoN 20))

(fn VolumeUpdate
  (if (Variables|BodyTemperatureSettings|GetInVolume)
    (CallFunction|AddHeat (* (- (Variables|BodyTemperatureSettings|GetVolumeTemperature) (Variables|BodyTemperatureSettings|GetPlayerTemperature)) (Variables|BodyTemperatureSettings|GetUpdateRatio)))
    (return)
    (else
      (Utilities|Time|ClearandInvalidateTimerbyHandle (Variables|BodyTemperatureSettings|GetVolumeTimer))
      (return))))