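; SGT_Component is a component Blueprint with empty Initialize and Reset events, apparently a base for other gameplay components.
; Its CommonComponents function looks up manager components on the given player controller: HUD always, visual feedback and stamina only when requested.
; It returns each reference with a "No" flag, which is set when that manager is missing or, for the optional two, not requested.
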(event Custom|Reset)

(event Custom|Initialize
  (params (PlayerController :type Player%20Controller%20Object%20Reference)))

(fn CommonComponents
  (params (Player :type Player%20Controller%20Object%20Reference) (VisualEffectsRequired? :type Boolean) (StaminaRequired? :type Boolean))
  (LocalVariables|SetControllerReference Player) ; Store input controller for cleaner use.
  (LocalVariables|SetbNeedsVisual VisualEffectsRequired?) ; Store visual feedback manage\nrequirement for cleaner use.
  (LocalVariables|SetbNeedsStamina StaminaRequired?) ; Store stamina manager requirement\nfor cleaner use.
  (Utilities|IsValid (Actor|GetComponentbyClass (LocalVariables|GetControllerReference) "/Game/SGT/Blueprints/Components/C_Manager-HUD.C_Manager-HUD_C") ; Is there a valid HUD manager?
    (:Is%20Valid
      (LocalVariables|SetC_HUDManager (Actor|GetComponentbyClass (LocalVariables|GetControllerReference) "/Game/SGT/Blueprints/Components/C_Manager-HUD.C_Manager-HUD_C")) ; Store HUD manager reference.
    )
    (:Is%20Not%20Valid
      (LocalVariables|SetbNoHUDManager true)))
  (if (LocalVariables|GetbNeedsVisual) ; Is a reference to the visual feedback manager required?
    (Utilities|IsValid (Actor|GetComponentbyClass (LocalVariables|GetControllerReference) "/Game/SGT/Blueprints/Components/C_Manager-VisualFeedback.C_Manager-VisualFeedback_C") ; Is there a valid VisualFeedback manager?
      (:Is%20Valid
        (LocalVariables|SetC_VisualFeedbackManager (Actor|GetComponentbyClass (LocalVariables|GetControllerReference) "/Game/SGT/Blueprints/Components/C_Manager-VisualFeedback.C_Manager-VisualFeedback_C")) ; Store visual feedback manager reference.
      )
      (:Is%20Not%20Valid
        (LocalVariables|SetbNoVisualManager true :!label _label) ; No visual feedback manager found/needed.
      ))
    (else
      (goto _label)))
  (if (LocalVariables|GetbNeedsStamina) ; Is a reference to the stamina required?
    (Utilities|IsValid (Actor|GetComponentbyClass (LocalVariables|GetControllerReference) "/Game/SGT/Blueprints/Components/C_Manager-Stamina.C_Manager-Stamina_C") ; Is there a valid Stamina manager?
      (:Is%20Valid
        (LocalVariables|SetC_StaminaManager (Actor|GetComponentbyClass (LocalVariables|GetControllerReference) "/Game/SGT/Blueprints/Components/C_Manager-Stamina.C_Manager-Stamina_C")) ; Store stamina manager reference.
      )
      (:Is%20Not%20Valid
        (LocalVariables|SetbNoStaminaManager true :!label _label_2) ; No stamina manager found/needed.
      ))
    (else
      (goto _label_2)))
  (return (LocalVariables|GetbNoHUDManager) (LocalVariables|GetC_HUDManager) (LocalVariables|GetbNoVisualManager) (LocalVariables|GetC_VisualFeedbackManager) (LocalVariables|GetbNoStaminaManager) (LocalVariables|GetC_StaminaManager)) ; Done.
)