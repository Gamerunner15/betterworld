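; Thirst manager component that tracks a player's water, draining it over time and applying dehydration damage when empty.
; UpdateThirst switches between looping Decay and Dehydration timers, both server-only in effect, with drain scaled by an adjustable multiplier.
; It drives the HUD, an optional low-water visual effect and an optional stamina-cap reduction through sibling managers found on the player controller.
; AddWater and Reset restore water, and a debug flag disables the system's events.
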(event Custom|Dehydration
  ;[1 0.2 0.2 0.5] Apply damage to the player when they are dehydrated.
  (if (not (Variables|ThirstSettings|GetDisableSystem)) ; DEBUG: Is the thirst system set to\ndisabled?
    (Utilities|SwitchAuthority ; Ensure this only runs on server.
      (:Authority
        (Game|Damage|ApplyDamage (Variables|ThirstSettings|GetPlayerController) (* (Variables|ThirstSettings|GetDehydrationDamage) (/ 1.0 (Math|Conversions|ToFloat(Integer) (Variables|ThirstSettings|GetUpdateFrequency)))) 0 0 "/Game/SGT/Blueprints/Misc/Damage_Statistical.Damage_Statistical_C")))))

(event Custom|UpdateHUD
  (params (Water :type Float%20%28single-precision%29))
  (bind _hudmanager (Variables|ThirstSettings|GetHUDManager))
  ;[0.2 1 0.2 0.5] Update player HUD.
  (if (not (Variables|ThirstSettings|GetDisableSystem)) ; DEBUG: Is the thirst system set to\ndisabled?
    (Utilities|IsValid _hudmanager
      (:Is%20Valid
        (Variables|/Game/SGT/Blueprints/Components/C_Manager-HUD.C_Manager-HUD_C|SetWater _hudmanager Water) ; Update HUD.
      ))))

(event Custom|ResetMultiplier
  ;[1 0.2 0.2 0.5] Reset drain multiplier to 1.
  (if (not (Variables|ThirstSettings|GetDisableSystem)) ; DEBUG: Is the thirst system set to\ndisabled?
    (Variables|ThirstSettings|SetDrainMultiplier 1.0) ; Update drain multiplier value.
  ))

(event Custom|AddToMultiplier
  (params (Amount :type Float%20%28single-precision%29))
  ;[1 0.2 0.2 0.5] Add input amount to drain multiplier and set.
  (if (not (Variables|ThirstSettings|GetDisableSystem)) ; DEBUG: Is the thirst system set to\ndisabled?
    (Variables|ThirstSettings|SetDrainMultiplier (+ (Variables|ThirstSettings|GetDrainMultiplier) Amount)) ; Update drain multiplier value.
  ))

(event Custom|AddWater
  (params (AmountToAdd :type Float%20%28single-precision%29))
  ;[1 0.2 0.2 0.5] Take input water and add to the current water, clamping within max water.
  (if (not (Variables|ThirstSettings|GetDisableSystem)) ; DEBUG: Is the thirst system set to\ndisabled?
    (Variables|ThirstSettings|SetPlayerWater (Math|Float|Clamp(Float) (+ (Variables|ThirstSettings|GetPlayerWater) AmountToAdd) 0.0 (Variables|ThirstSettings|GetMaxPlayerWater))) ; Update water value.
    (CallFunction|UpdateThirst) ; Run thirst update.
  ))

(event Custom|Decay
  ;[1 0.2 0.2 0.5] Decay player water based on update frequency and drain rate.
  (if (not (Variables|ThirstSettings|GetDisableSystem)) ; DEBUG: Is the thirst system set to\ndisabled?
    (Utilities|SwitchAuthority ; Ensure this only runs on server.
      (:Authority
        (Variables|ThirstSettings|SetPlayerWater (Math|Float|Clamp(Float) (- (Variables|ThirstSettings|GetPlayerWater) (/ (* (Variables|ThirstSettings|GetDrainRate) (Variables|ThirstSettings|GetDrainMultiplier)) (Math|Conversions|ToFloat(Integer) (Variables|ThirstSettings|GetUpdateFrequency)))) 0.0 (Variables|ThirstSettings|GetMaxPlayerWater))) ; Update water value.
        (CallFunction|UpdateThirst) ; Run thirst update.
      ))))

(event EventInitialize
  (params (PlayerController :type Player%20Controller%20Object%20Reference))
  ;[0.2 1 0.2 0.5] Initialize thirst system.
  (if (not (Variables|ThirstSettings|GetDisableSystem)) ; DEBUG: Is the thirst system set to\ndisabled?
    (Variables|ThirstSettings|SetPlayerController PlayerController) ; Set reference to controller.
    (bind (_no_hud _hudcomponent _novisualeffects _visualeffectscomponent _nostamina _staminacomponent) (CallFunction|CommonComponents (Variables|ThirstSettings|GetPlayerController) (Utilities|Enum|NotEqual(Enum) (Variables|ThirstSettings|GetLowWaterVisualEffect) "NewEnumerator11") (Variables|ThirstSettings|GetLimitStamina))) ; Retrieve common components from player controller.
    (if _no_hud ; Was there no HUD manager found?
      _
      (else
        (Variables|ThirstSettings|SetHUDManager _hudcomponent) ; Set reference to HUD manager.
      ))
    (if _novisualeffects ; Was there no visual feedback manager\nfound in the player controller?
      (Variables|ThirstSettings|SetLowWaterVisualEffect "NewEnumerator11") ; As no valid visual feedback manager was found,\nforce effect to none.
      (else
        (Variables|ThirstSettings|SetVisualFeedbackManager _visualeffectscomponent) ; Set reference to Visual Feedback manager.
      ))
    (if _nostamina ; Was there no stamina manager found\nin the player controller?
      (Variables|ThirstSettings|SetLimitStamina false) ; As no valid stamina manager exists,\nforce LimitStamina to false.
      (else
        (Variables|ThirstSettings|SetStaminaManager _staminacomponent) ; Set reference to Stamina manager.
      ))
    (CallFunction|ResetMultiplier) ; Ensure multiplier is reset on startup.
    (Variables|ThirstSettings|SetPlayerWater (Variables|ThirstSettings|GetMaxPlayerWater)) ; Initialize water value.
    (CallFunction|UpdateThirst) ; Run thirst update.
  ))

(event EventReset
  ;[0.2 1 0.2 0.5] Reset thirst system.
  (if (not (Variables|ThirstSettings|GetDisableSystem)) ; DEBUG: Is the thirst system set to\ndisabled?
    (Utilities|Time|ClearandInvalidateTimerbyHandle (Variables|ThirstSettings|GetDecayTimer)) ; Force stop decay timer.
    (Variables|ThirstSettings|SetDecayActive false) ; Reset decay active state bool.
    (Utilities|Time|ClearandInvalidateTimerbyHandle (Variables|ThirstSettings|GetDehydrationTimer)) ; Force stop dehydration timer.
    (Variables|ThirstSettings|SetIsDehydrated false) ; Reset dehydrated state bool.
    (CallFunction|ResetMultiplier) ; Ensure multiplier is reset on startup.
    (Variables|ThirstSettings|SetVisualEffectActive false) ; Reset visual effect state bool.
    (Variables|ThirstSettings|SetStaminaLimited false) ; Reset stamina limited state bool.
    (Variables|ThirstSettings|SetPlayerWater (Variables|ThirstSettings|GetMaxPlayerWater)) ; Reset water value.
  ))

(fn UpdateThirst
  (bind _playercontroller (Variables|ThirstSettings|GetPlayerController))
  (bind _hudmanager (Variables|ThirstSettings|GetHUDManager))
  (Utilities|IsValid _playercontroller ; Valid player controller?
    (:Is%20Valid
      (bind _isdead (Class|BPintController|GetLifeState(Message) _playercontroller)) ; Get the current life state from the controller via interface.
      (if _isdead ; Is the player dead?
        (return) ; As player is dead, do nothing.
        (elif (<= (Variables|ThirstSettings|GetPlayerWater) 0.0) ; Is the player out of water?
          (if (Variables|ThirstSettings|GetDecayActive) ; Is the decay loop currently active?
            (Utilities|Time|ClearandInvalidateTimerbyHandle (Variables|ThirstSettings|GetDecayTimer)) ; Stop the decay loop.
            (Variables|ThirstSettings|SetDecayActive false) ; Set decay loop boolean state.
            (Utilities|IsValid _hudmanager ; Is the HUD manager reference valid?
              (:Is%20Valid
                (Default|UpdateFeedback _hudmanager "You are dehydrated. Find some water.") ; Add feedback text for player.
              )
              (:Is%20Not%20Valid
                _)))
          (bind _returnvalue (Utilities|Time|SetTimerbyFunctionName 0 "Dehydration" (/ 1.0 (Math|Conversions|ToFloat(Integer) (Variables|ThirstSettings|GetUpdateFrequency))) true)) ; Start the dehydration loop.
          (Variables|ThirstSettings|SetDehydrationTimer _returnvalue) ; Store a reference to the dehydration timer.
          (Variables|ThirstSettings|SetIsDehydrated true) ; Set dehydrated state bool.
          (if (Variables|ThirstSettings|GetLimitStamina) ; Should the player's stamina be limited if they are dehydrated?
            (if (Variables|ThirstSettings|GetStaminaLimited)
              (return) ; Done.
              (else
                (Default|LowerCap (Variables|ThirstSettings|GetStaminaManager) (Variables|ThirstSettings|GetStaminaReduction)) ; Lower the player's stamina cap.
                (Variables|ThirstSettings|SetStaminaLimited true) ; Update limited stamina state bool.
                (return) ; Done.
              ))
            (else
              (return) ; Done.
            ))
          (else
            (CallFunction|UpdateVisualEffect) ; Run visual effect update.
            (if (Variables|ThirstSettings|GetDecayActive) ; Is the decay loop already active?
              (CallFunction|UpdateHUD (/ (Variables|ThirstSettings|GetPlayerWater) (Variables|ThirstSettings|GetMaxPlayerWater))) ; Update the player HUD.
              (return) ; Done.
              (else
                (if (Variables|ThirstSettings|GetIsDehydrated) ; Was the player previously dehydrated?
                  (Utilities|Time|ClearandInvalidateTimerbyHandle (Variables|ThirstSettings|GetDehydrationTimer)) ; Stop the dehydration update loop.
                  (Variables|ThirstSettings|SetIsDehydrated false) ; Set dehydrated state bool.
                  (if (Variables|ThirstSettings|GetStaminaLimited) ; Was the player's stamina previously limited?
                    (Default|RaiseCap (Variables|ThirstSettings|GetStaminaManager) (Variables|ThirstSettings|GetStaminaReduction)) ; Raise the stamina cap appropriately.
                    (Variables|ThirstSettings|SetStaminaLimited false) ; Update stamina limited bool.
                  ))
                (bind _returnvalue_2 (Utilities|Time|SetTimerbyFunctionName 0 "Decay" (/ 1.0 (Math|Conversions|ToFloat(Integer) (Variables|ThirstSettings|GetUpdateFrequency))) true)) ; Start the decay loop.
                (Variables|ThirstSettings|SetDecayTimer _returnvalue_2) ; Update reference to decay loop timer.
                (Variables|ThirstSettings|SetDecayActive true) ; Set decay loop boolean state.
                (return) ; Done.
              ))))))
    (:Is%20Not%20Valid
      (return) ; Done.
    )))

(fn UpdateVisualEffect
  (if (Utilities|Enum|NotEqual(Enum) (Variables|ThirstSettings|GetLowWaterVisualEffect) "NewEnumerator11") ; Is a visual effect enabled?
    (if (Variables|ThirstSettings|GetVisualEffectActive) ; Is the visual effect currently active?
      (if (<= (Variables|ThirstSettings|GetPlayerWater) (Variables|ThirstSettings|GetVisualEffectThreshold)) ; Is the player's water below the visual effect threshold level?
        _
        (else
          (Default|EffectControl (Variables|ThirstSettings|GetVisualFeedbackManager) (Variables|ThirstSettings|GetLowWaterVisualEffect) true) ; Begin the sequence to turn the visual effect off.
          (Variables|ThirstSettings|SetVisualEffectActive false) ; Update visual effect state bool.
          (return) ; Done.
        ))
      (elif (> (Variables|ThirstSettings|GetPlayerWater) (Variables|ThirstSettings|GetVisualEffectThreshold)) ; Is the player's water above the visual effect threshold level?
        _
        (else
          (Default|EffectControl (Variables|ThirstSettings|GetVisualFeedbackManager) (Variables|ThirstSettings|GetLowWaterVisualEffect) false) ; Begin the sequence to turn the visual effect on.
          (Variables|ThirstSettings|SetVisualEffectActive true) ; Update visual effect state bool.
          (return) ; Done.
        )))
    (return) ; Done.
    (else
      (return) ; Done.
    )))