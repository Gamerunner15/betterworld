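; Player blood manager component that handles bleeding, blood loss and hypotension.
; Armor-adjusted damage above a threshold can randomly start bleeding or raise its multiplier, until bandaging stops it.
; UpdateBlood switches looping timers: Bleed drains blood, and at zero Hypotension applies damage and optionally lowers the stamina cap, both ticks being authority-only.
; It also drives HUD and low-blood visual effects through managers found on the PlayerController.
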(event Custom|Bleed
  ;[1 0.2 0.2 0.5] Bleed loop.
  (if (not (Variables|BloodSettings|GetDisableSystem)) ; DEBUG: Is the blood system set to\ndisabled?
    (Utilities|SwitchHasAuthority ; Ensure this only runs on server.
      (:Authority
        (Variables|BloodSettings|SetPlayerBlood (Math|Float|Clamp(Float) (- (Variables|BloodSettings|GetPlayerBlood) (* (Variables|BloodSettings|GetMultiplier) (/ (Variables|BloodSettings|GetDrainRate) (Math|Conversions|ToFloat(Integer) (Variables|BloodSettings|GetUpdateFrequency))))) 0.0 (Variables|BloodSettings|GetMaxPlayerBlood))) ; Update food value.
        (CallFunction|UpdateBlood) ; Run blood update.
      ))))

(event Custom|BandageWounds
  ;[1 0.2 0.2 0.5] Stop bleeding on bandage item use.
  (if (not (Variables|BloodSettings|GetDisableSystem)) ; DEBUG: Is the blood system set to\ndisabled?
    (Utilities|SwitchHasAuthority ; Ensure this only runs on server.
      (:Authority
        (Variables|BloodSettings|SetIsBleeding false) ; Reset bleeding state bool.
        (Variables|BloodSettings|SetMultiplier 1) ; Reset bleeding multiplier to 1.
      ))))

(event Custom|TakeDamage
  (params (DamageAmount :type Float%20%28single-precision%29))
  ;[1 0.2 0.2 0.5] Damage event.
  (if (not (Variables|BloodSettings|GetDisableSystem)) ; DEBUG: Is the blood system set to\ndisabled?
    (CallFunction|DamageEvent DamageAmount)))

(event Custom|Hypotension
  ;[1 0.2 0.2 0.5] Hypotension loop.
  (if (not (Variables|BloodSettings|GetDisableSystem)) ; DEBUG: Is the blood system set to\ndisabled?
    (Utilities|SwitchHasAuthority ; Ensure this only runs on server.
      (:Authority
        (Game|Damage|ApplyDamage (Variables|BloodSettings|GetPlayerController) (* (Variables|BloodSettings|GetHypotensionDamage) (/ 1.0 (Math|Conversions|ToFloat(Integer) (Variables|BloodSettings|GetUpdateFrequency)))) 0 0 "/Game/SGT/Blueprints/Misc/Damage_Statistical.Damage_Statistical_C") ; Apply damage to player.
      ))))

(event Custom|UpdateHUD
  (params (Blood :type Float%20%28single-precision%29))
  (bind _hudmanager (Variables|BloodSettings|GetHUDManager))
  ;[0.2 1 0.2 0.5] Update player HUD.
  (if (not (Variables|BloodSettings|GetDisableSystem)) ; DEBUG: Is the blood system set to\ndisabled?
    (Utilities|IsValid _hudmanager ; Is the HUD manager valid?
      (:Is%20Valid
        (Variables|/Game/SGT/Blueprints/Components/C_Manager-HUD.C_Manager-HUD_C|SetBlood _hudmanager Blood) ; Update player HUD.
      ))))

(event Custom|AddBlood
  (params (AmmountToAdd :type Float%20%28single-precision%29))
  ;[1 0.2 0.2 0.5] Take input blood and add to the current blood, clamping within max blood.
  (if (not (Variables|BloodSettings|GetDisableSystem)) ; DEBUG: Is the blood system set to\ndisabled?
    (Variables|BloodSettings|SetPlayerBlood (Math|Float|Clamp(Float) (+ (Variables|BloodSettings|GetPlayerBlood) AmmountToAdd) 0.0 (Variables|BloodSettings|GetMaxPlayerBlood))) ; Update blood value.
    (CallFunction|UpdateBlood) ; Run blood update.
  ))

(event EventInitialize
  (params (PlayerController :type Player%20Controller%20Object%20Reference))
  ;[0.2 1 0.2 0.5] Initialize blood system.
  (if (not (Variables|BloodSettings|GetDisableSystem)) ; DEBUG: Is the blood system set to\ndisabled?
    (bind _output_get (Variables|BloodSettings|SetPlayerController PlayerController)) ; Set reference to controller.
    (bind (_no_hud _hudcomponent _novisualeffects _visualeffectscomponent _nostamina _staminacomponent) (CallFunction|CommonComponents _output_get (Utilities|Enum|NotEqual(Enum) (Variables|BloodSettings|GetLowBloodVisualEffect) "NewEnumerator11") (Variables|BloodSettings|GetLimitStamina))) ; Retrieve common components from player controller.
    (if _no_hud
      _
      (else
        (Variables|BloodSettings|SetHUDManager _hudcomponent) ; Set reference to HUD manager.
      ))
    (if _novisualeffects ; Was there no visual feedback manager\nfound in the player controller?
      (Variables|BloodSettings|SetLowBloodVisualEffect "NewEnumerator11") ; As no valid visual feedback manager was found,\nforce effect to none.
      (else
        (Variables|BloodSettings|SetVisualFeedbackManager _visualeffectscomponent) ; Set reference to Visual Feedback manager.
      ))
    (if _nostamina ; Was there no stamina manager found\nin the player controller?
      (Variables|BloodSettings|SetLimitStamina false) ; As no valid stamina manager exists,\nforce LimitStamina to false.
      (else
        (Variables|BloodSettings|SetStaminaManager _staminacomponent) ; Set reference to Stamina manager.
      ))
    (Variables|BloodSettings|SetPlayerBlood (Variables|BloodSettings|GetMaxPlayerBlood)) ; Initialize blood value.
    (Variables|BloodSettings|SetMultiplier 1) ; Initialize multiplier value.
    (Variables|BloodSettings|SetIsBleeding false) ; Initialize IsBleeding state bool.
    (CallFunction|UpdateHUD (/ (Variables|BloodSettings|GetPlayerBlood) (Variables|BloodSettings|GetMaxPlayerBlood))) ; Initialize player HUD.
  ))

(event EventReset
  ;[0.2 1 0.2 0.5] Force reset prior to death.
  (if (not (Variables|BloodSettings|GetDisableSystem)) ; DEBUG: Is the blood system set to\ndisabled?
    (Utilities|Time|ClearandInvalidateTimerbyHandle (Variables|BloodSettings|GetBleedingTimer)) ; Force stop the bleeding timer.
    (Variables|BloodSettings|SetBleedingActive false) ; Reset bleeding active state bool.
    (Utilities|Time|ClearandInvalidateTimerbyHandle (Variables|BloodSettings|GetHypotensionTimer)) ; Force stop hypotension timer.
    (Variables|BloodSettings|SetZeroBlood false) ; Reset zero blood state bool.
    (Variables|BloodSettings|SetVisualEffectActive false) ; Reset visual effect state bool.
    (Variables|BloodSettings|SetStaminaLimited false) ; Reset stamina limited state bool.
    (Variables|BloodSettings|SetPlayerBlood (Variables|BloodSettings|GetMaxPlayerBlood)) ; Reset blood value.
    (Variables|BloodSettings|SetMultiplier 1) ; Reset bleeding multiplier.
    (Variables|BloodSettings|SetIsBleeding false) ; Reset is bleeding state bool.
  ))

(fn DamageEvent
  (params (DamageAmount :type Float%20%28single-precision%29))
  (bind _hudmanager (Variables|BloodSettings|GetHUDManager))
  (LocalVariables|SetInputDamage DamageAmount) ; Store input damage for cleaner use.
  (if (== (Variables|BloodSettings|GetMultiplier) (Variables|BloodSettings|GetMaxMultiplier)) ; Is the player already at maximum blood loss rate?
    (return) ; Done.
    (else
      (bind _manager (Class|BPintController|GetInventory(Message) (Variables|BloodSettings|GetPlayerController)))
      (Utilities|IsValid _manager ; Does the player controller have an inventory manager?
        (:Is%20Valid
          (if (Variables|/Game/SGT/Blueprints/Components/C_Manager-Inventory.C_Manager-Inventory_C|GetUseArmorSystem _manager) ; Are we supposed to consider armor?
            (bind _currentrating (Default|GetArmorImpact _manager)) ; Retrieve the armor rating impact.
            (LocalVariables|SetInputDamage (* _currentrating (LocalVariables|GetInputDamage))) ; Update the input damage after adjusting for armor.
          ))
        (:Is%20Not%20Valid
          _))
      (if (>= (LocalVariables|GetInputDamage) (Variables|BloodSettings|GetMinimumDamage)) ; Does the damage received, after\nadjustment, exceed the minimum\nrequirement for bleeding consideration?
        (if (>= (Variables|BloodSettings|GetBleedChance) (Math|Random|RandomFloatinRange 0.0 1.0)) ; Is the RNG chance within the range?
          (Utilities|IsValid _hudmanager ; Is the HUD manager reference valid?
            (:Is%20Valid
              (Default|UpdateFeedback _hudmanager "You are losing blood.") ; Provide feedback to player.
            )
            (:Is%20Not%20Valid
              _))
          (if (Variables|BloodSettings|GetIsBleeding) ; Is the player already bleeding?
            (Variables|BloodSettings|SetMultiplier (Math|Integer|Clamp(Integer) (+ (Variables|BloodSettings|GetMultiplier) 1) 1 (Variables|BloodSettings|GetMaxMultiplier))) ; Increment multiplier by one.
            (return) ; Done.
            (else
              (Variables|BloodSettings|SetIsBleeding true) ; Update bleeding state bool.
              (CallFunction|UpdateBlood) ; Run blood system update.
              (return) ; Done.
            ))
          (else
            (return) ; Done.
          ))
        (else
          (return) ; Done.
        )))))

(fn UpdateBlood
  (bind _playercontroller (Variables|BloodSettings|GetPlayerController))
  (bind _hudmanager (Variables|BloodSettings|GetHUDManager))
  (Utilities|IsValid _playercontroller ; Is the player controller reference valid?
    (:Is%20Valid
      (bind _isdead (Class|BPintController|GetLifeState(Message) _playercontroller)) ; Return current life state of the player.
      (if _isdead ; Is the player dead?
        (return) ; Done.
        (elif (<= (Variables|BloodSettings|GetPlayerBlood) 0.0) ; Is the player's blood completely drained?
          (if (Variables|BloodSettings|GetBleedingActive) ; Is the player currently bleeding?
            (Utilities|Time|ClearandInvalidateTimerbyHandle (Variables|BloodSettings|GetBleedingTimer)) ; Stop the bleeding loop.
            (Variables|BloodSettings|SetBleedingActive false) ; Update bleeding active state bool.
            (elif (Variables|BloodSettings|GetZeroBlood) ; Is the player already in a zero blood state?
              (return) ; Done.
              (else
                _)))
          (bind _returnvalue (Utilities|Time|SetTimerbyFunctionName 0 "Hypotension" (/ 1.0 (Math|Conversions|ToFloat(Integer) (Variables|BloodSettings|GetUpdateFrequency))) true)) ; Start the hypotension loop.
          (Variables|BloodSettings|SetHypotensionTimer _returnvalue) ; Store reference to hypotension timer.
          (Variables|BloodSettings|SetZeroBlood true) ; Update zero blood state bool.
          (Utilities|IsValid _hudmanager ; Is the HUD manager reference valid?
            (:Is%20Valid
              (Default|UpdateFeedback _hudmanager "You are in a state of hypotension. Find blood!") ; Provide feedback to player.
            )
            (:Is%20Not%20Valid
              _))
          (if (Variables|BloodSettings|GetLimitStamina) ; Should the player's stamina be limited if they are at zero blood??
            (if (Variables|BloodSettings|GetStaminaLimited)
              (return) ; Done.
              (else
                (Default|LowerCap (Variables|BloodSettings|GetStaminaManager) (Variables|BloodSettings|GetStaminaReduction)) ; Lower the player's stamina cap.
                (Variables|BloodSettings|SetStaminaLimited true) ; Update limited stamina state bool.
                (return) ; Done.
              ))
            (else
              (return) ; Done.
            ))
          (else
            (CallFunction|UpdateVisualEffect) ; Run visual effect update.
            (if (Variables|BloodSettings|GetZeroBlood) ; Was the player previously at a zero blood state?
              (Utilities|Time|ClearandInvalidateTimerbyHandle (Variables|BloodSettings|GetHypotensionTimer)) ; Stop the hypotension update loop.
              (Variables|BloodSettings|SetZeroBlood false) ; Update zero blood state bool.
              (if (Variables|BloodSettings|GetStaminaLimited) ; Was the player's stamina previously limited?
                (Default|RaiseCap (Variables|BloodSettings|GetStaminaManager) (Variables|BloodSettings|GetStaminaReduction)) ; Raise the stamina cap appropriately.
                (Variables|BloodSettings|SetStaminaLimited false) ; Update stamina limited bool.
              ))
            (if (Variables|BloodSettings|GetIsBleeding) ; Should the player be bleeding at the moment?
              (if (Variables|BloodSettings|GetBleedingActive) ; Is the player currently bleeding?
                _
                (else
                  (bind _returnvalue_2 (Utilities|Time|SetTimerbyFunctionName 0 "Bleed" (/ 1.0 (Math|Conversions|ToFloat(Integer) (Variables|BloodSettings|GetUpdateFrequency))) true)) ; Start the bleeding timer.
                  (Variables|BloodSettings|SetBleedingTimer _returnvalue_2)
                  (Variables|BloodSettings|SetBleedingActive true) ; Update bleeding active state bool.
                ))
              (CallFunction|UpdateHUD (/ (Variables|BloodSettings|GetPlayerBlood) (Variables|BloodSettings|GetMaxPlayerBlood))) ; Update player's HUD.
              (return) ; Done.
              (elif (Variables|BloodSettings|GetBleedingActive) ; Is the player currently bleeding?
                (Utilities|Time|ClearandInvalidateTimerbyHandle (Variables|BloodSettings|GetBleedingTimer)) ; Stop the bleeding loop.
                (Variables|BloodSettings|SetBleedingActive false) ; Update bleeding active state bool.
                (return) ; Done.
                (else
                  (CallFunction|UpdateHUD (/ (Variables|BloodSettings|GetPlayerBlood) (Variables|BloodSettings|GetMaxPlayerBlood))) ; Update player's HUD.
                  (return) ; Done.
                )))))))
    (:Is%20Not%20Valid
      (return) ; Done.
    )))

(fn UpdateVisualEffect
  (if (Utilities|Enum|NotEqual(Enum) (Variables|BloodSettings|GetLowBloodVisualEffect) "NewEnumerator11") ; Is a visual effect enabled?
    (if (Variables|BloodSettings|GetVisualEffectActive) ; Is the visual effect currently active?
      (if (<= (Variables|BloodSettings|GetPlayerBlood) (Variables|BloodSettings|GetVisualEffectThreshold)) ; Is the player's blood below the visual effect threshold level?
        _
        (else
          (Default|EffectControl (Variables|BloodSettings|GetVisualFeedbackManager) (Variables|BloodSettings|GetLowBloodVisualEffect) true) ; Begin the sequence to turn the visual effect off.
          (Variables|BloodSettings|SetVisualEffectActive false) ; Update visual effect state bool.
          (return) ; Done.
        ))
      (elif (> (Variables|BloodSettings|GetPlayerBlood) (Variables|BloodSettings|GetVisualEffectThreshold)) ; Is the player's blood above the visual effect threshold level?
        _
        (else
          (Default|EffectControl (Variables|BloodSettings|GetVisualFeedbackManager) (Variables|BloodSettings|GetLowBloodVisualEffect) false) ; Begin the sequence to turn the visual effect on.
          (Variables|BloodSettings|SetVisualEffectActive true) ; Update visual effect state bool.
          (return) ; Done.
        )))
    (return) ; Done.
    (else
      (return) ; Done.
    )))