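; Flashlight manager component that toggles the controlled character's flashlight and optional chest light, with battery drain and low-power flicker.
; Toggles route to the server, push state to the character via messages and adjust the power manager's decay.
; Looping timers switch the light off at zero power and set LowPower below a threshold.
; Its OnRep counts calls toward random flicker intervals, keeping off periods about a third as long.
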(event Custom|FlickerCheck
  ;[1 0.2 0.2 0.5] Check if player is at low power, and if they are set LowPower bool to initiate flicker.
  (if (Variables|FlashlightSettings|GetUseFlicker) ; Is the flicker effect enabled?
    (if (<= (Variables|/Game/SGT/Blueprints/Components/C_Manager-Power.C_Manager-Power_C|GetPlayerPower (Variables|FlashlightSettings|GetPowerManager)) (Variables|FlashlightSettings|GetFlickerThreshold)) ; Does the player have low enough power to enable flicker?
      (Variables|FlashlightSettings|SetLowPower true) ; Enable low power and flicker.
      (else
        (Variables|FlashlightSettings|SetLowPower false) ; Disable low power and flicker.
      ))))

(event Custom|PowerCheck
  ;[1 0.2 0.2 0.5] If player's power hits 0, toggle the flashlight to off.
  (if (== (Variables|/Game/SGT/Blueprints/Components/C_Manager-Power.C_Manager-Power_C|GetPlayerPower (Variables|FlashlightSettings|GetPowerManager)) 0.0) ; Has the player got no power?
    (CallFunction|ToggleFlashlight) ; Toggle the flashlight off.
  ))

(event Custom|ToggleFlashlight
  ;[1 0.2 0.2 0.5] Toggle flashlight on/off.
  (CallFunction|FlashlightSwitch))

(event Custom|SRV_ToggleFlashlight
  ;[1 0.2 0.2 0.5] Toggle flashlight on/off.
  (CallFunction|FlashlightSwitch))

(event EventInitialize
  (params (PlayerController :type Player%20Controller%20Object%20Reference))
  ;[0.2 1 0.2 0.5] Initialize flashlight system.
  (bind _output_get (Variables|FlashlightSettings|SetPlayerController PlayerController)) ; Store a reference to the player controller.
  (bind _ascharacter (Utilities|Casting|CastToCharacter (Pawn|GetControlledPawn _output_get))) ; Check if the pawn is a derivative of the base character class.
  (Variables|FlashlightSettings|SetControlledChar _ascharacter) ; Set reference to base character class.
  (Utilities|IsValid (Actor|GetComponentbyClass (Variables|FlashlightSettings|GetPlayerController) "/Game/SGT/Blueprints/Components/C_Manager-Power.C_Manager-Power_C") ; Does the controller have a valid power manager?
    (:Is%20Valid
      (Variables|FlashlightSettings|SetPowerManager (Actor|GetComponentbyClass (Variables|FlashlightSettings|GetPlayerController) "/Game/SGT/Blueprints/Components/C_Manager-Power.C_Manager-Power_C")) ; Set reference to power manager component.
    )
    (:Is%20Not%20Valid
      _))
  (if (Variables|FlashlightSettings|GetUseFlashlight) ; Is the flashlight system enabled?
    (CallFunction|SetCharacterVariables) ; Update variables in the character blueprint based on developer input.
    (if (Variables|FlashlightSettings|GetShowFlashlightOnChest) ; Are players allowed to have the flashlight on their chest?
      (Variables|FlashlightSettings|SetShowChestLight true) ; Show the chest light.
      (else
        (Variables|FlashlightSettings|SetShowChestLight false :!label _label) ; Hide the chest light.
      ))
    (else
      (goto _label)))
  (CallFunction|UpdateChestLight) ; Run chest light update.
)

(fn SetCharacterVariables
  (Class|BPIntCharacter|SetFlashlightMat(Message) (Variables|FlashlightSettings|GetControlledChar) (Variables|FlashlightSettings|GetIntensity) (Variables|FlashlightSettings|GetEmissive)) ; Update material settings in character.
  (return) ; Done.
)

(fn OnRepLowPower
  (if (Variables|FlashlightSettings|GetLowPower) ; Is the character currently in Low Power mode?
    (if (Variables|FlashlightSettings|GetGotNextFlickerCount) ; Is the next flicker count calculated?
      (if (== (Variables|FlashlightSettings|GetCurrentFlickerCount) (Variables|FlashlightSettings|GetNextFlickerCount)) ; Is the current flickec count equal to the target count?
        (bind _state (Class|BPIntCharacter|ParseFlashlightState(Message) (Variables|FlashlightSettings|GetControlledChar))) ; Retrieve current flashlight state from character.
        (Class|BPIntCharacter|ToggleFlashlight(Message) (Variables|FlashlightSettings|GetControlledChar) (not _state)) ; Parse on/off state to character.
        (Variables|FlashlightSettings|SetGotNextFlickerCount false) ; Reset bool state to initiate recalculation.
        (return) ; Done.
        (else
          (Math|Integer|IncrementInt (Variables|FlashlightSettings|GetCurrentFlickerCount) ; If no, increment and set.
            (:%20%20
              (return) ; Done.
            ))))
      (else
        (bind _state_2 (Class|BPIntCharacter|ParseFlashlightState(Message) (Variables|FlashlightSettings|GetControlledChar))) ; Retrieve current flashlight state from character.
        (if _state_2 ; Is the flaslight on or off?
          (Variables|FlashlightSettings|SetNextFlickerCount (Math|Random|RandomIntegerinRange 0 (Variables|FlashlightSettings|GetFlickerRate))) ; Update next flicker count.
          (else
            (Variables|FlashlightSettings|SetNextFlickerCount (Math|Random|RandomIntegerinRange 0 (/ (Variables|FlashlightSettings|GetFlickerRate) 3))) ; Update next flicker count.
          ))
        (Variables|FlashlightSettings|SetCurrentFlickerCount 0) ; Reset current flicker count.
        (Variables|FlashlightSettings|SetGotNextFlickerCount true) ; Update bool reflecting count determined state.
        (return) ; Done.
      ))
    (else
      (return) ; Done.
    )))

(fn FlashlightSwitch
  (bind _powermanager (Variables|FlashlightSettings|GetPowerManager))
  (if (Ability|HasAuthority (Variables|FlashlightSettings|GetPlayerController)) ; Does this player have authority?
    (if (Variables|FlashlightSettings|GetFlashlightOn) ; Is the flashlight already on?
      (Variables|FlashlightSettings|SetFlashlightOn false) ; Set flashlight to OFF.
      (else
        (Utilities|IsValid _powermanager ; Does the controller have a power manager component?
          (:Is%20Valid
            (if (> (Variables|/Game/SGT/Blueprints/Components/C_Manager-Power.C_Manager-Power_C|GetPlayerPower _powermanager) 0.0) ; Does the player have any power left?
              _
              (else
                (return) ; Done.
              )))
          (:Is%20Not%20Valid
            _))
        (Variables|FlashlightSettings|SetFlashlightOn true) ; Set flashlight to ON.
      ))
    (Class|BPIntCharacter|ToggleFlashlight(Message) (Variables|FlashlightSettings|GetControlledChar) (Variables|FlashlightSettings|GetFlashlightOn)) ; Toggle the flashlight.
    (Utilities|IsValid (Variables|FlashlightSettings|GetPowerManager) ; Make sure player has a power manager component.
      (:Is%20Valid
        (if (Variables|FlashlightSettings|GetFlashlightOn) ; Is the flashlight on?
          (Default|SetDecay (Variables|FlashlightSettings|GetPowerManager) (Variables|FlashlightSettings|GetDrainRate)) ; Add to drain of power.
          (bind _returnvalue (Utilities|Time|SetTimerbyFunctionName 0 "PowerCheck" 0.05 true)) ; Check power levels on loop.
          (Variables|FlashlightSettings|SetPowerTest _returnvalue) ; Save reference to power level timer.
          (if (Variables|FlashlightSettings|GetUseFlicker) ; Is use flicker enabled?
            (bind _returnvalue_2 (Utilities|Time|SetTimerbyFunctionName 0 "FlickerCheck" 0.05 true)) ; Run flicker check to see if flicker needs to happen.
            (Variables|FlashlightSettings|SetFlickerTest _returnvalue_2) ; Save a reference to timer handle for later use.
            (return) ; Done.
            (else
              _))
          (else
            (Default|SetDecay (Variables|FlashlightSettings|GetPowerManager) (- 0.0 (Variables|FlashlightSettings|GetDrainRate))) ; Subtract to drain of power.
            (Utilities|Time|ClearandInvalidateTimerbyHandle (Variables|FlashlightSettings|GetFlickerTest)) ; Cancel the flicker test.
            (Utilities|Time|ClearandInvalidateTimerbyHandle (Variables|FlashlightSettings|GetPowerTest)) ; Cancel the power test.
          ))
        (return) ; Done.
      )
      (:Is%20Not%20Valid
        (return) ; Done.
      ))
    (else
      (CallFunction|SRVToggleFlashlight) ; Run again on the server.
      (return) ; Done.
    )))

(fn UpdateChestLight
  (Utilities|IsValid (Variables|FlashlightSettings|GetPlayerController) ; Ensure only local controller runs via validity check.
    (:Is%20Valid
      (Class|BPIntCharacter|ShowChestlight(Message) (Variables|FlashlightSettings|GetControlledChar) (Variables|FlashlightSettings|GetShowChestLight)) ; Parse chest flashlight state to character.
      (return) ; Done.
    )
    (:Is%20Not%20Valid
      (return) ; Done.
    )))