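; Player power manager component that handles a segmented power pool with instant costs, additions, continuous drain and delayed regeneration.
; Looping function timers run decay and recovery on authority only, at a shared update frequency.
; Recovery refills only to the top of the current partial segment and does not start from zero power.
; UpdatePower restarts or stops recovery and sends normalised power to the controller's HUD manager while the player is alive.
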(event Custom|UpdateHUD
  (params (Power :type Float%20%28double-precision%29))
  (bind _hudmanager (Variables|PowerSettings|GetHUDManager))
  ;[0.2 1 0.2 0.5] Update player HUD.
  (Utilities|IsValid _hudmanager ; Is the HUD manager valid?
    (:Is%20Valid
      (Variables|/Game/SGT/Blueprints/Components/C_Manager-HUD.C_Manager-HUD_C|SetPower _hudmanager Power))))

(event Custom|SetDecay
  (params (NewAmount :type Float%20%28double-precision%29))
  ;[1 0.2 0.2 0.5] Adjust power drain amount to incorporate new input.
  (Utilities|Time|ClearandInvalidateTimerbyHandle (Variables|PowerSettings|GetRecoveryTimer)) ; Stop the recovery loop.
  (Variables|PowerSettings|SetCellMaxCalculated false) ; Reset cell max calculated state.
  (Variables|PowerSettings|SetDelayCheck 0) ; Reset delay counter.
  (Variables|PowerSettings|SetPowerDrain (Math|Float|Clamp(Float) (+ (Variables|PowerSettings|GetPowerDrain) NewAmount) 0.0 1e+02)) ; Update power value.
  (CallFunction|DrainCheck) ; Run drain update.
)

(event Custom|Decay
  ;[1 0.2 0.2 0.5] Lower the player power by appropriate amount based on update frequency value.
  (Utilities|SwitchHasAuthority ; Ensure this only runs on the server.
    (:Authority
      (Variables|PowerSettings|SetPlayerPower (Math|Float|Clamp(Float) (- (Variables|PowerSettings|GetPlayerPower) (/ (Variables|PowerSettings|GetPowerDrain) (Math|Conversions|ToFloat(Integer) (Variables|PowerSettings|GetUpdateFrequency)))) 0.0 (Variables|PowerSettings|GetMaxPlayerPower))) ; Update power value.
      (CallFunction|UpdatePower) ; Run power update.
    )))

(event Custom|AddPower
  (params (AmountToAdd :type Float%20%28double-precision%29))
  ;[1 0.2 0.2 0.5] Take input power and add to the current power, clamping within max power.
  (Variables|PowerSettings|SetPlayerPower (Math|Float|Clamp(Float) (+ (Variables|PowerSettings|GetPlayerPower) AmountToAdd) 0.0 (Variables|PowerSettings|GetMaxPlayerPower))) ; Update power value.
  (CallFunction|UpdatePower) ; Run power update.
)

(event Custom|ResetDrain
  ;[1 0.2 0.2 0.5] Disable power drain.
  (Variables|PowerSettings|SetPowerDrain 0.0) ; Reset power drain to 0.
  (CallFunction|DrainCheck) ; Run drain update.
)

(event Custom|ConsumePower
  (params (Amount :type Float%20%28double-precision%29))
  ;[1 0.2 0.2 0.5] Lower power by input amount.
  (Utilities|Time|ClearandInvalidateTimerbyHandle (Variables|PowerSettings|GetRecoveryTimer)) ; Stop the recovery loop.
  (Variables|PowerSettings|SetCellMaxCalculated false) ; Reset cell max calculated state.
  (Variables|PowerSettings|SetDelayCheck 0) ; Reset delay counter.
  (Variables|PowerSettings|SetPlayerPower (Math|Float|Clamp(Float) (- (Variables|PowerSettings|GetPlayerPower) Amount) 0.0 (Variables|PowerSettings|GetMaxPlayerPower))) ; Update power value.
  (CallFunction|UpdatePower) ; Run power update.
)

(event Custom|Recover
  ;[1 0.2 0.2 0.5] Recover power.
  (Utilities|SwitchHasAuthority ; Ensure this only runs on the server.
    (:Authority
      (CallFunction|CalculateCellMax) ; Calculate the maximum power based on what cell is currently partially full.
      (if (> (Variables|PowerSettings|GetDelayCheck) (* (Variables|PowerSettings|GetRecoveryDelay) (Variables|PowerSettings|GetUpdateFrequency))) ; Has the recovery relay completed?
        (Variables|PowerSettings|SetPlayerPower (Math|Float|Clamp(Float) (+ (Variables|PowerSettings|GetPlayerPower) (/ (Variables|PowerSettings|GetRecoveryRate) (Math|Conversions|ToFloat(Integer) (Variables|PowerSettings|GetUpdateFrequency)))) 0.0 (Variables|PowerSettings|GetCellMax))) ; Update player power for recovery.
        (CallFunction|UpdatePower) ; Run power update.
        (if (>= (Variables|PowerSettings|GetPlayerPower) (Variables|PowerSettings|GetCellMax)) ; Has player power reached the max for this power cell?
          (Utilities|Time|ClearandInvalidateTimerbyHandle (Variables|PowerSettings|GetRecoveryTimer)) ; If yes, stop the recovery loop.
          (Variables|PowerSettings|SetCellMaxCalculated false) ; Reset variable for future use.
        )
        (else
          (Math|Integer|IncrementInt (Variables|PowerSettings|GetDelayCheck)) ; If no, increment delay by 1.
        )))))

(event EventInitialize
  (params (PlayerController :type Player%20Controller%20Object%20Reference))
  ;[0.2 1 0.2 0.5] Initialize power system.
  (bind _output_get (Variables|PowerSettings|SetPlayerController PlayerController)) ; Set reference to the player controller.
  (Utilities|IsValid (Actor|GetComponentbyClass _output_get "/Game/SGT/Blueprints/Components/C_Manager-HUD.C_Manager-HUD_C") ; Is there a valid HUD manager?
    (:Is%20Valid
      (Variables|PowerSettings|SetHUDManager (Actor|GetComponentbyClass _output_get "/Game/SGT/Blueprints/Components/C_Manager-HUD.C_Manager-HUD_C")) ; Set reference to HUD manager.
    )
    (:Is%20Not%20Valid
      _))
  (Variables|PowerSettings|SetPlayerPower (Variables|PowerSettings|GetMaxPlayerPower)) ; Set player power to max on startup.
  (Variables|PowerSettings|SetSegmentMultiplier (/ 1.0 (Math|Conversions|ToFloat(Integer) (Variables|PowerSettings|GetNumberOfSegments)))) ; Set segment multiplier.
  (CallFunction|SetSegments) ; Update segments.
  (CallFunction|UpdatePower) ; Run power update.
)

(event EventReset
  ;[0.2 1 0.2 0.5] Force reset prior to death.
  (Utilities|Time|ClearandInvalidateTimerbyHandle (Variables|PowerSettings|GetRecoveryTimer))
  (Utilities|Time|ClearandInvalidateTimerbyHandle (Variables|PowerSettings|GetDecayTimer))
  (Variables|PowerSettings|SetDecayActive false)
  (Variables|PowerSettings|SetPlayerPower (Variables|PowerSettings|GetMaxPlayerPower)))

(fn SetSegments
  (bind _widget (Default|ParseHUDWidget (Variables|PowerSettings|GetHUDManager))) ; Get the HUD widget.
  (Class|BPIntHUD|SetSegmentsCount(Message) _widget (Variables|PowerSettings|GetNumberOfSegments) 0.0) ; Update the segment count in the HUD widget.
  (return))

(fn CalculateCellMax
  (if (Variables|PowerSettings|GetCellMaxCalculated) ; Has this calc already been run this time?
    (return) ; Calc already run. Do nothing.
    (else
      (Variables|PowerSettings|SetCellMax (Math|Float|Clamp(Float) (* (+ (Math|Float|Truncate (* (Variables|PowerSettings|GetNumberOfSegments) (/ (Variables|PowerSettings|GetPlayerPower) (Variables|PowerSettings|GetMaxPlayerPower)))) 1) (* (Variables|PowerSettings|GetSegmentMultiplier) (Variables|PowerSettings|GetMaxPlayerPower))) 0.0 (Variables|PowerSettings|GetMaxPlayerPower))) ; Set max cell value.
      (Variables|PowerSettings|SetCellMaxCalculated true) ; Set variable to reflect calc-complete state.
      (return))))

(fn DrainCheck
  (if (Math|Float|NearlyEqual(Float) (Variables|PowerSettings|GetPowerDrain) 0.0 0.0005) ; Is the stamina drain currently equal or less than 5/1000ths of a unit?
    (Utilities|Time|ClearandInvalidateTimerbyHandle (Variables|PowerSettings|GetDecayTimer)) ; Stop the decay timer.
    (Variables|PowerSettings|SetDecayActive false) ; Update bool to reflect decay state.
    (if (== (Variables|PowerSettings|GetPlayerPower) 0.0) ; Is player power at 0?
      (return) ; Player has no power. Do not recover.
      (else
        (bind _returnvalue (Utilities|Time|SetTimerbyFunctionName 0 "Recover" (/ 1.0 (Math|Conversions|ToFloat(Integer) (Variables|PowerSettings|GetUpdateFrequency))) true)) ; Initiate power recover loop.
        (Variables|PowerSettings|SetRecoveryTimer _returnvalue) ; Store reference to timer for later use.
        (return)))
    (elif (Variables|PowerSettings|GetDecayActive) ; Check if decay is already active.
      (return) ; Decay already active. No further action needed.
      (else
        (Variables|PowerSettings|SetDecayActive true) ; Update bool to reflect decay state.
        (Utilities|Time|ClearandInvalidateTimerbyHandle (Variables|PowerSettings|GetRecoveryTimer)) ; Stop the recovery timer.
        (Variables|PowerSettings|SetDelayCheck 0) ; Reset the delay counter.
        (bind _returnvalue_2 (Utilities|Time|SetTimerbyFunctionName 0 "Decay" (/ 1.0 (Math|Conversions|ToFloat(Integer) (Variables|PowerSettings|GetUpdateFrequency))) true)) ; Initiate power decay loop.
        (Variables|PowerSettings|SetDecayTimer _returnvalue_2) ; Store reference to timer for later use.
        (return)))))

(fn UpdatePower
  (bind _playercontroller (Variables|PowerSettings|GetPlayerController))
  (if (== (Variables|PowerSettings|GetPlayerPower) 0.0) ; Is the player power at 0?
    (Utilities|Time|ClearandInvalidateTimerbyHandle (Variables|PowerSettings|GetRecoveryTimer)) ; Stop the recovery loop.
    (return) ; As no power, don't recover.
    (else
      (Utilities|IsValid _playercontroller ; Is the controller valid?
        (:Is%20Valid
          (bind _isdead (Class|BPintController|GetLifeState(Message) _playercontroller)) ; Retrieve player life state.
          (if _isdead ; Is the player dead?
            (return) ; As player is dead, do nothing.
            (else
              (CallFunction|UpdateHUD (/ (Variables|PowerSettings|GetPlayerPower) (Variables|PowerSettings|GetMaxPlayerPower))) ; Update player's HUD.
              (if (<= (Variables|PowerSettings|GetPlayerPower) 0.0) ; Does the player have any power left?
                (return)
                (elif (< (Variables|PowerSettings|GetPlayerPower) (Variables|PowerSettings|GetMaxPlayerPower)) ; Is the player's power full?
                  (bind _returnvalue (Utilities|Time|SetTimerbyFunctionName 0 "Recover" (/ 1.0 (Math|Conversions|ToFloat(Integer) (Variables|PowerSettings|GetUpdateFrequency))) true)) ; Initiate power recover loop.
                  (Variables|PowerSettings|SetRecoveryTimer _returnvalue) ; Store a reference to the handle for use.
                  (return)
                  (else
                    (Utilities|Time|ClearandInvalidateTimerbyHandle (Variables|PowerSettings|GetRecoveryTimer)) ; Stop the recovery loop.
                    (return)))))))
        (:Is%20Not%20Valid
          (return) ; Done.
        )))))

(fn ParseHUDWidget
  (return 0))