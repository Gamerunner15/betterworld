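; Stamina manager component that tracks the controlled character's stamina, adjustable cap and exhausted state, with a debug switch to disable it.
; One-off consume and add events change stamina directly, while accumulated drain runs a looping Decay timer that replaces the Recover timer.
; Recovery waits out a delay and can slow while moving; both timer ticks apply only with authority.
; Updates push normalized stamina to the HUD manager.
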(event Custom|SetDecay
  (params (New%20Amount :type Float%20%28single-precision%29))
  ;[1 0.2 0.2 0.5] Adjust stamina drain amount to incorporate new input.
  (if (not (Variables|StaminaSettings|GetDisableSystem)) ; DEBUG: Is the stamina system set to\ndisabled?
    (Utilities|Time|ClearandInvalidateTimerbyHandle (Variables|StaminaSettings|GetRecoveryTimer)) ; Stop the recovery loop.
    (Variables|StaminaSettings|SetInRecovery false) ; Update recovery state boolean.
    (Variables|StaminaSettings|SetDelayCheck 0) ; Reset the delay counter.
    (Variables|StaminaSettings|SetStaminaDrain (Math|Float|Clamp(Float) (+ (Variables|StaminaSettings|GetStaminaDrain) New%20Amount) 0.0 1e+02)) ; Update stamina value.
    (CallFunction|CheckDrain) ; Run stamina drain update.
  ))

(event Custom|UpdateHUD
  (params (Stamina :type Float%20%28single-precision%29))
  (bind _hudmanager (Variables|StaminaSettings|GetHUDManager))
  ;[0.2 1 0.2 0.5] Update player HUD.
  (if (not (Variables|StaminaSettings|GetDisableSystem)) ; DEBUG: Is the stamina system set to\ndisabled?
    (Utilities|IsValid _hudmanager ; Is the HUD manager valid?
      (:Is%20Valid
        (Variables|/Game/SGT/Blueprints/Components/C_Manager-HUD.C_Manager-HUD_C|SetStamina _hudmanager Stamina) ; Convert player stamina to percentage and update HUD.
      ))))

(event Custom|ConsumeStamina
  (params (Amount :type Float%20%28single-precision%29))
  ;[1 0.2 0.2 0.5] Lower stamina by input amount.
  (if (not (Variables|StaminaSettings|GetDisableSystem)) ; DEBUG: Is the stamina system set to\ndisabled?
    (Utilities|Time|ClearandInvalidateTimerbyHandle (Variables|StaminaSettings|GetRecoveryTimer)) ; Stop the recovery loop.
    (Variables|StaminaSettings|SetInRecovery false) ; Update recovery state boolean.
    (Variables|StaminaSettings|SetDelayCheck 0) ; Reset the delay counter.
    (Variables|StaminaSettings|SetPlayerStamina (Math|Float|Clamp(Float) (- (Variables|StaminaSettings|GetPlayerStamina) Amount) 0.0 (Variables|StaminaSettings|GetStaminaCap))) ; Update stamina value.
    (CallFunction|UpdateStamina) ; Run stamina update.
  ))

(event Custom|Decay
  ;[1 0.2 0.2 0.5] Lower the player stamina by appropriate amount based on update frequency value.
  (if (not (Variables|StaminaSettings|GetDisableSystem)) ; DEBUG: Is the stamina system set to\ndisabled?
    (Utilities|SwitchHasAuthority ; Ensure this only runs on the server.
      (:Authority
        (Variables|StaminaSettings|SetPlayerStamina (Math|Float|Clamp(Float) (- (Variables|StaminaSettings|GetPlayerStamina) (/ (Variables|StaminaSettings|GetStaminaDrain) (Math|Conversions|ToFloat(Integer) (Variables|StaminaSettings|GetUpdateFrequency)))) 0.0 (Variables|StaminaSettings|GetStaminaCap))) ; Update stamina value.
        (CallFunction|UpdateStamina) ; Run stamina update.
      ))))

(event Custom|AddStamina
  (params (AmountToAdd :type Float%20%28single-precision%29))
  ;[1 0.2 0.2 0.5] Take input stamina and add to the current stamina, clamping within max stamina.
  (if (not (Variables|StaminaSettings|GetDisableSystem)) ; DEBUG: Is the stamina system set to\ndisabled?
    (Variables|StaminaSettings|SetPlayerStamina (Math|Float|Clamp(Float) (+ (Variables|StaminaSettings|GetPlayerStamina) AmountToAdd) 0.0 (Variables|StaminaSettings|GetStaminaCap))) ; Update stamina value.
    (CallFunction|UpdateStamina) ; Run stamina update.
  ))

(event Custom|ResetDrain
  ;[1 0.2 0.2 0.5] Disable stamina drain.
  (if (not (Variables|StaminaSettings|GetDisableSystem)) ; DEBUG: Is the stamina system set to\ndisabled?
    (Variables|StaminaSettings|SetStaminaDrain 0.0) ; Reset stamina drain to 0.
    (CallFunction|CheckDrain) ; Run stamina drain update.
  ))

(event Custom|LowerCap
  (params (Amount :type Float%20%28single-precision%29))
  ;[1 0.2 0.2 0.5] Lower the stamina cap by input amount.
  (if (not (Variables|StaminaSettings|GetDisableSystem)) ; DEBUG: Is the stamina system set to\ndisabled?
    (Variables|StaminaSettings|SetStaminaCap (- (Variables|StaminaSettings|GetStaminaCap) Amount)) ; Update stamina cap value.
    (CallFunction|CapStamina) ; Force stamina cap.
  ))

(event Custom|RaiseCap
  (params (Amount :type Float%20%28single-precision%29))
  ;[1 0.2 0.2 0.5] Raise the stamina cap by input amount.
  (if (not (Variables|StaminaSettings|GetDisableSystem)) ; DEBUG: Is the stamina system set to\ndisabled?
    (Variables|StaminaSettings|SetStaminaCap (+ (Variables|StaminaSettings|GetStaminaCap) Amount)) ; Update stamina cap value.
    (CallFunction|CapStamina) ; Force stamina cap.
    (CallFunction|UpdateStamina) ; Run stamina update.
  ))

(event Custom|ResetCap
  ;[1 0.2 0.2 0.5] Disable stamina cap.
  (if (not (Variables|StaminaSettings|GetDisableSystem)) ; DEBUG: Is the stamina system set to\ndisabled?
    (Variables|StaminaSettings|SetStaminaCap (Variables|StaminaSettings|GetMaxPlayerStamina)) ; Update stamina cap value.
    (CallFunction|CapStamina) ; Force stamina cap.
  ))

(event Custom|Recover
  ;[1 0.2 0.2 0.5] Recover stamina.
  (if (not (Variables|StaminaSettings|GetDisableSystem)) ; DEBUG: Is the stamina system set to\ndisabled?
    (Utilities|SwitchHasAuthority ; Ensure this only runs on the server.
      (:Authority
        (if (>= (Variables|StaminaSettings|GetDelayCheck) (* (Variables|StaminaSettings|GetRecoveryDelay) (Variables|StaminaSettings|GetUpdateFrequency))) ; Has the appropriate delay occured?
          (CallFunction|GetRecoveryRate) ; Determine correct recovery rate.
          (bind _output_get (Variables|StaminaSettings|SetPlayerStamina (Math|Float|Clamp(Float) (+ (Variables|StaminaSettings|GetPlayerStamina) (/ (Variables|StaminaSettings|GetCurrentRecoveryRate) (Math|Conversions|ToFloat(Integer) (Variables|StaminaSettings|GetUpdateFrequency)))) 0.0 (Variables|StaminaSettings|GetStaminaCap)))) ; Add 1/5th of the recovery rate to the player stamina, clamping it within the stamina cap.
          (CallFunction|UpdateStamina) ; Run stamina update.
          (if (>= _output_get (Variables|StaminaSettings|GetStaminaCap)) ; Has the players stamina reached the stamina cap?
            (Utilities|Time|ClearandInvalidateTimerbyHandle (Variables|StaminaSettings|GetRecoveryTimer)) ; Stop the recovery loop.
            (Variables|StaminaSettings|SetInRecovery false) ; Update recovery state boolean.
          )
          (else
            (Math|Integer|IncrementInt (Variables|StaminaSettings|GetDelayCheck))))))))

(event EventInitialize
  (params (PlayerController :type Player%20Controller%20Object%20Reference))
  ;[0.2 1 0.2 0.5] Initialize stamina system.
  (if (not (Variables|StaminaSettings|GetDisableSystem)) ; DEBUG: Is the stamina system set to\ndisabled?
    (bind _output_get (Variables|StaminaSettings|SetPlayerController PlayerController)) ; Store a reference to the controller.
    (bind _ascharacter (Utilities|Casting|CastToCharacter (Pawn|GetControlledPawn _output_get))) ; Check if the pawn is a derivative of the base character class.
    (Variables|StaminaSettings|SetControlledChar _ascharacter) ; Store a reference to base character.
    (Utilities|IsValid (Actor|GetComponentbyClass (Variables|StaminaSettings|GetPlayerController) "/Game/SGT/Blueprints/Components/C_Manager-HUD.C_Manager-HUD_C") ; Is there a valid HUD manager?
      (:Is%20Valid
        (Variables|StaminaSettings|SetHUDManager (Actor|GetComponentbyClass (Variables|StaminaSettings|GetPlayerController) "/Game/SGT/Blueprints/Components/C_Manager-HUD.C_Manager-HUD_C")) ; Set reference to HUD manager component.
      )
      (:Is%20Not%20Valid
        _))
    (Variables|StaminaSettings|SetPlayerStamina (Variables|StaminaSettings|GetMaxPlayerStamina)) ; Ensure player stamina set to max on startup.
    (CallFunction|UpdateStamina) ; Run stamina update.
    (Variables|StaminaSettings|SetStaminaCap (Variables|StaminaSettings|GetMaxPlayerStamina)) ; Ensure stamina cap is set to max on startup.
    (CallFunction|CapStamina) ; Force stamina cap.
  ))

(event EventReset
  ;[0.2 1 0.2 0.5] Reset stamina system.
  (if (not (Variables|StaminaSettings|GetDisableSystem)) ; DEBUG: Is the stamina system set to\ndisabled?
    (Utilities|Time|ClearandInvalidateTimerbyHandle (Variables|StaminaSettings|GetDecayTimer)) ; Force stop decay timer.
    (Variables|StaminaSettings|SetDecayActive false) ; Reset decay active state bool.
    (Utilities|Time|ClearandInvalidateTimerbyHandle (Variables|StaminaSettings|GetRecoveryTimer)) ; Force stop recovery timer.
    (Variables|StaminaSettings|SetInRecovery false) ; Reset recovery active state bool.
    (Variables|StaminaSettings|SetPlayerStamina (Variables|StaminaSettings|GetMaxPlayerStamina)) ; Reset stamina value.
    (Variables|StaminaSettings|SetStaminaCap (Variables|StaminaSettings|GetMaxPlayerStamina)) ; Reset stamina cap.
  ))

(fn GetStamina
  (return (Variables|StaminaSettings|GetPlayerStamina)) ; Done.
)

(fn GetRecoveryRate
  (if (Variables|StaminaSettings|GetLowerRecoveryWhenMoving) ; Should movement impact the recovery rate?
    (if (Math|Vector|Equal(Vector) (Transformation|GetVelocity (Variables|StaminaSettings|GetControlledChar)) "0, 0, 0" 0.0001) ; Is the player currently moving?
      _
      (else
        (Variables|StaminaSettings|SetCurrentRecoveryRate (Variables|StaminaSettings|GetLowerRecorveryRate)) ; Use lower moving recovery rate.
        (return) ; Done.
      )))
  (Variables|StaminaSettings|SetCurrentRecoveryRate (Variables|StaminaSettings|GetRecoveryRate)) ; Use non-moving recovery rate.
  (return) ; Done.
)

(fn CapStamina
  (Variables|StaminaSettings|SetPlayerStamina (Math|Float|Clamp(Float) (Variables|StaminaSettings|GetPlayerStamina) 0.0 (Variables|StaminaSettings|GetStaminaCap))) ; Reset stamina to keep within the current stamina cap.
  (CallFunction|UpdateHUD (/ (Variables|StaminaSettings|GetPlayerStamina) (Variables|StaminaSettings|GetMaxPlayerStamina))) ; Update the player's HUD.
  (return) ; Done.
)

(fn CheckDrain
  (if (Math|Float|NearlyEqual(Float) (Variables|StaminaSettings|GetStaminaDrain) 0.0 0.0005) ; Is the stamina drain currently equal or less than 5/1000ths of a unit?
    (Utilities|Time|ClearandInvalidateTimerbyHandle (Variables|StaminaSettings|GetDecayTimer)) ; Stop the decay loop.
    (Variables|StaminaSettings|SetDecayActive false) ; Update bool to reflect decay state.
    (if (Variables|StaminaSettings|GetInRecovery) ; Is the recovery timer loop already active?
      (return) ; Done.
      (else
        (bind _returnvalue (Utilities|Time|SetTimerbyFunctionName 0 "Recover" (/ 1.0 (Math|Conversions|ToFloat(Integer) (Variables|StaminaSettings|GetUpdateFrequency))) true)) ; Initiate stamina recover loop.
        (Variables|StaminaSettings|SetRecoveryTimer _returnvalue) ; Store reference to timer for later use.
        (Variables|StaminaSettings|SetInRecovery true) ; Update recovery state boolean.
        (return) ; Done.
      ))
    (elif (Variables|StaminaSettings|GetDecayActive) ; Check if decay is already active.
      (return) ; Done.
      (else
        (Variables|StaminaSettings|SetDecayActive true) ; Update bool to reflect decay state.
        (Utilities|Time|ClearandInvalidateTimerbyHandle (Variables|StaminaSettings|GetRecoveryTimer)) ; Disable the recovery loop.
        (Variables|StaminaSettings|SetInRecovery false) ; Update recovery state boolean.
        (Variables|StaminaSettings|SetDelayCheck 0) ; Reset the delay counter.
        (bind _returnvalue_2 (Utilities|Time|SetTimerbyFunctionName 0 "Decay" (/ 1.0 (Math|Conversions|ToFloat(Integer) (Variables|StaminaSettings|GetUpdateFrequency))) true)) ; Initiate stamina decay loop.
        (Variables|StaminaSettings|SetDecayTimer _returnvalue_2) ; Store reference to timer for later use.
        (return) ; Done.
      ))))

(fn UpdateStamina
  (Utilities|IsValid (Variables|StaminaSettings|GetPlayerController) ; Is the player controller reference valid?
    (:Is%20Valid
      (bind _isdead (Class|BPintController|GetLifeState(Message) (Variables|StaminaSettings|GetPlayerController))) ; Get alive state from controller.
      (if _isdead ; Is the player dead?
        (return) ; Done.
        (else
          (CallFunction|UpdateHUD (/ (Variables|StaminaSettings|GetPlayerStamina) (Variables|StaminaSettings|GetMaxPlayerStamina))) ; Update the palyer's HUD.
          (if (<= (Variables|StaminaSettings|GetPlayerStamina) 0.0) ; Does the player have any stamina left?
            (Variables|StaminaSettings|SetExhausted true) ; Set exhausted state to true.
            (if (<= (Variables|StaminaSettings|GetStaminaDrain) 0.0) ; Is stamina drain set to 0 or less than 0?
              (if (Variables|StaminaSettings|GetInRecovery) :!label _label ; Is the recovery timer loop already active?
                _
                (elif (Variables|StaminaSettings|GetDecayActive) ; Is decay currently active?
                  _
                  (else
                    (bind _returnvalue (Utilities|Time|SetTimerbyFunctionName 0 "Recover" (/ 1.0 (Math|Conversions|ToFloat(Integer) (Variables|StaminaSettings|GetUpdateFrequency))) true)) ; Initiate stamina recover loop.
                    (Variables|StaminaSettings|SetRecoveryTimer _returnvalue) ; Store reference to recovery timer.
                    (Variables|StaminaSettings|SetInRecovery true) ; Update recovery state boolean.
                    (return) ; Done.
                  ))))
            (else
              (Variables|StaminaSettings|SetExhausted false) ; Set exhausted state to false.
              (if (< (Variables|StaminaSettings|GetPlayerStamina) (Variables|StaminaSettings|GetMaxPlayerStamina)) ; Is the player's stamina full?
                (goto _label)
                (else
                  (Utilities|Time|ClearandInvalidateTimerbyHandle (Variables|StaminaSettings|GetRecoveryTimer)) ; Stop the recovery loop.
                  (Variables|StaminaSettings|SetInRecovery false) ; Update recovery state boolean.
                  (return) ; Done.
                ))))
          (return) ; Done.
        )))
    (:Is%20Not%20Valid
      (return) ; Done.
    )))