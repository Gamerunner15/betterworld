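; Poison manager component that tracks a player's poison level and applies toxicity damage.
; Volume enter and exit events, gated to the server, control a looping timer that adds poison over time.
; Poison maps to threshold-based toxicity levels, which scale the damage dealt by a second server-authoritative timer.
; Changes feed the HUD and an optional high-poison visual effect through sibling managers fetched from the player controller at initialization.
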(event Custom|UpdateHUD
  (params (Poison :type Float%20%28single-precision%29))
  (bind _hudmanager (Variables|PoisonSettings|GetHUDManager))
  ;[0.2 1 0.2 0.5] Update player HUD.
  (if (not (Variables|PoisonSettings|GetDisableSystem)) ; DEBUG: Is the poison system set to\ndisabled?
    (Utilities|IsValid _hudmanager ; Is the HUD manager valid?
      (:Is%20Valid
        (Variables|/Game/SGT/Blueprints/Components/C_Manager-HUD.C_Manager-HUD_C|SetPoison _hudmanager Poison) ; Update player HUD.
      ))))

(event Custom|Toxicity
  ;[1 0.2 0.2 0.5] Apply damage to the player based on toxicity level.
  (if (not (Variables|PoisonSettings|GetDisableSystem)) ; DEBUG: Is the poison system set to\ndisabled?
    (Utilities|SwitchHasAuthority ; Ensure this only runs on server.
      (:Authority
        (Game|Damage|ApplyDamage (Variables|PoisonSettings|GetPlayerController) (* (Variables|PoisonSettings|GetCurrentDamage) (/ 1.0 (Math|Conversions|ToFloat(Integer) (Variables|PoisonSettings|GetUpdateFrequency)))) 0 0 "/Game/SGT/Blueprints/Misc/Damage_Statistical.Damage_Statistical_C") ; Apply damage to player.
      ))))

(event Custom|PoisonLoop
  ;[1 0.2 0.2 0.5] Volume poison loop.
  (if (not (Variables|PoisonSettings|GetDisableSystem)) ; DEBUG: Is the poison system set to\ndisabled?
    (CallFunction|AddPoison (Variables|PoisonSettings|GetVolumePoison)) ; Update poison based on volume.
  ))

(event Custom|VolumeExit
  ;[1 0.2 0.2 0.5] Stop the poison loop timer.
  (if (not (Variables|PoisonSettings|GetDisableSystem)) ; DEBUG: Is the poison system set to\ndisabled?
    (Utilities|Time|ClearandInvalidateTimerbyHandle (Variables|PoisonSettings|GetPoisonLoopTimer))))

(event Custom|AddPoison
  (params (AmountToAdd :type Float%20%28single-precision%29))
  ;[1 0.2 0.2 0.5] Take input poison and add to the current poison, clamping within max poison.
  (if (not (Variables|PoisonSettings|GetDisableSystem)) ; DEBUG: Is the poison system set to\ndisabled?
    (Variables|PoisonSettings|SetPlayerPoison (Math|Float|Clamp(Float) (+ (Variables|PoisonSettings|GetPlayerPoison) AmountToAdd) 0.0 (Variables|PoisonSettings|GetMaxPlayerToxicity))) ; Update poison value.
    (CallFunction|UpdatePoison) ; Run poison update.
    (CallFunction|UpdateVisualEffect)
    (CallFunction|UpdateHUD (/ (Variables|PoisonSettings|GetPlayerPoison) (Variables|PoisonSettings|GetMaxPlayerToxicity))) ; Update HUD poison value.
  ))

(event Custom|VolumeTriggered
  (params (Amount :type Float%20%28single-precision%29) (Delay :type Float%20%28single-precision%29))
  ;[1 0.2 0.2 0.5] Perform initial poisoning on enter, and trigger loop for further poison over time.
  (if (not (Variables|PoisonSettings|GetDisableSystem)) ; DEBUG: Is the poison system set to\ndisabled?
    (Variables|PoisonSettings|SetVolumePoison Amount) ; Store volume poison rate.
    (Variables|PoisonSettings|SetVolumeUpdateDelay Delay) ; Store volume update delay.
    (CallFunction|AddPoison (Variables|PoisonSettings|GetVolumePoison)) ; Perform initial poison.
    (bind _returnvalue (Utilities|Time|SetTimerbyFunctionName 0 "PoisonLoop" (Variables|PoisonSettings|GetVolumeUpdateDelay) true)) ; Trigger poison loop.
    (Variables|PoisonSettings|SetPoisonLoopTimer _returnvalue) ; Store reference to handle for use.
  ))

(event EventInitialize
  (params (PlayerController :type Player%20Controller%20Object%20Reference))
  ;[0.2 1 0.2 0.5] Initialize poisoned system.
  (if (not (Variables|PoisonSettings|GetDisableSystem)) ; DEBUG: Is the poison system set to\ndisabled?
    (Variables|PoisonSettings|SetPlayerController PlayerController) ; Set a reference to controller.
    (bind (_no_hud _hudcomponent _novisualeffects _visualeffectscomponent _nostamina _staminacomponent) (CallFunction|CommonComponents (Variables|PoisonSettings|GetPlayerController) (Utilities|Enum|NotEqual(Enum) (Variables|PoisonSettings|GetHighPoisonVisualEffect) "NewEnumerator11") (Variables|PoisonSettings|GetLimitStamina))) ; Retrieve common components from player controller.
    (if (not _no_hud) ; Was there no HUD manager found?
      (Variables|PoisonSettings|SetHUDManager _hudcomponent) ; Set reference to HUD manager.
      (if _novisualeffects ; Was there no visual feedback manager\nfound in the player controller?
        (Variables|PoisonSettings|SetHighPoisonVisualEffect "NewEnumerator11") ; As no valid visual feedback manager was found,\nforce effect to none.
        (else
          (Variables|PoisonSettings|SetVisualFeedbackManager _visualeffectscomponent) ; Set reference to Visual Feedback manager.
        ))
      (if _nostamina ; Was there no stamina manager found\nin the player controller?
        (Variables|PoisonSettings|SetLimitStamina false) ; As no valid stamina manager exists,\nforce LimitStamina to false.
        (else
          (Variables|PoisonSettings|SetStaminaManager _staminacomponent) ; Set reference to Stamina manager.
        ))
      (Variables|PoisonSettings|SetPlayerPoison 0.0) ; Set initial poison level to zero.
      (Variables|PoisonSettings|SetToxicityLevelCount (- (Utilities|Array|Length (Variables|PoisonSettings|GetToxicityLevels)) 1)) ; Determine how many toxicity levels\nthere are.
      (Variables|PoisonSettings|SetActiveToxicity 0) ; Set the initial active toxicity level to zero.
      (Variables|PoisonSettings|SetLowestToxicity (Variables|PoisonSettings|GetMaxPlayerToxicity)) ; Set initial lowest toxicity to max.
      (for _array_element (Variables|PoisonSettings|GetToxicityLevels) ; For each entry in the ToxicityLevels array...
        (if (< _array_element (Variables|PoisonSettings|GetLowestToxicity)) ; Is this level lower than the current\nlowest toxicity?
          (Variables|PoisonSettings|SetLowestToxicity _array_element) ; Update to lower value.
          (CallFunction|UpdatePoison) ; Run poison update.
        )))))

(event EventReset
  ;[0.2 1 0.2 0.5] Force reset prior to death.
  (if (not (Variables|PoisonSettings|GetDisableSystem)) ; DEBUG: Is the poison system set to\ndisabled?
    (Utilities|Time|ClearandInvalidateTimerbyHandle (Variables|PoisonSettings|GetToxicTimer))
    (Variables|PoisonSettings|SetToxicActive false)
    (Variables|PoisonSettings|SetVisualEffectActive false) ; Reset visual effect state bool.
    (Variables|PoisonSettings|SetStaminaLimited false) ; Reset stamina limited state bool.
    (Variables|PoisonSettings|SetPlayerPoison 0.0)
    (Variables|PoisonSettings|SetActiveToxicity 0)
    (Utilities|Time|ClearandInvalidateTimerbyHandle (Variables|PoisonSettings|GetPoisonLoopTimer))))

(event EventVolumeTriggeredEvent
  (params (PoisonAmount :type Float%20%28single-precision%29) (LoopDelay :type Float%20%28single-precision%29))
  ;[1 0.2 0.2 0.5] Volume triggered sequence.
  (if (not (Variables|PoisonSettings|GetDisableSystem)) ; DEBUG: Is the poison system set to\ndisabled?
    (Utilities|SwitchHasAuthority ; Ensure this only runs on the server.
      (:Authority
        (CallFunction|VolumeTriggered PoisonAmount LoopDelay) ; Trigger the poison volume event.
      ))))

(event EventVolumeExitEvent
  ;[1 0.2 0.2 0.5] Volume exit sequence.
  (if (not (Variables|PoisonSettings|GetDisableSystem)) ; DEBUG: Is the poison system set to\ndisabled?
    (Utilities|SwitchHasAuthority ; Ensure this only runs on the server.
      (:Authority
        (CallFunction|VolumeExit) ; Trigger the poison volume exit event.
      ))))

(fn UpdatePoison
  (bind _playercontroller (Variables|PoisonSettings|GetPlayerController))
  (bind _hudmanager (Variables|PoisonSettings|GetHUDManager))
  (Utilities|IsValid _playercontroller ; Valid player controller?
    (:Is%20Valid
      (bind _isdead (Class|BPintController|GetLifeState(Message) _playercontroller)) ; Get the current life state from the controller\nvia interface.
      (if _isdead ; Is the player dead?
        (return) ; As player is dead, do nothing.
        (else
          (Variables|PoisonSettings|SetCurrentToxicity 0) ; Reset the current toxicity level.
          (bind (_array_element _array_index) (Utilities|Array|ForEachLoopwithBreak (Variables|PoisonSettings|GetToxicityLevels) :!label _label) ; For each entry in the toxicity levels array...
            (:LoopBody
              (if (>= (Variables|PoisonSettings|GetPlayerPoison) _array_element) ; Does the player's poison exceed this\nlevel's starting amount?
                (Variables|PoisonSettings|SetCurrentToxicity _array_index) ; Update the current toxicity level.
                (else
                  (goto _label Break))))
            (:Completed
              (if (== (Variables|PoisonSettings|GetCurrentToxicity) 0) ; Is the player currently below poisoning thresholds?
                (if (Variables|PoisonSettings|GetToxicActive) ; Was the player previously losing health due to toxicity?
                  (Utilities|Time|ClearandInvalidateTimerbyHandle (Variables|PoisonSettings|GetToxicTimer)) ; Stop the toxicity loop timer. Eating seeds is a past time activity.
                  (Variables|PoisonSettings|SetToxicActive false) ; Update toxic active state bool.
                )
                (elif (== (Variables|PoisonSettings|GetCurrentToxicity) (Variables|PoisonSettings|GetActiveToxicity)) ; Is the current toxicity level the same as the active toxicity level?
                  _
                  (else
                    (Variables|PoisonSettings|SetCurrentDamage (* (/ (Math|Conversions|ToFloat(Integer) (Variables|PoisonSettings|GetCurrentToxicity)) (Math|Conversions|ToFloat(Integer) (Variables|PoisonSettings|GetToxicityLevelCount))) (Variables|PoisonSettings|GetMaxToxicityDamage))) ; Update the damage rate.
                    (Variables|PoisonSettings|SetActiveToxicity (Variables|PoisonSettings|GetCurrentToxicity)) ; Update the active toxicity. Disorder, disorder, disorder.
                    (if (Variables|PoisonSettings|GetToxicActive) ; Was the player previously losing health\ndue to toxicity?
                      (return) ; Done.
                      (else
                        (bind _returnvalue (Utilities|Time|SetTimerbyFunctionName 0 "Toxicity" (/ 1.0 (Math|Conversions|ToFloat(Integer) (Variables|PoisonSettings|GetUpdateFrequency))) true)) ; Start the toxicity loop. Somewhere between the sacred\nsilence and sleep.
                        (Variables|PoisonSettings|SetToxicTimer _returnvalue) ; Store a reference to the toxicity timer.
                        (Utilities|IsValid _hudmanager ; Is the HUD manager reference valid?
                          (:Is%20Valid
                            (Default|UpdateFeedback _hudmanager "You are now suffering from toxic shock.") ; Add feedback text for player.
                          )
                          (:Is%20Not%20Valid
                            _))
                        (Variables|PoisonSettings|SetToxicActive true) ; Update toxic active state bool.
                        (return) ; Done.
                      )))))
              (CallFunction|UpdateHUD (/ (Variables|PoisonSettings|GetPlayerPoison) (Variables|PoisonSettings|GetMaxPlayerToxicity))) ; Update HUD poison value.
              (return) ; Done.
            )))))
    (:Is%20Not%20Valid
      (return) ; Done.
    )))

(fn UpdateVisualEffect
  (if (Utilities|Enum|NotEqual(Enum) (Variables|PoisonSettings|GetHighPoisonVisualEffect) "NewEnumerator11") ; Is a visual effect enabled?
    (if (Variables|PoisonSettings|GetVisualEffectActive) ; Is the visual effect currently active?
      (if (>= (Variables|PoisonSettings|GetPlayerPoison) (Variables|PoisonSettings|GetVisualEffectThreshold)) ; Is the player's water below the visual effect threshold level?
        _
        (else
          (Default|EffectControl (Variables|PoisonSettings|GetVisualFeedbackManager) (Variables|PoisonSettings|GetHighPoisonVisualEffect) true) ; Begin the sequence to turn the visual effect off.
          (Variables|PoisonSettings|SetVisualEffectActive false) ; Update visual effect state bool.
          (return) ; Done.
        ))
      (elif (< (Variables|PoisonSettings|GetPlayerPoison) (Variables|PoisonSettings|GetVisualEffectThreshold)) ; Is the player's water above the visual effect threshold level?
        _
        (else
          (Default|EffectControl (Variables|PoisonSettings|GetVisualFeedbackManager) (Variables|PoisonSettings|GetHighPoisonVisualEffect) false) ; Begin the sequence to turn the visual effect on.
          (Variables|PoisonSettings|SetVisualEffectActive true) ; Update visual effect state bool.
          (return) ; Done.
        )))
    (return) ; Done.
    (else
      (return) ; Done.
    )))