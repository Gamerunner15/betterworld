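; Player hunger manager component that drains food over time, accepts added food and damages the player through starvation when it runs out.
; UpdateHunger switches between looping Decay and Starvation timers, whose effects apply only with server authority.
; It feeds the HUD manager, toggles an optional low-food visual effect at a threshold and can lower the stamina cap while starving.
; Initialize fetches these sibling managers from the player controller, disabling visual or stamina features when absent.
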(event Custom|Starvation
  ;[1 0.2 0.2 0.5] Apply damage to the player when they are starving.
  (if (not (Variables|HungerSettings|GetDisableSystem)) ; DEBUG: Is the hunger system set to \ndisabled?
    (Utilities|SwitchHasAuthority ; Ensure this only runs on the server.
      (:Authority
        (Game|Damage|ApplyDamage (Variables|HungerSettings|GetPlayerController) (* (Variables|HungerSettings|GetStarvationDamage) (/ 1.0 (Math|Conversions|ToFloat(Integer) (Variables|HungerSettings|GetUpdateFrequency)))) 0 0 "/Game/SGT/Blueprints/Misc/Damage_Statistical.Damage_Statistical_C") ; Apply damage to player.
      ))))

(event Custom|AddFood
  (params (AmountToAdd :type Float%20%28single-precision%29))
  ;[1 0.2 0.2 0.5] Take input food and add to the current food, clamping within max food.
  (if (not (Variables|HungerSettings|GetDisableSystem)) ; DEBUG: Is the hunger system set to \ndisabled?
    (Variables|HungerSettings|SetPlayerFood (Math|Float|Clamp(Float) (+ (Variables|HungerSettings|GetPlayerFood) AmountToAdd) 0.0 (Variables|HungerSettings|GetMaxPlayerFood))) ; Update food value.
    (CallFunction|UpdateHunger) ; Run hunger update.
  ))

(event Custom|UpdateHUD
  (params (Hunger :type Float%20%28single-precision%29))
  (bind _hudmanager (Variables|HungerSettings|GetHUDManager))
  ;[0.2 1 0.2 0.5] Update player HUD.
  (if (not (Variables|HungerSettings|GetDisableSystem)) ; DEBUG: Is the hunger system set to \ndisabled?
    (Utilities|IsValid _hudmanager ; Is the HUD manager valid?
      (:Is%20Valid
        (Variables|/Game/SGT/Blueprints/Components/C_Manager-HUD.C_Manager-HUD_C|SetFood _hudmanager Hunger) ; Update player HUD.
      ))))

(event Custom|Decay
  ;[1 0.2 0.2 0.5] Decay player food based on update frequency and drain rate.
  (if (not (Variables|HungerSettings|GetDisableSystem)) ; DEBUG: Is the hunger system set to \ndisabled?
    (Utilities|SwitchHasAuthority ; Ensure this only runs on the server.
      (:Authority
        (Variables|HungerSettings|SetPlayerFood (Math|Float|Clamp(Float) (- (Variables|HungerSettings|GetPlayerFood) (/ (Variables|HungerSettings|GetDrainRate) (Math|Conversions|ToFloat(Integer) (Variables|HungerSettings|GetUpdateFrequency)))) 0.0 (Variables|HungerSettings|GetMaxPlayerFood))) ; Update food value.
        (CallFunction|UpdateHunger) ; Run hunger update.
      ))))

(event EventInitialize
  (params (PlayerController :type Player%20Controller%20Object%20Reference))
  ;[0.2 1 0.2 0.5] Initialize hunger system.
  (if (not (Variables|HungerSettings|GetDisableSystem)) ; DEBUG: Is the hunger system set to\ndisabled?
    (Variables|HungerSettings|SetPlayerController PlayerController) ; Set reference to controller.
    (bind (_no_hud _hudcomponent _novisualeffects _visualeffectscomponent _nostamina _staminacomponent) (CallFunction|CommonComponents (Variables|HungerSettings|GetPlayerController) (Utilities|Enum|NotEqual(Enum) (Variables|HungerSettings|GetLowFoodVisualEffect) "NewEnumerator11") (Variables|HungerSettings|GetLimitStamina))) ; Retrieve common components from player controller.
    (if _no_hud ; Was there no HUD manager found?
      _
      (else
        (Variables|HungerSettings|SetHUDManager _hudcomponent) ; Set reference to HUD manager.
      ))
    (if _novisualeffects ; Was there no visual feedback manager\nfound in the player controller?
      (Variables|HungerSettings|SetLowFoodVisualEffect "NewEnumerator11") ; As no valid visual feedback manager was found,\nforce effect to none.
      (else
        (Variables|HungerSettings|SetVisualFeedbackManager _visualeffectscomponent) ; Set reference to Visual Feedback manager.
      ))
    (if _nostamina ; Was there no stamina manager found\nin the player controller?
      (Variables|HungerSettings|SetLimitStamina false) ; As no valid stamina manager exists,\nforce LimitStamina to false.
      (else
        (Variables|HungerSettings|SetStaminaManager _staminacomponent) ; Set reference to Stamina manager.
      ))
    (Variables|HungerSettings|SetPlayerFood (Variables|HungerSettings|GetMaxPlayerFood)) ; Initialize food value.
    (CallFunction|UpdateHunger) ; Run hunger update.
  ))

(event EventReset
  ;[0.2 1 0.2 0.5] Force reset prior to death.
  (if (not (Variables|HungerSettings|GetDisableSystem)) ; DEBUG: Is the hunger system set to\ndisabled?
    (Utilities|Time|ClearandInvalidateTimerbyHandle (Variables|HungerSettings|GetDecayTimer))
    (Variables|HungerSettings|SetDecayActive false)
    (Utilities|Time|ClearandInvalidateTimerbyHandle (Variables|HungerSettings|GetStarvationTimer))
    (Variables|HungerSettings|SetIsStarving false)
    (Variables|HungerSettings|SetVisualEffectActive false) ; Reset visual effect state bool.
    (Variables|HungerSettings|SetStaminaLimited false) ; Reset stamina limited state bool.
    (Variables|HungerSettings|SetPlayerFood (Variables|HungerSettings|GetMaxPlayerFood)) ; Initialize food value.
  ))

(fn UpdateHunger
  (bind _hudmanager (Variables|HungerSettings|GetHUDManager))
  (bind _isdead (Class|BPintController|GetLifeState(Message) (Variables|HungerSettings|GetPlayerController))) ; Is the player controller reference valid?
  (if _isdead ; Is the player dead?
    (return) ; As player is dead, do nothing.
    (elif (<= (Variables|HungerSettings|GetPlayerFood) 0.0)
      (if (Variables|HungerSettings|GetDecayActive) ; Is the decay loop currently active?
        (Utilities|Time|ClearandInvalidateTimerbyHandle (Variables|HungerSettings|GetDecayTimer)) ; Stop the decay loop.
        (Variables|HungerSettings|SetDecayActive false) ; Set decay loop boolean state.
      )
      (bind _returnvalue (Utilities|Time|SetTimerbyFunctionName 0 "Starvation" (/ 1.0 (Math|Conversions|ToFloat(Integer) (Variables|HungerSettings|GetUpdateFrequency))) true)) ; Start the starvation loop.
      (Variables|HungerSettings|SetStarvationTimer _returnvalue) ; Store a reference to the starvation timer.
      (Variables|HungerSettings|SetIsStarving true) ; Set starving state bool.
      (Utilities|IsValid _hudmanager ; Is the HUD manager reference valid?
        (:Is%20Valid
          (Default|UpdateFeedback _hudmanager "You are starving and will soon die without food.") ; Provide feedback to player.
        )
        (:Is%20Not%20Valid
          _))
      (if (Variables|HungerSettings|GetLimitStamina) ; Should the player's stamina be limited if they are starving?
        (if (Variables|HungerSettings|GetStaminaLimited)
          (return) ; Done.
          (else
            (Default|LowerCap (Variables|HungerSettings|GetStaminaManager) (Variables|HungerSettings|GetStaminaReduction)) ; Lower the player's stamina cap.
            (Variables|HungerSettings|SetStaminaLimited true) ; Update limited stamina state bool.
            (return) ; Done.
          ))
        (else
          (return) ; Done.
        ))
      (else
        (CallFunction|UpdateVisualEffect)
        (if (Variables|HungerSettings|GetDecayActive) ; Is the decay loop already active?
          (CallFunction|UpdateHUD (/ (Variables|HungerSettings|GetPlayerFood) (Variables|HungerSettings|GetMaxPlayerFood))) ; Update the player HUD.
          (return) ; Done.
          (else
            (if (Variables|HungerSettings|GetIsStarving) ; Was the player previously starving?
              (Utilities|Time|ClearandInvalidateTimerbyHandle (Variables|HungerSettings|GetStarvationTimer)) ; Stop the starvation update loop.
              (Variables|HungerSettings|SetIsStarving false) ; Set starvation state bool.
              (if (Variables|HungerSettings|GetStaminaLimited) ; Was the player's stamina previously limited?
                (Default|RaiseCap (Variables|HungerSettings|GetStaminaManager) (Variables|HungerSettings|GetStaminaReduction)) ; Raise the stamina cap appropriately.
                (Variables|HungerSettings|SetStaminaLimited false) ; Update stamina limited bool.
              ))
            (bind _returnvalue_2 (Utilities|Time|SetTimerbyFunctionName 0 "Decay" (/ 1.0 (Math|Conversions|ToFloat(Integer) (Variables|HungerSettings|GetUpdateFrequency))) true)) ; Start the decay loop.
            (Variables|HungerSettings|SetDecayTimer _returnvalue_2) ; Update reference to decay loop timer.
            (Variables|HungerSettings|SetDecayActive true) ; Set decay loop boolean state.
            (return) ; Done.
          ))))))

(fn UpdateVisualEffect
  (if (Utilities|Enum|NotEqual(Enum) (Variables|HungerSettings|GetLowFoodVisualEffect) "NewEnumerator11") ; Is a visual effect enabled?
    (if (Variables|HungerSettings|GetVisualEffectActive) ; Is the visual effect currently active?
      (if (<= (Variables|HungerSettings|GetPlayerFood) (Variables|HungerSettings|GetVisualEffectThreshold)) ; Is the player's food below the visual effect threshold level?
        _
        (else
          (Default|EffectControl (Variables|HungerSettings|GetVisualFeedbackManager) (Variables|HungerSettings|GetLowFoodVisualEffect) true) ; Begin the sequence to turn the visual effect off.
          (Variables|HungerSettings|SetVisualEffectActive false) ; Update visual effect state bool.
          (return) ; Done.
        ))
      (elif (> (Variables|HungerSettings|GetPlayerFood) (Variables|HungerSettings|GetVisualEffectThreshold)) ; Is the player's food above the visual effect threshold level?
        _
        (else
          (Default|EffectControl (Variables|HungerSettings|GetVisualFeedbackManager) (Variables|HungerSettings|GetLowFoodVisualEffect) false) ; Begin the sequence to turn the visual effect on.
          (Variables|HungerSettings|SetVisualEffectActive true) ; Update visual effect state bool.
          (return) ; Done.
        )))
    (return) ; Done.
    (else
      (return) ; Done.
    )))