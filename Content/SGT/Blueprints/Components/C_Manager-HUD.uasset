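; HUD manager component that creates and drives the local player's survival HUD: stats, clock, compass, focus item and feedback messages.
; A looping timer pushes stats, ages feedback lines and traces from the camera, ignoring living characters, to match hit actors against interactive classes.
; Interactive hits get a custom-depth outline through interface-supplied meshes.
; A faster timer feeds control yaw into the compass material, and events toggle visibility or post feedback.
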(event Custom|CompassLoop
  ;[0.2 1 0.2 0.5] Update the compass every call.
  (CallFunction|UpdateCompass))

(event Custom|UpdateLoop
  ;[0.2 1 0.2 0.5] Update the HUD every call.
  (Update|Update)
  (Utilities|FlowControl|Delay 0.5)
  (CallFunction|UpdateFeedbackScroller)
  (CallFunction|AddNewFeedbackItem))

(event Custom|UpdateFeedback
  (params (Text :type Text))
  (CallFunction|AddNewFeedbackItem Text))

(event Custom|ToggleHUD
  (params (ForceVisibilityOn :type Boolean) (ForceVisibilityOff :type Boolean))
  ;[0.2 1 0.2 0.5] Toggle the HUD on or off.
  (CallFunction|ToggleWidget ForceVisibilityOn ForceVisibilityOff))

(event EventInitialize
  (params (PlayerController :type Player%20Controller%20Object%20Reference))
  ;[0.2 1 0.2 0.5] Initialize HUD system.
  (bind _output_get (Variables|HUDSettings|SetPlayerController PlayerController)) ; Store a reference for use.
  (Variables|HUDSettings|SetControlledChar (Pawn|GetControlledPawn _output_get)) ; Set a reference to the controller character.
  (if (Pawn|IsLocalController (Variables|HUDSettings|GetPlayerController)) ; Ensure only local controller runs the rest of the initialization.
    (bind _returnvalue (UserInterface|CreateWidget "/Game/SGT/Blueprints/HUD/W_SGT_HUDLayout.W_SGT_HUDLayout_C")) ; Create the HUD widget.
    (bind _output_get_2 (Variables|HUDSettings|SetHUDWidget _returnvalue)) ; Store a reference to the HUD widget.
    (Class|BPintController|SetHUDWidget(Message) (Variables|HUDSettings|GetPlayerController) _output_get_2) ; Update HUD widget reference in controller.
    (UserInterface|Viewport|AddtoViewport (Variables|HUDSettings|GetHUDWidget) -1) ; Add the HUD widget to the viewport.
    (Variables|HUDSettings|SetHUDOn true) ; Set initial visibility state.
    (Utilities|Time|SetTimerbyFunctionName 0 "UpdateLoop" 0.05 true) ; Initiate the update loop timer.
    (CallFunction|ToggleStatsStyle) ; Setup the player statistics based on bool.
    ;[0.2 1 0.2 0.5] Initialize the compass.
    (bind _compasswidget (Class|BPIntHUD|GetCompass(Message) (Variables|HUDSettings|GetHUDWidget))) ; Get W_Compass Widget.
    (if (Variables|HUDSettings|GetUseCompass) ; Is Use Compass set to on or off?
      (bind _returnvalue_2 (Appearance|GetDynamicMaterial (Variables|/Game/SGT/Blueprints/HUD/W_SGT_Compass.W_SGT_Compass_C|GetCompass _compasswidget) :!class /Script/UMG.Image)) ; Get the material for the compass.
      (Variables|HUDSettings|SetCompassMaterial _returnvalue_2) ; Store a reference to the compass material for use.
      (Utilities|Time|SetTimerbyFunctionName 0 "CompassLoop" 0.025 true) ; Initiate the compass update loop timer.
      (else
        (Widget|SetVisibility _compasswidget "Collapsed") ; Hide the compass.
      ))))

(event EventReset
  (if (Pawn|IsLocalController (Variables|HUDSettings|GetPlayerController))
    (Widget|RemovefromParent (Variables|HUDSettings|GetHUDWidget))))

(fn Update
  (bind _playercontroller (Variables|HUDSettings|GetPlayerController))
  (Utilities|IsValid _playercontroller ; Valid player controller?
    (:Is%20Valid
      (bind _isdead (Class|BPintController|GetLifeState(Message) _playercontroller)) ; Retrieve current life state.
      (if _isdead ; Is the player alive?
        (InteractiveOutline|ResetActor) ; Reset the item outline.
        (return) ; Done.
        (else
          (bind _actorhit (InteractiveOutline|InteractiveTrace)) ; Check if the player is looking at an item in reach.
          (Variables|HUDSettings|SetActorHit _actorhit) ; Store a reference to the actor hit.
          (InteractiveOutline|CheckforInteractive) ; Is that actor interactive?
          (InteractiveOutline|OutlineActor) ; Show interaction visuals.
          (Update|SetStats) ; Update HUD.
          (return) ; Done.
        )))
    (:Is%20Not%20Valid
      (return) ; Done.
    )))

(fn CheckforInteractive
  (if (== (Variables|HUDSettings|GetActorHit) (Variables|HUDSettings|GetLastActorHit)) ; Is the hit actor the same as last time?
    (return) ; Do nothing.
    (else
      (InteractiveOutline|ResetActor) ; Reset the last hit actor.
      (LocalVariables|SetActorClass (Utilities|GetClass (Variables|HUDSettings|GetActorHit))) ; Store the actor class for reference.
      (bind _array_element (Utilities|Array|ForEachLoopwithBreak (Variables|HUDSettings|GetInteractiveObjects) :!label _label) ; For each class in the InteractiveObjects array...
        (:LoopBody
          (LocalVariables|SetElementClass _array_element) ; Store the current array class.
          (bind _output_get (Variables|HUDSettings|SetCurrentFocusInteractive (or (== (LocalVariables|GetActorClass) (LocalVariables|GetElementClass)) (Utilities|ClassIsChildOf (LocalVariables|GetActorClass) (LocalVariables|GetElementClass))))) ; If either condition is true, the actor is interactive.
          (if _output_get ; If the actor is interactive, then stop the loop.
            (goto _label Break)))
        (:Completed
          (Variables|HUDSettings|SetLastActorHit (Variables|HUDSettings|GetActorHit)) ; Update LastHitActor
          (return) ; Done.
        )))))

(fn ResetActor
  (Utilities|IsValid (Variables|HUDSettings|GetLastActorHit) ; Is this object still valid (if object has been destroy, it will nolonger be valid, for example).
    (:Is%20Valid
      (bind _meshcomponent (Class|BPIntMeshActor|GetActorMeshComponent(Message) (Variables|HUDSettings|GetLastActorHit))) ; INTERFACE CALL: Retrieve actor mesh from input.
      ;[1 1 1] Ensure we only attempt to highlight Static and Skeletal meshes.
      (Utilities|Casting|CastToStaticMeshComponent _meshcomponent
        (:then
          (Rendering|SetRenderCustomDepth _meshcomponent false :!label _label) ; Turn off the item outline.
          (return) ; Done.
        )
        (:CastFailed
          (Utilities|Casting|CastToSkeletalMeshComponent _meshcomponent
            (:then
              (goto _label))
            (:CastFailed
              _)))))
    (:Is%20Not%20Valid
      _))
  (return) ; Done.
)

(fn OutlineActor
  (if (Variables|HUDSettings|GetCurrentFocusInteractive) ; Is the current focus item interactive?
    (Class|BPIntHUD|SetFocusItem(Message) (Variables|HUDSettings|GetHUDWidget) (Variables|HUDSettings|GetLastActorHit)) ; Set HUD focus item to the interactive actor.
    (bind _meshcomponent (Class|BPIntMeshActor|GetActorMeshComponent(Message) (Variables|HUDSettings|GetActorHit))) ; INTERFACE CALL: Retrieve actor mesh from input.
    ;[1 1 1] Ensure we only attempt to highlight Static and Skeletal meshes.
    (Utilities|Casting|CastToStaticMeshComponent _meshcomponent
      (:then
        _)
      (:CastFailed
        (Utilities|Casting|CastToSkeletalMeshComponent _meshcomponent
          (:then
            _)
          (:CastFailed
            (return) ; Done.
          ))))
    (Rendering|SetRenderCustomDepth _meshcomponent true) ; Turn on the item outline.
    (return) ; Done.
    (else
      (Class|BPIntHUD|SetFocusItem(Message) (Variables|HUDSettings|GetHUDWidget) (Variables|HUDSettings|GetLastActorHit)) ; Clear HUD focus item if not interactive.
      (return) ; Done.
    )))

(fn SetStats
  (Class|BPIntHUD|SetStatistics(Message) (Variables|HUDSettings|GetHUDWidget) (Variables|HUDSettings|GetHealth) (Variables|HUDSettings|GetStamina) (Variables|HUDSettings|GetPower) (Variables|HUDSettings|GetWater) (Variables|HUDSettings|GetFood) (Variables|HUDSettings|GetPoison) (Utilities|Text|ToText(Float) (Variables|HUDSettings|GetTempWorld) "HalfToEven" false true 1 3 1 1) (Utilities|Text|ToText(Float) (Variables|HUDSettings|GetTempBody) "HalfToEven" false true 1 3 1 1) (Variables|HUDSettings|GetOxygen) (Variables|HUDSettings|GetBlood)) ; Transfer player statistics data to the HUD widget for display.
  (Class|BPIntHUD|SetClock(Message) (Variables|HUDSettings|GetHUDWidget) (Variables|HUDSettings|GetDisplayDate) (Variables|HUDSettings|GetDisplayTime)) ; Update time and date on UI clock.
  (return) ; Done.
)

(fn ToggleStatsStyle
  ;[1 1 1] Retrieve and store references to the two different stat panels.
  (bind (_verticalstyle _horizontalstyle) (Class|BPIntHUD|GetStatPanels(Message) (Variables|HUDSettings|GetHUDWidget)))
  (LocalVariables|SetVPanel _verticalstyle)
  (LocalVariables|SetHPanel _horizontalstyle)
  (if (Variables|HUDSettings|GetVerticalStats) ; Is this player set to use a vertical style HUD?
    (Widget|SetVisibility (LocalVariables|GetVPanel) "Visible") ; Show the vertical stats HUD.
    (Widget|SetVisibility (LocalVariables|GetHPanel) "Hidden") ; Hide the horizontal stats HUD.
    (else
      (Widget|SetVisibility (LocalVariables|GetVPanel) "Hidden") ; Hide the vertical stats HUD.
      (Widget|SetVisibility (LocalVariables|GetHPanel) "Visible") ; Show the horizontal stats HUD.
    ))
  (return) ; Done.
)

(fn UpdateCompass
  (Utilities|IsValid (Variables|HUDSettings|GetCompassMaterial) ; Is the compass material valid?
    (:Is%20Valid
      (Rendering|Material|SetScalarParameterValue (Variables|HUDSettings|GetCompassMaterial) "PlayerInput" (/ (.Yaw (Math|Rotator|BreakRotator (Pawn|GetControlRotation (Variables|HUDSettings|GetPlayerController) :!class /Script/Engine.Controller))) 3.6e+02) :!class /Script/Engine.MaterialInstanceDynamic) ; Update compass rotation based on player direction.
      (return) ; Done.
    )
    (:Is%20Not%20Valid
      (return) ; Invalid material. Do nothing.
    )))

(fn ToggleWidget
  (params (ForceVisibilityOn :type Boolean) (ForceVisibilityOff :type Boolean))
  (if ForceVisibilityOn ; Are we forcing the HUD to be visible?
    (Class|BPIntHUD|ToggleHUD(Message) (Variables|HUDSettings|GetHUDWidget) true) ; Show the HUD.
    (Variables|HUDSettings|SetHUDOn true) ; Set HUDOn to reflect current HUD visibility.
    (elif ForceVisibilityOff ; Are we forcing the HUD to be hidden?
      (Class|BPIntHUD|ToggleHUD(Message) (Variables|HUDSettings|GetHUDWidget) false :!label _label) ; Hide the HUD.
      (Variables|HUDSettings|SetHUDOn false) ; Set HUDOn to reflect current HUD visibility.
      (elif (Variables|HUDSettings|GetHUDOn) ; Is the HUD currently visible or not?
        (goto _label)
        (else
          (Class|BPIntHUD|ToggleHUD(Message) (Variables|HUDSettings|GetHUDWidget) true) ; Show the HUD.
          (Variables|HUDSettings|SetHUDOn true) ; Set HUDOn to reflect current HUD visibility.
        ))))
  (return) ; Done.
)

(fn InteractiveTrace
  (bind _playercontroller (Variables|HUDSettings|GetPlayerController))
  (bind _playercameramanager (Variables|/Script/Engine.PlayerController|GetPlayerCameraManager _playercontroller))
  (bind _returnvalue (Camera|GetCameraLocation _playercameramanager))
  (InteractiveOutline|GetLivingPlayers) ; Update AlivePlayers array.
  (Utilities|IsValid (Variables|HUDSettings|GetControlledChar) ; Make sure there is a valid character.
    (:Is%20Valid
      (bind _boom (Class|BPIntCharacter|GetCamera(Message) (Variables|HUDSettings|GetControlledChar))) ; Retrieve player camera location.
      (Utilities|IsValid _boom ; Is a valid spring arm attached to the character?
        (:Is%20Valid
          (LocalVariables|SetArmLength (Variables|/Script/Engine.SpringArmComponent|GetTargetArmLength _boom)) ; Use spring arm length.
        )
        (:Is%20Not%20Valid
          (LocalVariables|SetArmLength 0.0) ; No spring arm, use zero.
        ))
      (bind (_outhit _returnvalue_2) (Collision|LineTraceByChannel _returnvalue (+ _returnvalue (* (Transformation|GetActorForwardVector _playercameramanager) (+ (Variables|HUDSettings|GetReach) (LocalVariables|GetArmLength)))) "TraceTypeQuery1" false (Variables|HUDSettings|GetAlivePlayers) "None")) ; Perform a trace from the player's head to look for interactive items.
      (if _returnvalue_2 ; Did the tract hit something?
        (return (.HitActor (Collision|BreakHitResult _outhit)) (.ImpactPoint (Collision|BreakHitResult _outhit))) ; Set output to actor hit.
        (else
          (return 0 (.TraceEnd (Collision|BreakHitResult _outhit))) ; Set output to null.
        )))
    (:Is%20Not%20Valid
      (return 0 "0, 0, 0") ; Do nothing.
    )))

(fn GetLivingPlayers
  (Utilities|Array|Clear (Variables|HUDSettings|GetAlivePlayers)) ; Clear array for use.
  (bind _outactors (Actor|GetAllActorsOfClass "/Script/Engine.Character")) ; Get all instances of SurvivalCharacters, living and dead.
  (for _array_element _outactors ; For every instance...
    (bind _isdead (Class|BPIntCharacter|GetLifeState(Message) _array_element)) ; Retrieve character life state.
    (if (not _isdead) ; Check life state of character.
      (Utilities|Array|Add (Variables|HUDSettings|GetAlivePlayers) _array_element) ; If alive, add to characters to ignore.
    ))
  (return) ; Done.
)

(fn AddNewFeedbackItem
  (params (Text :type Text))
  (bind _output_get (LocalVariables|SetInput Text))
  (if (Utilities|Enum|Equal(Enum) _output_get (Class|KismetTextLibrary|GetEmptyText))
    _
    (else
      (Utilities|Array|Insert (Variables|HUDSettings|GetFeedbackText) (Utilities|Struct|MakeStr_SGT_FeedbackItem (LocalVariables|GetInput) (Variables|HUDSettings|GetFeedbackLifetime)))))
  (Utilities|Array|Resize (Variables|HUDSettings|GetFeedbackText) 6)
  (bind _scroller (Class|BPIntHUD|GetFeedbackScroller(Message) (Variables|HUDSettings|GetHUDWidget)))
  (bind _output_get_2 (LocalVariables|SetScroller _scroller))
  (Widget|Panel|ClearChildren _output_get_2)
  (bind _arrayelement (Utilities|ReverseforEachLoop (Variables|HUDSettings|GetFeedbackText))
    (:LoopBody
      (bind _returnvalue (UserInterface|CreateWidget "/Game/SGT/Blueprints/HUD/W_SGT_Feedback.W_SGT_Feedback_C"))
      (Rendering|Components|TextRender|SetText (Variables|/Game/SGT/Blueprints/HUD/W_SGT_Feedback.W_SGT_Feedback_C|GetFeedbackText _returnvalue) (Utilities|Struct|BreakStr_SGT_FeedbackItem _arrayelement))
      (Widget|Panel|AddChild (LocalVariables|GetScroller) _returnvalue))
    (:Completed
      (if (< (Class|PanelWidget|GetChildrenCount (LocalVariables|GetScroller)) 4) :!label _label
        (bind _returnvalue_2 (UserInterface|CreateWidget "/Game/SGT/Blueprints/HUD/W_SGT_Feedback.W_SGT_Feedback_C"))
        (Widget|Panel|AddChild (LocalVariables|GetScroller) _returnvalue_2)
        (goto _label)
        (else
          (return) ; Done.
        )))))

(fn UpdateFeedbackScroller
  (for (_array_element _array_index) (Variables|HUDSettings|GetFeedbackText)
    (LocalVariables|SetData _array_element)
    (LocalVariables|SetIndex _array_index)
    (if (Math|Float|NearlyEqual(Float) (.Lifetime (Utilities|Struct|BreakStr_SGT_FeedbackItem _array_element)) 0.0 1e-06)
      (Utilities|Array|RemoveIndex (Variables|HUDSettings|GetFeedbackText) (LocalVariables|GetIndex))
      (else
        (Utilities|Array|SetArrayElem (Variables|HUDSettings|GetFeedbackText) _array_index (Utilities|Struct|MakeStr_SGT_FeedbackItem (.Text (Utilities|Struct|BreakStr_SGT_FeedbackItem _array_element)) (Math|Float|Clamp(Float) (- (.Lifetime (Utilities|Struct|BreakStr_SGT_FeedbackItem _array_element)) 0.5) 0.0 (Variables|HUDSettings|GetFeedbackLifetime))))))))

(fn ParseHUDWidget
  (return (Variables|HUDSettings|GetHUDWidget)))