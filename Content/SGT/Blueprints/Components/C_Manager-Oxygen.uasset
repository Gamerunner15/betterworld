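; Oxygen manager component that drains, restores and tracks player oxygen, applying damage when it runs out.
; Overlap-counted volumes mark oxygen-free zones, or safe zones when AlwaysDrain is set.
; UpdateOxygen acts as a state machine, switching looping Hypoxia, Recovery and Asphyxiation timers whose ticks run with authority and call it again.
; It also drives the HUD, an optional low-oxygen visual effect and an optional stamina cap reduction during asphyxiation.
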(event Custom|UpdateHUD
  (params (Oxygen :type Float%20%28single-precision%29))
  (bind _hudmanager (Variables|OxygenSettings|GetHUDManager))
  ;[0.2 1 0.2 0.5] Update player HUD.
  (if (not (Variables|OxygenSettings|GetDisableSystem)) ; DEBUG: Is the oxygen system set to\ndisabled?
    (Utilities|IsValid _hudmanager ; Is the HUD manager reference valid?
      (:Is%20Valid
        (Variables|/Game/SGT/Blueprints/Components/C_Manager-HUD.C_Manager-HUD_C|SetOxygen _hudmanager Oxygen) ; Update player HUD.
      ))))

(event Custom|AddOxygen
  (params (AmountToAdd :type Float%20%28single-precision%29))
  ;[1 0.2 0.2 0.5] Take input oxygen and add to the current oxygen, clamping within max oxygen.
  (if (not (Variables|OxygenSettings|GetDisableSystem)) ; DEBUG: Is the oxygen system set to\ndisabled?
    (Variables|OxygenSettings|SetPlayerOxygen (Math|Float|Clamp(Float) (+ (Variables|OxygenSettings|GetPlayerOxygen) AmountToAdd) 0.0 (Variables|OxygenSettings|GetMaxPlayerOxygen))) ; Update oxygen value.
    (CallFunction|UpdateOxygen) ; Run oxygen update.
  ))

(event Custom|VolumeExit
  ;[1 0.2 0.2 0.5] Lower volume overlaps count by 1. If that was the last one, reset oxy free state.
  (if (not (Variables|OxygenSettings|GetDisableSystem)) ; DEBUG: Is the oxygen system set to\ndisabled?
    (if (not (== (Variables|OxygenSettings|GetVolumeOverlaps) 0)) ; Is the volume overlaps already zero?
      (bind _result (Math|Integer|DecrementInt (Variables|OxygenSettings|GetVolumeOverlaps)) ; Decrement VolumeOverlaps count.
        (:%20%20
          (if (== _result 0) ; Did the player just exit the only remaining volume overlap?
            (if (Variables|OxygenSettings|GetAlwaysDrain) ; Is the oxygen system set to always\ndrain?
              (Variables|OxygenSettings|SetInOxyFree true) ; Set oxy free state back to true.
              (else
                (Variables|OxygenSettings|SetInOxyFree false) ; Set oxy free state back to false.
              ))))))))

(event Custom|Asphyxiation
  ;[1 0.2 0.2 0.5] Apply damage to the player when they are asphyxiating.
  (if (not (Variables|OxygenSettings|GetDisableSystem)) ; DEBUG: Is the oxygen system set to\ndisabled?
    (Utilities|SwitchHasAuthority ; Ensure this only runs on the server.
      (:Authority
        (Game|Damage|ApplyDamage (Variables|OxygenSettings|GetPlayerController) (* (Variables|OxygenSettings|GetAsphyxiationDamage) (/ 1.0 (Math|Conversions|ToFloat(Integer) (Variables|OxygenSettings|GetUpdateFrequency)))) 0 0 "/Game/SGT/Blueprints/Misc/Damage_Statistical.Damage_Statistical_C") ; Apply damage to player.
        (CallFunction|UpdateOxygen) ; Run oxygen update.
      ))))

(event Custom|Recovery
  ;[1 0.2 0.2 0.5] Recovery oxygen based on update frequency and recovery rate.
  (if (not (Variables|OxygenSettings|GetDisableSystem)) ; DEBUG: Is the oxygen system set to\ndisabled?
    (Utilities|SwitchHasAuthority ; Ensure this only runs on the server.
      (:Authority
        (Variables|OxygenSettings|SetPlayerOxygen (Math|Float|Clamp(Float) (+ (Variables|OxygenSettings|GetPlayerOxygen) (/ (Variables|OxygenSettings|GetRecoveryRate) (Math|Conversions|ToFloat(Integer) (Variables|OxygenSettings|GetUpdateFrequency)))) 0.0 (Variables|OxygenSettings|GetMaxPlayerOxygen))) ; Update oxygen value.
        (CallFunction|UpdateOxygen) ; Run oxygen update.
      ))))

(event Custom|VolumeTriggered
  ;[1 0.2 0.2 0.5] Set oxy free to opposing state to normal on overlap and record number of volumes active.
  (if (not (Variables|OxygenSettings|GetDisableSystem)) ; DEBUG: Is the oxygen system set to\ndisabled?
    (if (Variables|OxygenSettings|GetAlwaysDrain) ; Is the oxygen system set to always\ndrain?
      (Variables|OxygenSettings|SetInOxyFree false) ; As this volume represents an oxygen\nsafe house, clear InOxyFree bool.
      (else
        (Variables|OxygenSettings|SetInOxyFree true) ; As this volume represents an oxygen\nfree zone, set InOxyFree bool to true.
      ))
    (Math|Integer|IncrementInt (Variables|OxygenSettings|GetVolumeOverlaps)) ; Increment VolumeOverlaps count.
  ))

(event Custom|Hypoxia
  ;[1 0.2 0.2 0.5] Decay oxygen while player is in a state of hypoxia based on update frequency and drain rate.
  (if (not (Variables|OxygenSettings|GetDisableSystem)) ; DEBUG: Is the oxygen system set to\ndisabled?
    (Utilities|SwitchHasAuthority ; Ensure this only runs on the server.
      (:Authority
        (Variables|OxygenSettings|SetPlayerOxygen (Math|Float|Clamp(Float) (- (Variables|OxygenSettings|GetPlayerOxygen) (/ (Variables|OxygenSettings|GetDrainRate) (Math|Conversions|ToFloat(Integer) (Variables|OxygenSettings|GetUpdateFrequency)))) 0.0 (Variables|OxygenSettings|GetMaxPlayerOxygen))) ; Update oxygen value.
        (CallFunction|UpdateOxygen) ; Run oxygen update.
      ))))

(event EventVolumeTriggeredEvent
  ;[1 0.2 0.2 0.5] Volume triggered sequence.
  (if (not (Variables|OxygenSettings|GetDisableSystem)) ; DEBUG: Is the oxygen system set to\ndisabled?
    (Utilities|SwitchHasAuthority ; Ensure this only runs on the server.
      (:Authority
        (CallFunction|VolumeTriggered) ; Trigger the oxygen volume event.
      ))))

(event EventVolumeExitEvent
  ;[1 0.2 0.2 0.5] Volume exit sequence.
  (if (not (Variables|OxygenSettings|GetDisableSystem)) ; DEBUG: Is the oxygen system set to\ndisabled?
    (Utilities|SwitchHasAuthority ; Ensure this only runs on the server.
      (:Authority
        (CallFunction|VolumeExit) ; Trigger the oxygen volume exit event.
      ))))

(event EventReset
  ;[0.2 1 0.2 0.5] Force reset prior to death.
  (if (not (Variables|OxygenSettings|GetDisableSystem)) ; DEBUG: Is the oxygen system set to\ndisabled?
    (Utilities|Time|ClearandInvalidateTimerbyHandle (Variables|OxygenSettings|GetHypoxiaTimer))
    (Variables|OxygenSettings|SetHypoxiaActive false)
    (Utilities|Time|ClearandInvalidateTimerbyHandle (Variables|OxygenSettings|GetRecoveryTimer))
    (Variables|OxygenSettings|SetRecoveryActive false)
    (Utilities|Time|ClearandInvalidateTimerbyHandle (Variables|OxygenSettings|GetAsphyxiationTimer))
    (Variables|OxygenSettings|SetIsAsphyxiating false)
    (Variables|OxygenSettings|SetVisualEffectActive false) ; Reset visual effect state bool.
    (Variables|OxygenSettings|SetStaminaLimited false) ; Reset stamina limited state bool.
    (Variables|OxygenSettings|SetPlayerOxygen (Variables|OxygenSettings|GetMaxPlayerOxygen)) ; Initialize oxygen value.
  ))

(event EventInitialize
  (params (PlayerController :type Player%20Controller%20Object%20Reference))
  ;[0.2 1 0.2 0.5] Initialize oxygen system.
  (if (not (Variables|OxygenSettings|GetDisableSystem)) ; DEBUG: Is the oxygen system set to\ndisabled?
    (Variables|OxygenSettings|SetPlayerController PlayerController) ; Set reference to controller.
    (bind (_no_hud _hudcomponent _novisualeffects _visualeffectscomponent _nostamina _staminacomponent) (CallFunction|CommonComponents (Variables|OxygenSettings|GetPlayerController) (Utilities|Enum|NotEqual(Enum) (Variables|OxygenSettings|GetLowOxygenVisualEffect) "NewEnumerator11") (Variables|OxygenSettings|GetLimitStamina))) ; Retrieve common components from player controller.
    (if _no_hud ; Was there no HUD manager found?
      _
      (else
        (Variables|OxygenSettings|SetHUDManager _hudcomponent) ; Set reference to HUD manager.
      ))
    (if _novisualeffects ; Was there no visual feedback manager\nfound in the player controller?
      (Variables|OxygenSettings|SetLowOxygenVisualEffect "NewEnumerator11") ; As no valid visual feedback manager was found,\nforce effect to none.
      (else
        (Variables|OxygenSettings|SetVisualFeedbackManager _visualeffectscomponent) ; Set reference to Visual Feedback manager.
      ))
    (if _nostamina ; Was there no stamina manager found\nin the player controller?
      (Variables|OxygenSettings|SetLimitStamina false) ; As no valid stamina manager exists,\nforce LimitStamina to false.
      (else
        (Variables|OxygenSettings|SetStaminaManager _staminacomponent) ; Set reference to Stamina manager.
      ))
    (Variables|OxygenSettings|SetPlayerOxygen (Variables|OxygenSettings|GetMaxPlayerOxygen)) ; Initialize oxygen value.
    (if (Variables|OxygenSettings|GetAlwaysDrain) ; Is the system set up for always drain?
      (Variables|OxygenSettings|SetInOxyFree true)
      (else
        (Variables|OxygenSettings|SetInOxyFree false)))
    (CallFunction|UpdateOxygen) ; Run oxygen update.
    (Variables|OxygenSettings|SetVolumeOverlaps 0) ; Set initial overlap count.
  ))

(fn UpdateOxygen
  (bind _playercontroller (Variables|OxygenSettings|GetPlayerController))
  (bind _hudmanager (Variables|OxygenSettings|GetHUDManager))
  (Utilities|IsValid _playercontroller ; Is the player controller reference valid?
    (:Is%20Valid
      (bind _isdead (Class|BPintController|GetLifeState(Message) _playercontroller)) ; Return current life state of the player.
      (if _isdead ; Is the player dead?
        (return) ; Done.
        (elif (<= (Variables|OxygenSettings|GetPlayerOxygen) 0.0) ; Is the player completely drained of oxygen?
          (if (Variables|OxygenSettings|GetInOxyFree) ; Is the player currently in an Oxygen Free environment?
            (if (Variables|OxygenSettings|GetRecoveryActive) ; Is player oxygen recovery active?
              (Utilities|Time|ClearandInvalidateTimerbyHandle (Variables|OxygenSettings|GetRecoveryTimer)) ; Stop the hypoxia timer.
              (Variables|OxygenSettings|SetRecoveryActive false) ; Update hypoxia state bool.
            )
            (if (Variables|OxygenSettings|GetHypoxiaActive) ; Is the player already in a state of hypoxia?
              (Utilities|Time|ClearandInvalidateTimerbyHandle (Variables|OxygenSettings|GetHypoxiaTimer)) ; Stop the hypoxia timer.
              (Variables|OxygenSettings|SetHypoxiaActive false) ; Update hypoxia state bool.
            )
            (if (Variables|OxygenSettings|GetIsAsphyxiating) ; Is the player asphyxiating?
              (return) ; Done.
              (else
                (bind _returnvalue (Utilities|Time|SetTimerbyFunctionName 0 "Asphyxiation" (/ 1.0 (Math|Conversions|ToFloat(Integer) (Variables|OxygenSettings|GetUpdateFrequency))) true)) ; Start the asphyxiation loop.
                (Variables|OxygenSettings|SetAsphyxiationTimer _returnvalue) ; Store a reference to the asphyxiation\ntimer for use.
                (Variables|OxygenSettings|SetIsAsphyxiating true) ; Update asphyxiation state bool.
                (Utilities|IsValid _hudmanager ; Is the HUD manager reference valid?
                  (:Is%20Valid
                    (Default|UpdateFeedback _hudmanager "You are asphysxiating and will soon die without oxygen.") ; Notify player of asphyxiation.
                  )
                  (:Is%20Not%20Valid
                    _))
                (if (Variables|OxygenSettings|GetLimitStamina) ; Should the player's stamina be limited if they are asphyxiating?
                  (if (Variables|OxygenSettings|GetStaminaLimited)
                    (return) ; Done.
                    (else
                      (Default|LowerCap (Variables|OxygenSettings|GetStaminaManager) (Variables|OxygenSettings|GetStaminaReduction)) ; Lower the player's stamina cap.
                      (Variables|OxygenSettings|SetStaminaLimited true) ; Update limited stamina state bool.
                      (return) ; Done.
                    ))
                  (else
                    (return) ; Done.
                  ))))
            (else
              (if (Variables|OxygenSettings|GetHypoxiaActive) ; Is the player already in a state of hypoxia?
                (Utilities|Time|ClearandInvalidateTimerbyHandle (Variables|OxygenSettings|GetHypoxiaTimer)) ; Stop the hypoxia timer.
                (Variables|OxygenSettings|SetHypoxiaActive false) ; Update hypoxia state bool.
              )
              (if (Variables|OxygenSettings|GetIsAsphyxiating) ; Is the player asphyxiating?
                (Utilities|Time|ClearandInvalidateTimerbyHandle (Variables|OxygenSettings|GetAsphyxiationTimer)) ; Stop the asphyxiation timer.
                (Variables|OxygenSettings|SetIsAsphyxiating false) ; Update asphyxiation state bool.
              )
              (if (Variables|OxygenSettings|GetRecoveryActive) ; Is player oxygen recovery active?
                (return) ; Done.
                (else
                  (bind _returnvalue_2 (Utilities|Time|SetTimerbyFunctionName 0 "Recovery" (/ 1.0 (Math|Conversions|ToFloat(Integer) (Variables|OxygenSettings|GetUpdateFrequency))) true)) ; Start the recovery loop.
                  (Variables|OxygenSettings|SetRecoveryTimer _returnvalue_2) ; Store a reference to the recovery\ntimer for use.
                  (Variables|OxygenSettings|SetRecoveryActive true) ; Update recovery state bool.
                  (return) ; Done.
                ))))
          (else
            (CallFunction|UpdateVisualEffect) ; Run visual effect update.
            (if (Variables|OxygenSettings|GetIsAsphyxiating) ; Is the player asphyxiating?
              (Utilities|Time|ClearandInvalidateTimerbyHandle (Variables|OxygenSettings|GetAsphyxiationTimer)) ; Stop the asphyxiation timer.
              (Variables|OxygenSettings|SetIsAsphyxiating false) ; Update asphyxiation state bool.
            )
            (if (Variables|OxygenSettings|GetInOxyFree) ; Is the player currently in an Oxygen Free environment?
              (if (Variables|OxygenSettings|GetRecoveryActive) ; Is player oxygen recovery active?
                (Utilities|Time|ClearandInvalidateTimerbyHandle (Variables|OxygenSettings|GetRecoveryTimer)) ; Stop the recovery timer.
                (Variables|OxygenSettings|SetRecoveryActive false) ; Update recovery state bool.
              )
              (if (Variables|OxygenSettings|GetHypoxiaActive) ; Is the player already in a state of hypoxia?
                _
                (else
                  (bind _returnvalue_3 (Utilities|Time|SetTimerbyFunctionName 0 "Hypoxia" (/ 1.0 (Math|Conversions|ToFloat(Integer) (Variables|OxygenSettings|GetUpdateFrequency))) true)) ; Start the hypoxia loop.
                  (Variables|OxygenSettings|SetHypoxiaTimer _returnvalue_3) ; Store a reference to the hypoxia\ntimer for use.
                  (Variables|OxygenSettings|SetHypoxiaActive true) ; Update hypoxia state bool.
                ))
              (CallFunction|UpdateHUD (/ (Variables|OxygenSettings|GetPlayerOxygen) (Variables|OxygenSettings|GetMaxPlayerOxygen))) ; Update the player HUD.
              (return) ; Done.
              (else
                (if (Variables|OxygenSettings|GetHypoxiaActive) ; Is the player already in a state of hypoxia?
                  (Utilities|Time|ClearandInvalidateTimerbyHandle (Variables|OxygenSettings|GetHypoxiaTimer)) ; Stop the hypoxia timer.
                  (Variables|OxygenSettings|SetHypoxiaActive false) ; Update hypoxia state bool.
                )
                (if (Variables|OxygenSettings|GetStaminaLimited) ; Was the player's stamina previously limited?
                  (Default|RaiseCap (Variables|OxygenSettings|GetStaminaManager) (Variables|OxygenSettings|GetStaminaReduction)) ; Raise the stamina cap appropriately.
                  (Variables|OxygenSettings|SetStaminaLimited false) ; Update stamina limited bool.
                )
                (if (Variables|OxygenSettings|GetRecoveryActive) ; Is player oxygen recovery active?
                  _
                  (else
                    (bind _returnvalue_4 (Utilities|Time|SetTimerbyFunctionName 0 "Recovery" (/ 1.0 (Math|Conversions|ToFloat(Integer) (Variables|OxygenSettings|GetUpdateFrequency))) true)) ; Start the recovery loop.
                    (Variables|OxygenSettings|SetRecoveryTimer _returnvalue_4) ; Store a reference to the recovery\ntimer for use.
                    (Variables|OxygenSettings|SetRecoveryActive true) ; Update recovery state bool.
                  ))
                (CallFunction|UpdateHUD (/ (Variables|OxygenSettings|GetPlayerOxygen) (Variables|OxygenSettings|GetMaxPlayerOxygen))) ; Update the player HUD.
                (return) ; Done.
              ))))))
    (:Is%20Not%20Valid
      (return) ; Done.
    )))

(fn UpdateVisualEffect
  (if (Utilities|Enum|NotEqual(Enum) (Variables|OxygenSettings|GetLowOxygenVisualEffect) "NewEnumerator11") ; Is a visual effect enabled?
    (if (Variables|OxygenSettings|GetVisualEffectActive) ; Is the visual effect currently active?
      (if (<= (Variables|OxygenSettings|GetPlayerOxygen) (Variables|OxygenSettings|GetVisualEffectThreshold)) ; Is the player's water below the visual effect threshold level?
        _
        (else
          (Default|EffectControl (Variables|OxygenSettings|GetVisualFeedbackManager) (Variables|OxygenSettings|GetLowOxygenVisualEffect) true) ; Begin the sequence to turn the visual effect off.
          (Variables|OxygenSettings|SetVisualEffectActive false) ; Update visual effect state bool.
          (return) ; Done.
        ))
      (elif (> (Variables|OxygenSettings|GetPlayerOxygen) (Variables|OxygenSettings|GetVisualEffectThreshold)) ; Is the player's water above the visual effect threshold level?
        _
        (else
          (Default|EffectControl (Variables|OxygenSettings|GetVisualFeedbackManager) (Variables|OxygenSettings|GetLowOxygenVisualEffect) false) ; Begin the sequence to turn the visual effect on.
          (Variables|OxygenSettings|SetVisualEffectActive true) ; Update visual effect state bool.
          (return) ; Done.
        )))
    (return) ; Done.
    (else
      (return) ; Done.
    )))