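; Movement manager component that handles sprint, crouch, prone, jump and temporary speed overrides for a player-controlled Character.
; Switch functions check movement allowance, then the authority sets state, walk speed, view limits and stance camera offsets.
; Remote clients forward requests to the server while applying speed changes and jump launches locally.
; An optional stamina manager link charges jumps and drains during moving sprints, using a looping timer to end sprint on depletion.
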(event Custom|ToggleProne
  ;[1 0.2 0.2 0.5] Toggle prone on and off.
  (Movement|ProneSwitch))

(event Custom|SRV_Jump
  ;[1 0.2 0.2 0.5] Player jump.
  (Movement|Jump|JumpSwitch))

(event Custom|SRV_ToggleProne
  ;[1 0.2 0.2 0.5] Toggle prone on and off.
  (Movement|ProneSwitch))

(event Custom|SRV_ToggleSprint
  (params (State :type Boolean))
  ;[1 0.2 0.2 0.5] Toggle sprinting on and off.
  (Movement|SprintSwitch State))

(event Custom|ToggleSprint
  (params (State :type Boolean))
  ;[1 0.2 0.2 0.5] Toggle sprinting on and off.
  (Movement|SprintSwitch State))

(event Custom|ToggleCrouch
  ;[1 0.2 0.2 0.5] Toggle crouching on and off.
  (Movement|CrouchSwitch))

(event Custom|TemporarySpeed
  (params (State :type Boolean) (NewSpeed :type Float%20%28single-precision%29))
  ;[1 0.2 0.2 0.5] Set a new speed temporarily.
  (Movement|SetTemporarySpeed State NewSpeed))

(event Custom|Jump
  ;[1 0.2 0.2 0.5] Player jump.
  (Movement|Jump|JumpSwitch))

(event Custom|SRV_ToggleCrouch
  ;[1 0.2 0.2 0.5] Toggle crouching on and off.
  (Movement|CrouchSwitch))

(event Custom|SRV_TemporarySpeed
  (params (State :type Boolean) (NewSpeed :type Float%20%28single-precision%29))
  ;[1 0.2 0.2 0.5] Set a new speed temporarily.
  (Movement|SetTemporarySpeed State NewSpeed))

(event EventReset
  (Utilities|Time|ClearandInvalidateTimerbyHandle (Variables|SprintSettings|GetStaminaSprintTimer)) ; Force stop the stamina sprint timer.
  (Variables|SprintSettings|SetIsSprinting false) ; Ensure player sprint is OFF by default.
  (Variables|CrouchSettings|SetIsCrouched false) ; Ensure player crouch is OFF by default.
  (Variables|ProneSettings|SetIsProne false) ; Ensure player prone is OFF by default.
)

(event EventInitialize
  (params (PlayerController :type Player%20Controller%20Object%20Reference))
  ;[0.2 1 0.2 0.5] Initialize movement system.
  (bind _output_get (Variables|BaseMovementSettings|SetPlayerController PlayerController)) ; Save reference to controller.
  (bind _ascharacter (Utilities|Casting|CastToCharacter (Pawn|GetControlledPawn _output_get))) ; Check if the pawn is a derivative of the base character class.
  (Variables|BaseMovementSettings|SetControlledChar _ascharacter) ; Store reference to base character.
  (Utilities|IsValid (Actor|GetComponentbyClass (Variables|BaseMovementSettings|GetPlayerController) "/Game/SGT/Blueprints/Components/C_Manager-Stamina.C_Manager-Stamina_C") ; Does the controller have a valid stamina manager attached?
    (:Is%20Valid
      (Variables|BaseMovementSettings|SetManager-Stamina (Actor|GetComponentbyClass (Variables|BaseMovementSettings|GetPlayerController) "/Game/SGT/Blueprints/Components/C_Manager-Stamina.C_Manager-Stamina_C")) ; Set reference to stamina manager component.
    )
    (:Is%20Not%20Valid
      _))
  (Variables|SprintSettings|SetIsSprinting false) ; Ensure player sprint is OFF by default.
  (Variables|CrouchSettings|SetIsCrouched false) ; Ensure player crouch is OFF by default.
  (Variables|ProneSettings|SetIsProne false) ; Ensure player prone is OFF by default.
  (Utilities|UpdateViewAngles true))

(fn CheckStaminaforSprint
  (bind _manager_stamina (Variables|BaseMovementSettings|GetManager-Stamina))
  (bind _staminavalue (Default|GetStamina _manager_stamina)) ; Get the current player stamina.
  (if (<= (- _staminavalue (/ (Variables|SprintSettings|GetStaminaDrainOnSprint) (Math|Conversions|ToFloat(Integer) (Variables|/Game/SGT/Blueprints/Components/C_Manager-Stamina.C_Manager-Stamina_C|GetUpdateFrequency _manager_stamina)))) 0.0) ; Has the player's stamina depleted?
    (Movement|SprintSwitch false) ; Deactivate sprint.
    (return) ; Done.
    (elif (> (Math|Vector|VectorLength (Transformation|GetVelocity (Variables|BaseMovementSettings|GetControlledChar))) 0.0) ; Is the player currently moving?
      (if (Variables|SprintSettings|GetSprintDecayActive) ; Is sprint decay already active?
        (return) ; Done.
        (else
          (Default|SetDecay (Variables|BaseMovementSettings|GetManager-Stamina) (Variables|SprintSettings|GetStaminaDrainOnSprint)) ; Add a drain to the stamina associated with sprinting.
          (Variables|SprintSettings|SetSprintDecayActive true) ; Set bool to reflect sprint decay state.
          (return) ; Done.
        ))
      (elif (Variables|SprintSettings|GetSprintDecayActive) ; Is sprint decay already active?
        (Default|SetDecay (Variables|BaseMovementSettings|GetManager-Stamina) (* -1 (Variables|SprintSettings|GetStaminaDrainOnSprint))) ; Add a drain to the stamina associated with sprinting.
        (Variables|SprintSettings|SetSprintDecayActive false) ; Set bool to reflect sprint decay state.
        (return) ; Done.
        (else
          (return) ; Done.
        )))))

(fn JumpSwitch
  (bind _jump (CallFunction|QueryMovementAllowance)) ; Check current movement allowance...
  (if _jump ; Can the player currently prone?
    (Utilities|SwitchHasAuthority ; Does the player have authority?
      (:Authority
        (if (Variables|JumpSettings|GetJumpRequiresStamina) ; Does jumping require stamina?
          (bind _staminavalue (Default|GetStamina (Variables|BaseMovementSettings|GetManager-Stamina))) ; Get the current player stamina.
          (if (> _staminavalue 0.0) ; Does the player currently have any stamina remaining?
            (Default|ConsumeStamina (Variables|BaseMovementSettings|GetManager-Stamina) (Variables|JumpSettings|GetStaminaDrainOnJump)) ; Consume appropriate stamina amount.
            (else
              (return) ; Done.
            ))))
      (:Remote
        (CallFunction|SRVJump) ; Run this again on the server.
      ))
    (Movement|Jump|CallJump (Movement|Jump|GetJumpVelocity)) ; Jump.
    (return) ; Done.
    (else
      (return) ; Done.
    )))

(fn CallJump
  (params (Jump%20Velocity :type Float%20%28single-precision%29))
  (bind _output_get (Variables|/Script/Engine.CharacterMovementComponent|SetJumpZVelocity (Variables|/Script/Engine.Character|GetCharacterMovement (Variables|BaseMovementSettings|GetControlledChar)) Jump%20Velocity)) ; Update player jump velocity.
  (Character|LaunchCharacter (Variables|BaseMovementSettings|GetControlledChar) (Math|Vector|MakeVector 0.0 0.0 _output_get) false false) ; Jump.
  (return) ; Done.
)

(fn GetJumpVelocity
  (if (Variables|JumpSettings|GetJumpHigherWhenSprinting) ; Are players meant to be able to jump higher whislt sprinting?
    (if (Variables|SprintSettings|GetIsSprinting) ; Is the player currently sprinting?
      (return (Variables|JumpSettings|GetJumpVelocityWhenSprinting)) ; Done.
      (else
        _)))
  (return (Variables|JumpSettings|GetJumpVelocity)) ; Done.
)

(fn CrouchSwitch
  (bind _crouch (CallFunction|QueryMovementAllowance)) ; Check current movement allowance...
  (if _crouch ; Can the player currently crouch?
    (Utilities|SwitchHasAuthority ; Does the player have authority?
      (:Authority
        (if (not (Variables|CrouchSettings|GetIsCrouched)) ; Is the player entering or leaving crouch?
          (bind _camera (Class|BPIntCharacter|GetCamera(Message) (Variables|BaseMovementSettings|GetControlledChar))) ; Get player camera.
          (Transformation|SetRelativeLocation _camera (Math|Vector|MakeVector (.X (Math|Vector|BreakVector (.Location (Math|Transform|BreakTransform (Transformation|GetRelativeTransform _camera))))) (.Y (Math|Vector|BreakVector (.Location (Math|Transform|BreakTransform (Transformation|GetRelativeTransform _camera))))) (- (.Z (Math|Vector|BreakVector (.Location (Math|Transform|BreakTransform (Transformation|GetRelativeTransform _camera))))) (Variables|CrouchSettings|GetCrouchCameraOffset))) true false) ; Adjust player camera based on CrouchCameraOffset.
          (Movement|SprintSwitch false) ; Ensure sprint is off.
          (Utilities|UpdatePlayerSpeed (Variables|CrouchSettings|GetCrouchWalkingSpeed)) ; Set character speed to crouch speed.
          (Utilities|UpdateViewAngles false (Variables|CrouchSettings|GetCrouchViewRange))
          (else
            (bind _camera_2 (Class|BPIntCharacter|GetCamera(Message) (Variables|BaseMovementSettings|GetControlledChar))) ; Get player camera.
            (Transformation|SetRelativeLocation _camera_2 (Math|Vector|MakeVector (.X (Math|Vector|BreakVector (.Location (Math|Transform|BreakTransform (Transformation|GetRelativeTransform _camera_2))))) (.Y (Math|Vector|BreakVector (.Location (Math|Transform|BreakTransform (Transformation|GetRelativeTransform _camera_2))))) (+ (.Z (Math|Vector|BreakVector (.Location (Math|Transform|BreakTransform (Transformation|GetRelativeTransform _camera_2))))) (Variables|CrouchSettings|GetCrouchCameraOffset))) true false) ; Adjust player camera based on CrouchCameraOffset.
            (Utilities|UpdatePlayerSpeed (Variables|BaseMovementSettings|GetBaseWalkSpeed)) ; Set character speed to walk speed.
            (Utilities|UpdateViewAngles true)))
        (bind _output_get (Variables|CrouchSettings|SetIsCrouched (not (Variables|CrouchSettings|GetIsCrouched)))) ; Update IsCrouched state.
        (Class|BPIntCharacter|SetCrouch(Message) (Variables|BaseMovementSettings|GetControlledChar) _output_get) ; Parse crouched state to character.
        (return) ; Done.
      )
      (:Remote
        (CallFunction|SRVToggleCrouch) ; Run this again on the server.
        (if (not (Variables|CrouchSettings|GetIsCrouched)) ; Is the player entering or leaving crouch?
          (Utilities|UpdatePlayerSpeed (Variables|CrouchSettings|GetCrouchWalkingSpeed)) ; Set character speed to crouch speed.
          (else
            (Utilities|UpdatePlayerSpeed (Variables|BaseMovementSettings|GetBaseWalkSpeed)) ; Set character speed to walk speed.
          ))
        (return) ; Done.
      ))
    (else
      (return) ; Done.
    )))

(fn ProneSwitch
  (bind _prone (CallFunction|QueryMovementAllowance)) ; Check current movement allowance...
  (if _prone ; Can the player currently prone?
    (Utilities|SwitchHasAuthority ; Does the player have authority?
      (:Authority
        (if (not (Variables|ProneSettings|GetIsProne)) ; Is the player entering or leaving prone?
          (bind _camera (Class|BPIntCharacter|GetCamera(Message) (Variables|BaseMovementSettings|GetControlledChar))) ; Get player camera.
          (Transformation|SetRelativeLocation _camera (Math|Vector|MakeVector (.X (Math|Vector|BreakVector (.Location (Math|Transform|BreakTransform (Transformation|GetRelativeTransform _camera))))) (.Y (Math|Vector|BreakVector (.Location (Math|Transform|BreakTransform (Transformation|GetRelativeTransform _camera))))) (- (.Z (Math|Vector|BreakVector (.Location (Math|Transform|BreakTransform (Transformation|GetRelativeTransform _camera))))) (Variables|ProneSettings|GetProneCameraOffset))) true false) ; Adjust player camera based on CrouchCameraOffset.
          (Utilities|UpdatePlayerSpeed (Variables|ProneSettings|GetProneMoveSpeed)) ; Set character speed to prone speed.
          (Utilities|UpdateViewAngles false (Variables|ProneSettings|GetProneViewRange))
          (else
            (bind _camera_2 (Class|BPIntCharacter|GetCamera(Message) (Variables|BaseMovementSettings|GetControlledChar))) ; Get player camera.
            (Transformation|SetRelativeLocation _camera_2 (Math|Vector|MakeVector (.X (Math|Vector|BreakVector (.Location (Math|Transform|BreakTransform (Transformation|GetRelativeTransform _camera_2))))) (.Y (Math|Vector|BreakVector (.Location (Math|Transform|BreakTransform (Transformation|GetRelativeTransform _camera_2))))) (+ (.Z (Math|Vector|BreakVector (.Location (Math|Transform|BreakTransform (Transformation|GetRelativeTransform _camera_2))))) (Variables|ProneSettings|GetProneCameraOffset))) true false) ; Adjust player camera based on CrouchCameraOffset.
            (Utilities|UpdatePlayerSpeed (Variables|BaseMovementSettings|GetBaseWalkSpeed)) ; Set character speed to walk speed.
            (Utilities|UpdateViewAngles true)))
        (bind _output_get (Variables|ProneSettings|SetIsProne (not (Variables|ProneSettings|GetIsProne)))) ; Update IsProne state.
        (Class|BPIntCharacter|SetProne(Message) (Variables|BaseMovementSettings|GetControlledChar) _output_get) ; Parse prone state to character.
        (return) ; Done.
      )
      (:Remote
        (CallFunction|SRVToggleProne) ; Run this again on the server.
        (if (not (Variables|ProneSettings|GetIsProne)) ; Is the player entering or leaving prone?
          (Utilities|UpdatePlayerSpeed (Variables|ProneSettings|GetProneMoveSpeed)) ; Set character speed to prone speed.
          (else
            (Utilities|UpdatePlayerSpeed (Variables|BaseMovementSettings|GetBaseWalkSpeed)) ; Set character speed to walk speed.
          ))
        (return) ; Done.
      ))
    (else
      (return) ; Done.
    )))

(fn SprintSwitch
  (params (State :type Boolean))
  (bind _output_get (LocalVariables|SetSprintState State)) ; Store input for use.
  (if (Math|Boolean|Equal(Boolean) _output_get (Variables|SprintSettings|GetIsSprinting)) ; Is the player already in the right sprint state?
    (return) ; Done.
    (else
      (bind _sprint (CallFunction|QueryMovementAllowance)) ; Check current movement allowance...
      (if _sprint ; Can the player currently sprint?
        (Utilities|SwitchHasAuthority ; Does the player have authority?
          (:Authority
            (if (Variables|CrouchSettings|GetIsCrouched) ; Is the player currently crouched?
              (Movement|CrouchSwitch) ; Toggle crouching off.
            )
            (bind _output_get_2 (Variables|SprintSettings|SetIsSprinting (LocalVariables|GetSprintState))) ; Set IsSprinting state.
            (Class|BPIntCharacter|SetSprint(Message) (Variables|BaseMovementSettings|GetControlledChar) _output_get_2) ; Update sprint state in character.
            (if (LocalVariables|GetSprintState) ; Enable or disable sprint?
              (Utilities|UpdatePlayerSpeed (Variables|SprintSettings|GetSprintSpeed)) ; Set character speed to sprint speed.
              (Utilities|UpdateViewAngles false (Variables|SprintSettings|GetSprintViewRange))
              (else
                (Utilities|UpdatePlayerSpeed (Variables|BaseMovementSettings|GetBaseWalkSpeed)) ; Set character speed to walk speed.
                (Utilities|UpdateViewAngles true)))
            (if (Variables|SprintSettings|GetSprintRequiresStamina) ; Does sprinting consume stamina?
              (if (LocalVariables|GetSprintState) ; Enable or disable sprint?
                (bind _returnvalue (Utilities|Time|SetTimerbyFunctionName 0 "CheckStaminaForSprint" 0.05 true)) ; Initiate loop to check if stainda depletes whilst sprinting.
                (Variables|SprintSettings|SetStaminaSprintTimer _returnvalue) ; Store timer for later use.
                (return) ; Done.
                (else
                  (Utilities|Time|ClearandInvalidateTimerbyHandle (Variables|SprintSettings|GetStaminaSprintTimer)) ; Stop the stamina check timer.
                  (if (Variables|SprintSettings|GetSprintDecayActive) ; Is the sprint decay currently active?
                    (Default|SetDecay (Variables|BaseMovementSettings|GetManager-Stamina) (* -1 (Variables|SprintSettings|GetStaminaDrainOnSprint))) ; Remove a drain to the stamina associated with sprinting.
                    (Variables|SprintSettings|SetSprintDecayActive false) ; Reset sprint decay bool.
                    (return) ; Done.
                    (else
                      (return) ; Done.
                    ))))
              (else
                (return) ; Done.
              )))
          (:Remote
            (CallFunction|SRVToggleSprint (LocalVariables|GetSprintState)) ; Run this again on the server.
            (if (LocalVariables|GetSprintState) ; Enable or disable sprint?
              (Utilities|UpdatePlayerSpeed (Variables|SprintSettings|GetSprintSpeed)) ; Set character speed to sprint speed.
              (else
                (Utilities|UpdatePlayerSpeed (Variables|BaseMovementSettings|GetBaseWalkSpeed)) ; Set character speed to walk speed.
              ))
            (return) ; Done.
          ))
        (else
          (return) ; Done.
        )))))

(fn QueryMovementAllowance
  (bind _controlledchar (Variables|BaseMovementSettings|GetControlledChar))
  (Utilities|IsValid _controlledchar ; Valid character/
    (:Is%20Valid
      (LocalVariables|SetIsInAir (AI|Components|NavMovement|IsFalling (Variables|/Script/Engine.Character|GetCharacterMovement _controlledchar))) ; Update current fall state.
      (Utilities|FlowControl|Sequence
        (:then_0
          ;[1 1 1] Current in anim state fro crouch? Crouch allowed? Currently not prone or in air?
          (bind _newstate (Class|BPIntCharacter|ParseCrouchAnimState(Message) (Variables|BaseMovementSettings|GetControlledChar)))
          (LocalVariables|SetCanCrouch (Math|Boolean|ANDBoolean _newstate (Variables|CrouchSettings|GetAllowCrouch) (Math|Boolean|NotEqual(Boolean) (Variables|ProneSettings|GetIsProne) true) (Math|Boolean|NotEqual(Boolean) (LocalVariables|GetIsInAir) true))))
        (:then_1
          ;[1 1 1] Currently in anim state for prone? Prone allowed? Currently not in crouch or sprint or in air?
          (bind _newstate_2 (Class|BPIntCharacter|ParseProneAnimState(Message) (Variables|BaseMovementSettings|GetControlledChar)))
          (LocalVariables|SetCanProne (Math|Boolean|ANDBoolean _newstate_2 (Variables|ProneSettings|GetAllowProne) (Math|Boolean|NotEqual(Boolean) (Variables|CrouchSettings|GetIsCrouched) true) (Math|Boolean|NotEqual(Boolean) (Variables|SprintSettings|GetIsSprinting) true) (Math|Boolean|NotEqual(Boolean) (LocalVariables|GetIsInAir) true))))
        (:then_2
          ;[1 1 1] Sprint allowed? Currently not prone?
          (LocalVariables|SetCanSprint (Math|Boolean|ANDBoolean (Variables|SprintSettings|GetAllowSprint) (Math|Boolean|NotEqual(Boolean) (Variables|ProneSettings|GetIsProne) true) (Math|Boolean|NotEqual(Boolean) (Variables|BaseMovementSettings|GetSpeedAltered) true))))
        (:then_3
          ;[1 1 1] Jump allowed? Currently not prone, crouched or in air?
          (LocalVariables|SetCanJump (Math|Boolean|ANDBoolean (Variables|JumpSettings|GetAllowJump) (Math|Boolean|NotEqual(Boolean) (Variables|ProneSettings|GetIsProne) true) (Math|Boolean|NotEqual(Boolean) (Variables|CrouchSettings|GetIsCrouched) true) (Math|Boolean|NotEqual(Boolean) (LocalVariables|GetIsInAir) true)))
          (return (LocalVariables|GetCanCrouch) (LocalVariables|GetCanProne) (LocalVariables|GetCanSprint) (LocalVariables|GetCanJump)) ; Done.
        )))
    (:Is%20Not%20Valid
      (return false false false false) ; Done.
    )))

(fn SetTemporarySpeed
  (params (State :type Boolean) (NewSpeed :type Float%20%28single-precision%29))
  (LocalVariables|SetInState State) ; Set a reference to input state for\ncleaner use.
  (LocalVariables|SetInSpeed NewSpeed) ; Set a reference to input speed for\ncleaner use.
  (Utilities|SwitchHasAuthority ; Ensure this is running on the server.
    (:Authority
      (if (LocalVariables|GetInState) ; Are we enabling the temporary speed?
        (Variables|BaseMovementSettings|SetSpeedAltered true) ; Update speed altered bool to limit sprint.
        (Utilities|UpdatePlayerSpeed (LocalVariables|GetInSpeed)) ; Set the new player speed based on the\ninput speed.
        (return) ; Done
        (else
          (Utilities|UpdatePlayerSpeed (Variables|BaseMovementSettings|GetBaseWalkSpeed)) ; Set the player speed back to default.
          (Variables|BaseMovementSettings|SetSpeedAltered false) ; Reset the speed altered bool to enable\nsprint again.
          (return) ; Done
        )))
    (:Remote
      (CallFunction|SRVTemporarySpeed (LocalVariables|GetInState) (LocalVariables|GetInSpeed))
      (if (LocalVariables|GetInState) ; Are we enabling the temporary speed?
        (Utilities|UpdatePlayerSpeed (LocalVariables|GetInSpeed)) ; Set the new player speed based on the\ninput speed.
        (else
          (Utilities|UpdatePlayerSpeed (Variables|BaseMovementSettings|GetBaseWalkSpeed)) ; Set the player speed back to default.
        ))
      (return) ; Done
    )))