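; Inventory component that holds player inventory state: items, hotbar, equipment, held item, keys, discovered ingredients, available recipes, cooldowns and ammo.
; Reset and Initialize share one path that clears these collections and refills the fixed-size hotbar and equipment arrays with -1 as the empty marker.
; It then rebuilds the ammo pools by iterating the ammo type enum, adding a zero-count pool for each type.
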(event EventInitialize
  (params (PlayerController :type Player%20Controller%20Object%20Reference))
  (Utilities|Array|Clear (Variables|StorageVariables-DONOTEDIT|GetInventory)) ; Clear player inventory on startup\nand reinitialize.
  (Variables|StorageVariables-DONOTEDIT|SetHotbar (Utilities|Array|MakeArray -1 -1 -1 -1 -1 -1 -1 -1 -1 -1)) ; Create empty hotbar array on startup.
  (Variables|StorageVariables-DONOTEDIT|SetEquipment (Utilities|Array|MakeArray -1 -1 -1 -1 -1 -1 -1 -1 -1)) ; Create empty equipment array on startup.
  (Variables|StorageVariables-DONOTEDIT|SetHeldItem -1) ; Clear held item reference on startup.
  (Utilities|Array|Clear (Variables|StorageVariables-DONOTEDIT|GetPlayerKeys)) ; Clear player keys on startup.
  (Utilities|Array|Clear (Variables|StorageVariables-DONOTEDIT|GetDiscoveredIngredients)) ; Clear player's discovered ingredients on startup.
  (Utilities|Array|Clear (Variables|StorageVariables-DONOTEDIT|GetAvailableRecipes)) ; Clear player's available recipes on startup.
  (Utilities|Array|Clear (Variables|StorageVariables-DONOTEDIT|GetActiveCooldowns)) ; Clear active cooldowns array on startup.
  (Utilities|Array|Clear (Variables|StorageVariables-DONOTEDIT|GetAmmo)) ; Clear ammo pools on startup.
  (bind _enumvalue (|ForEachE_SGT_AmmoType) ; For each type of ammo listed in the Ammo enumerator...
    (:LoopBody
      (Utilities|Array|Add (Variables|StorageVariables-DONOTEDIT|GetAmmo) (Utilities|Struct|MakeStr_SGT_AmmoPool _enumvalue)) ; Create a new ammo pool with a count of 0.
    )))

(event EventReset
  (Utilities|Array|Clear (Variables|StorageVariables-DONOTEDIT|GetInventory)) ; Clear player inventory on startup\nand reinitialize.
  (Variables|StorageVariables-DONOTEDIT|SetHotbar (Utilities|Array|MakeArray -1 -1 -1 -1 -1 -1 -1 -1 -1 -1)) ; Create empty hotbar array on startup.
  (Variables|StorageVariables-DONOTEDIT|SetEquipment (Utilities|Array|MakeArray -1 -1 -1 -1 -1 -1 -1 -1 -1)) ; Create empty equipment array on startup.
  (Variables|StorageVariables-DONOTEDIT|SetHeldItem -1) ; Clear held item reference on startup.
  (Utilities|Array|Clear (Variables|StorageVariables-DONOTEDIT|GetPlayerKeys)) ; Clear player keys on startup.
  (Utilities|Array|Clear (Variables|StorageVariables-DONOTEDIT|GetDiscoveredIngredients)) ; Clear player's discovered ingredients on startup.
  (Utilities|Array|Clear (Variables|StorageVariables-DONOTEDIT|GetAvailableRecipes)) ; Clear player's available recipes on startup.
  (Utilities|Array|Clear (Variables|StorageVariables-DONOTEDIT|GetActiveCooldowns)) ; Clear active cooldowns array on startup.
  (Utilities|Array|Clear (Variables|StorageVariables-DONOTEDIT|GetAmmo)) ; Clear ammo pools on startup.
  (bind _enumvalue (|ForEachE_SGT_AmmoType) ; For each type of ammo listed in the Ammo enumerator...
    (:LoopBody
      (Utilities|Array|Add (Variables|StorageVariables-DONOTEDIT|GetAmmo) (Utilities|Struct|MakeStr_SGT_AmmoPool _enumvalue)) ; Create a new ammo pool with a count of 0.
    )))